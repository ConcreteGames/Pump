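; Test actor, apparently for HISM transform behavior, that pairs a very large instanced mesh field with an oscillating Arrow component.
; The construction script adds 100,000 HISM instances with random XY positions, rotations and scales.
; Tick accumulates time at half speed and feeds sine waves into the Arrow's relative location and rotation, with a different amplitude per axis.
; Leftover timeline oscillation logic is disconnected and never runs.
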(event `self.ReceiveBeginPlay`)

(event `self.ReceiveTick`
  (params (DeltaSeconds :type "Float (single-precision)"))
  (bind _newvar_0 (`self.NewVar_0`))
  (set `self.NewVar_0` (+ (* (`GameplayStatics.GetWorldDeltaSeconds`) 0.5) (`self.NewVar_0`)))
  (`SceneComponent.K2_SetRelativeLocationAndRotation` (`self.Arrow`) (`KismetMathLibrary.MakeVector` (+ 0.0 (* 100.0 (`KismetMathLibrary.Sin` (* _newvar_0 (`KismetMathLibrary.GetPI`) 2.0)))) (+ 0.0 (* 500.0 (`KismetMathLibrary.Sin` (* _newvar_0 (`KismetMathLibrary.GetPI`) 2.0)))) (+ 0.0 (* 1000.0 (`KismetMathLibrary.Sin` (* _newvar_0 (`KismetMathLibrary.GetPI`) 2.0))))) (`KismetMathLibrary.MakeRotator` (+ 0.0 (* 30.0 (`KismetMathLibrary.Sin` (* _newvar_0 (`KismetMathLibrary.GetPI`) 2.0)))) (+ 0.0 (* 5.0 (`KismetMathLibrary.Sin` (* _newvar_0 (`KismetMathLibrary.GetPI`) 2.0)))) (+ 0.0 (* 10.0 (`KismetMathLibrary.Sin` (* _newvar_0 (`KismetMathLibrary.GetPI`) 2.0))))) false false))

(fn `UserConstructionScript`
  (bind _returnvalue (`KismetMathLibrary.RandomFloatInRange` 1.0 2.0))
  (for _ (range 1 100001)
    (`InstancedStaticMeshComponent.AddInstance` (`self.HISM`) (`KismetMathLibrary.MakeTransform` (`KismetMathLibrary.MakeVector` (`KismetMathLibrary.RandomFloatInRange` -3000.0 3000.0) (`KismetMathLibrary.RandomFloatInRange` -3000.0 3000.0)) (`KismetMathLibrary.RandomRotator` false) (`KismetMathLibrary.MakeVector` _returnvalue _returnvalue _returnvalue)))))