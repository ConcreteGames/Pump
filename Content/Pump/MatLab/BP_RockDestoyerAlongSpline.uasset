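; BP_RockDestoyerAlongSpline removes hierarchical instanced static mesh instances, presumably rocks, along line segments passed to its TraceLine event.
; TraceLine runs one exact trace plus three copies with endpoints randomly offset by Marge to widen coverage.
; MultiLT multi-traces world static and dynamic objects with timed debug drawing, removing each hit HISM instance by its hit item index.
; No spline logic appears in these graphs.
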(event `TraceLine`
  (params (Start :type "Vector Structure") (End :type "Vector Structure"))
  (bind _marge (`self.Marge`))
  (`self.MultiLT` Start End (struct :`R` 1.0 :`B` 0.606405 :`A` 1.0) (struct :`G` 1.0 :`B` 0.333189 :`A` 1.0))
  (for _ (range 1 4)
    (`self.MultiLT` (+ Start (* (`KismetMathLibrary.RandomUnitVector`) _marge)) (+ End (* (`KismetMathLibrary.RandomUnitVector`) _marge)) (struct :`G` 0.788106 :`B` 1.0 :`A` 1.0) (struct :`R` 1.0 :`G` 0.926686 :`A` 1.0))))

(fn `MultiLT`
  (params (Start :type "Vector Structure") (End :type "Vector Structure") (TraceColor :type "LinearColor Structure") (TraceHitColor :type "LinearColor Structure"))
  (bind _outhits (`KismetSystemLibrary.LineTraceMultiForObjects` :`Start` Start :`End` End :`ObjectTypes` (`|MakeArray` "ObjectTypeQuery1" "ObjectTypeQuery2" :!type "EObjectTypeQuery Enum") :`DrawDebugType` "ForDuration" :`TraceColor` TraceColor :`TraceHitColor` TraceHitColor :`DrawTime` 20.0))
  (for (_array_element _array_index) _outhits
    (bind _ashierarchical_instanced_static_mesh_component (cast `HierarchicalInstancedStaticMeshComponent` (`.HitComponent` (`GameplayStatics.BreakHitResult` _array_element))))
    (`InstancedStaticMeshComponent.RemoveInstance` _ashierarchical_instanced_static_mesh_component (`.HitItem` (`GameplayStatics.BreakHitResult` _array_element)))))

(fn `UserConstructionScript`)