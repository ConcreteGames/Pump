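; BP_CubesGenerator scatters a field of cubes and gravity platforms around the world.
; When Activate is set, the construction script fills an instanced static mesh with about 20,000 randomly rotated, scaled cubes along random directions at random distances.
; On BeginPlay, a DoN loop spawns 20 randomly placed, rotated and scaled BP_GravityPlateform actors, pausing two frames between spawns, each with six downward gravity boxes.
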(event `self.ReceiveBeginPlay`
  (bind _returnvalue (`KismetMathLibrary.RandomFloatInRange` 1500.0 1500.0))
  (`/Engine/EditorBlueprintResources/StandardMacros.Do N` 20 :!label _label
    (:`Exit`
      (`|ExecutionSequence`
        (:`then_0`
          (`|SpawnActorFromClass` "/Game/Pump/LD/BP_GravityPlateform.BP_GravityPlateform_C" (`KismetMathLibrary.MakeTransform` (`KismetMathLibrary.MakeVector` (`KismetMathLibrary.RandomFloatInRange` -50000.0 50000.0) (`KismetMathLibrary.RandomFloatInRange` -50000.0 50000.0) (`KismetMathLibrary.RandomFloatInRange` -50000.0 50000.0)) (`KismetMathLibrary.RandomRotator` true) (`KismetMathLibrary.MakeVector` (`KismetMathLibrary.RandomFloatInRange` 0.5 20.0) (`KismetMathLibrary.RandomFloatInRange` 0.5 20.0) (`KismetMathLibrary.RandomFloatInRange` 0.5 20.0))) "Undefined" "OverrideRootScale" null (`|MakeArray` true true true true true true) (`|MakeArray` 3.0 0.0 0.0 0.0 0.0 0.0 :!type "Float (single-precision)") (`|MakeArray` _returnvalue _returnvalue _returnvalue _returnvalue _returnvalue _returnvalue) (`|MakeArray` (0.0 0.0 -1.0) (0.0 0.0 -1.0) (0.0 0.0 -1.0) (0.0 0.0 -1.0) (0.0 0.0 -1.0) (0.0 0.0 -1.0) :!type "Vector Structure") null))
        (:`then_1`
          (`LowEntryExtendedStandardLibrary.DelayFrames` 2)
          (goto _label))))))

(fn `UserConstructionScript`
  (if (`self.Activate`)
    (for _ (range 20001)
      (`SceneComponent.K2_SetWorldRotation` (`self.GenerationDirection`) (`KismetMathLibrary.MakeRotator` (`KismetMathLibrary.RandomFloatInRange` 0.0 360.0) (`KismetMathLibrary.RandomFloatInRange` 0.0 360.0) (`KismetMathLibrary.RandomFloatInRange` 0.0 360.0)) false false)
      (`InstancedStaticMeshComponent.AddInstance` (`self.ISM_Cube`) (`KismetMathLibrary.MakeTransform` (* (`SceneComponent.GetForwardVector` (`self.GenerationDirection`)) (`KismetMathLibrary.RandomIntegerInRange` 5000 100000)) (`KismetMathLibrary.RandomRotator` true) (`KismetMathLibrary.MakeVector` (`KismetMathLibrary.RandomFloatInRange` 0.0 2.5) (`KismetMathLibrary.RandomFloatInRange` 0.0 5.0) (`KismetMathLibrary.RandomFloatInRange` 0.0 50.0)))))))