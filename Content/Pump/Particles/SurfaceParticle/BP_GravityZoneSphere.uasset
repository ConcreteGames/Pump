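; BP_GravityZoneSphere is an actor that, going by its name and folder, shows a spherical gravity zone as a surface particle effect.
; It pushes its Velocity and SphereScale values into the Niagara component's matching user parameters.
; This runs in the Construction Script for editor preview and again on BeginPlay.
; The graphs contain no gravity or overlap logic.
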(event `self.ReceiveBeginPlay`
  (bind _niagara (`self.Niagara`))
  (`NiagaraComponent.SetNiagaraVariableFloat` _niagara "User.Velocity" (`self.Velocity`))
  (`NiagaraComponent.SetNiagaraVariableFloat` _niagara "User.SphereScale" (`self.SphereScale`)))

(fn `UserConstructionScript`
  (bind _niagara (`self.Niagara`))
  (`NiagaraComponent.SetNiagaraVariableFloat` _niagara "User.Velocity" (`self.Velocity`))
  (`NiagaraComponent.SetNiagaraVariableFloat` _niagara "User.SphereScale" (`self.SphereScale`)))