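; BP_TestSphere is a test actor that pairs a sphere component with a Niagara effect in the GravityParticle folder.
; The construction script sets the sphere's radius from the Radius variable, then feeds the scaled radius plus a fixed padding into the Niagara User.SphereRadius parameter.
; BeginPlay pushes the same padded value again, and both graphs print the scaled radius for debugging.
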(event `self.ReceiveBeginPlay`
  (bind _returnvalue (`SphereComponent.GetScaledSphereRadius` (`self.Sphere1`)))
  (`KismetSystemLibrary.PrintString` (`KismetStringLibrary.Conv_DoubleToString` _returnvalue))
  (`NiagaraComponent.SetNiagaraVariableFloat` (`self.Niagara`) "User.SphereRadius" (+ _returnvalue 20.0)))

(fn `UserConstructionScript`
  (bind _returnvalue (`SphereComponent.GetScaledSphereRadius` (`self.Sphere1`)))
  (`SphereComponent.SetSphereRadius` (`self.Sphere1`) (`self.Radius`) true)
  (`KismetSystemLibrary.PrintString` (`KismetStringLibrary.Conv_DoubleToString` _returnvalue))
  (`NiagaraComponent.SetNiagaraVariableFloat` (`self.Niagara`) "User.SphereRadius" (+ _returnvalue 20.0)))