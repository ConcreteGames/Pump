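; BP_Cloud is a placeable cloud actor for level dressing, built from an optional volumetric fog volume and an optional Niagara particle cloud.
; Its construction script creates a dynamic instance of the fog material to set extinction, and passes spawn rate and sprite size to the Niagara component.
; Whichever layer is toggled off has its component destroyed during construction.
; The event graph holds no runtime logic.
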(fn `UserConstructionScript`
  (bind _fogvolume (`self.FogVolume`))
  (if (`self.UseVolumetricFogVolume`)
    (bind _returnvalue (`PrimitiveComponent.CreateDynamicMaterialInstance` _fogvolume 0 "/Game/Pump/BadPaul/LevelBuildingRessources/Clouds/M_VolumetricFog_Inst.M_VolumetricFog_Inst" "None"))
    (`MaterialInstanceDynamic.SetScalarParameterValue` _returnvalue "Extinction" (`self.FogExtinction`))
    (else
      (`ActorComponent.K2_DestroyComponent` _fogvolume)))
  (if (`self.UseParticles`)
    (`NiagaraComponent.SetNiagaraVariableFloat` (`self.Niagara_Clouds`) "User.B.SpawnRate" (`self.ParticleSpawnRateMultiplier`))
    (`NiagaraComponent.SetNiagaraVariableFloat` (`self.Niagara_Clouds`) "User.B.Particles.SpriteSize.Value" (`self.ParticleSpriteSize`))
    (else
      (`ActorComponent.K2_DestroyComponent` (`self.Niagara_Clouds`)))))