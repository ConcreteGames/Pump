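; BP_LookAtPlayer is an actor that turns to face the player's gravity character.
; BeginPlay caches the player pawn as a BP_GravityCharacter_Pump reference.
; While its root component is visible, each Tick snaps the actor's rotation toward that character with a look-at rotation and teleport physics.
; Each of those ticks also prints the computed rotation to screen.
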(event `self.ReceiveBeginPlay`
  (bind _asbp_gravity_character_pump (cast `/Game/Pump/Core/Character/BP_GravityCharacter_Pump` (`GameplayStatics.GetPlayerPawn` 0)))
  (set `self.pChar` _asbp_gravity_character_pump))

(event `self.ReceiveTick`
  (params (DeltaSeconds :type "Float (single-precision)"))
  (bind _returnvalue (`KismetMathLibrary.FindLookAtRotation` (`self.K2_GetActorLocation`) (`self.K2_GetActorLocation` (`self.pChar`))))
  (if (`SceneComponent.IsVisible` (`self.DefaultSceneRoot`))
    (`KismetSystemLibrary.PrintString` (`KismetStringLibrary.Conv_RotatorToString` _returnvalue))
    (`self.K2_SetActorRotation` _returnvalue true)))

(fn `UserConstructionScript`)