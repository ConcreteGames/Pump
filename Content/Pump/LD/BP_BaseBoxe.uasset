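; Base box-shaped gravity volume that applies gravity through its BPGravityVolumeComponent every Tick.
; The construction script passes the actor's Force and Priority to that component.
; InitParticle configures the Niagara effect from box size and MapGravitySphereParticleValues, with an optional manual spawn rate.
; Inverted gravity halves the particle box and flips velocity sign, while hard or soft gravity picks the color.
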(event `self.ReceiveTick`
  (params (DeltaSeconds :type "Float (single-precision)"))
  (`/Game/DirectionalGravity/Blueprints/GravityLogic/BP_GravityVolumeComponent.ApplyGravity` (`self.BP_GravityVolumeComponent`)))

(fn `InitParticle`
  (bind _returnvalue (`self.MapGravitySphereParticleValues` 5.0 100.0))
  (bind _gravityboxsize (`self.GravityBoxSize`))
  (bind _particle (`self.Particle`))
  (`NiagaraComponent.SetNiagaraVariableVec3` _particle "User.BoxSize" (select `bool` (`self.InvertGravity`) :`false` _gravityboxsize :`true` (/ _gravityboxsize 2.0)))
  (`NiagaraComponent.SetNiagaraVariableFloat` _particle "User.SpawnRate" (select `bool` (`self.bManualParticleSpawnRate`) :`false` (`self.MapGravitySphereParticleValues` 100.0 10000.0) :`true` (`self.ParticleSpawnRate`)))
  (`NiagaraComponent.SetNiagaraVariableVec2` _particle "User.SpriteSize" (`KismetMathLibrary.MakeVector2D` _returnvalue (* _returnvalue 10.0)))
  (`NiagaraComponent.SetNiagaraVariableFloat` _particle "User.Velocity" (select `bool` (`self.InvertGravity`) :`false` (`self.MapGravitySphereParticleValues` -2.0 -20.0) :`true` (`self.MapGravitySphereParticleValues` 2.0 20.0)))
  (`NiagaraComponent.SetNiagaraVariableLinearColor` _particle "User.Color" (select `bool` (`self.bGravityHard`) :`false` (`self.SoftGravityColor`) :`true` (`self.HardGravityColor`)))
  (`NiagaraComponent.SetNiagaraVariableFloat` _particle "User.ParticleLifetime" (`self.MapGravitySphereParticleValues` 1.0 6.0)))

(fn `UserConstructionScript`
  (bind _bp_gravityvolumecomponent (`self.BP_GravityVolumeComponent`))
  (set `/Game/DirectionalGravity/Blueprints/GravityLogic/BP_GravityVolumeComponent.Force` (`self.Force`) _bp_gravityvolumecomponent)
  (set `/Game/DirectionalGravity/Blueprints/GravityLogic/BP_GravityVolumeComponent.Priority` (`self.Priority`) _bp_gravityvolumecomponent))