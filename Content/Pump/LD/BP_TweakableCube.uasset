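; Level-design cube that spawns gravity volumes on any of its six faces, toggled and tuned through per-face arrays.
; The Construction Script converts each face arrow's transform through a helper arrow, adds a child-actor gravity box there, then sets force, direction, priority and Z scale.
; A zero Z scale falls back to the first face's value.
; Each box also gets a Niagara effect positioned and sized from its calculated bounds, with a debug size print.
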(fn `UserConstructionScript`
  (bind _newvar_0 (`self.NewVar_0`))
  (bind _newvar_1 (`self.NewVar_1`))
  (bind _gravboxesscalez (`self.GravBoxesScaleZ`))
  (bind _output_get (set `self.ArrowArray` (`|MakeArray` (`self.Arrow0Top`) (`self.Arrow1Bot`) (`self.Arrow2Front`) (`self.Arrow3Back`) (`self.Arrow4Left`) (`self.Arrow5Right`))))
  (for (_array_element _array_index) _output_get
    (if (`|GetArrayItem` (`self.SpawnGravBoxes`) _array_index)
      (bind (_returnvalue_location _returnvalue_rotation _returnvalue_scale) (`KismetMathLibrary.BreakTransform` (`SceneComponent.K2_GetComponentToWorld` _array_element)))
      (bind (_returnvalue_location_2 _returnvalue_rotation_2) (`KismetMathLibrary.BreakTransform` (`SceneComponent.GetRelativeTransform` _array_element)))
      (`SceneComponent.K2_SetWorldTransform` (`self.ArrowConversion`) (`KismetMathLibrary.MakeTransform` _returnvalue_location _returnvalue_rotation (`KismetMathLibrary.GreaterGreater_VectorRotator` _returnvalue_scale _returnvalue_rotation_2)) false false)
      (bind _returnvalue (`AddComponent|NODE_AddChildActorComponent-0` :`RelativeTransform` (`SceneComponent.GetRelativeTransform` (`self.ArrowConversion`))))
      (bind (_returnvalue_x _returnvalue_y) (`KismetMathLibrary.BreakVector` (`SceneComponent.K2_GetComponentScale` _returnvalue)))
      (bind _output (`|GetArrayItem` _gravboxesscalez _array_index))
      (`SceneComponent.SetWorldScale3D` _returnvalue (`KismetMathLibrary.MakeVector` _returnvalue_x _returnvalue_y (select `bool` (!= _output 0.0) :`false` (`|GetArrayItem` _gravboxesscalez) :`true` _output)))
      (bind _childactor (`ChildActorComponent.ChildActor` _returnvalue))
      (bind _asbp_gravity_volume_base (cast `/Game/DirectionalGravity/Blueprints/GravityLogic/BP_GravityVolumeBase` _childactor))
      (set `/Game/DirectionalGravity/Blueprints/GravityLogic/BP_GravityVolumeBase.Force` (`|GetArrayItem` (`self.GravBoxesForce`) _array_index) _asbp_gravity_volume_base)
      (set `/Game/DirectionalGravity/Blueprints/GravityLogic/BP_GravityVolumeBase.LocalDirection` (`|GetArrayItem` (`self.GravBoxesDirection`) _array_index) _asbp_gravity_volume_base)
      (set `/Game/DirectionalGravity/Blueprints/GravityLogic/BP_GravityVolumeBase.Priority` (`|GetArrayItem` (`self.GravBoxesPriority`) _array_index) _asbp_gravity_volume_base)
      (bind _returnvalue_2 (`AddComponent|NODE_AddNiagaraComponent-1` :`RelativeTransform` (`KismetMathLibrary.MakeTransform` (0.0 0.0 0.0))))
      (bind _asbp_gravity_box (cast `/Game/Pump/LD/BP_GravityBox` _childactor :!pure true))
      (`SceneComponent.K2_SetWorldRotation` _returnvalue_2 (`self.K2_GetActorRotation` _asbp_gravity_box) false false)
      (bind (_xdistance _ydistance _zdistance _centerlocation) (`/Game/Pump/LD/BP_GravityBox.SizeCalculation` _asbp_gravity_box))
      (set `self.NewVar_0` _xdistance)
      (set `self.NewVar_1` _ydistance)
      (`SceneComponent.K2_SetWorldLocation` _returnvalue_2 _centerlocation false false)
      (`KismetSystemLibrary.PrintString` (`KismetStringLibrary.Concat_StrStr` (`KismetStringLibrary.Conv_DoubleToString` _newvar_0) "---" (`KismetStringLibrary.Conv_DoubleToString` _newvar_1)))
      (`NiagaraComponent.SetNiagaraVariableVec2` _returnvalue_2 "User.PlainSize" (`KismetMathLibrary.MakeVector2D` _newvar_0 _newvar_1)))))