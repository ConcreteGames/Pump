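; Chapter 2 decor manager that gathers level decor into Hierarchical Instanced Static Mesh components.
; BeginPlay fills AllHISM with the chapter's HISM components for root rocks, root rocks with trees and big mossy rocks.
; CheckAllAssetsAndConvertToHISM converts BP_ChouRomanesco actors into their own HISM, then runs ConvertMeshesToHISM on each component in that array.
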(event `self.ReceiveBeginPlay`
  (set `self.AllHISM` (`|MakeArray` (`self.HISM_SM_MERGED_RootsRock3_b`) (`self.HISM_SM_MERGED_RootsRock1_b`) (`self.HISM_SM_MERGED_RootsRock1_b_fixed`) (`self.HISM_SM_MERGED_RootsRock1_fixed`) (`self.HISM_SM_MERGED_RootsRock2`) (`self.HISM_SM_MERGED_RootsRock2_b`) (`self.HISM_SM_MERGED_RootsRock1`) (`self.HISM_SM_MERGED_RootsRock3`) (`self.HISM_SM_MERGED_RootsRock2_b_fixed`) (`self.HISM_SM_MERGED_RootsRock3_b_fixed`) (`self.HISM_SM_MERGED_RootsRock3_fixed`) (`self.HISM_SM_MERGED_RootsRock4`) (`self.HISM_SM_MERGED_RootsRock4_b`) (`self.HISM_MossyRockBigSize_2`) (`self.HISM_MossyRockBigSize_3`) (`self.HISM_MossyRockBigSize_4`) (`self.HISM_MossyRockBigSize_1`) (`self.HISM_SM_MERGED_RootsRockTree_1`) (`self.HISM_SM_MERGED_RootsRockTree_1_B`) (`self.HISM_SM_MERGED_RootsRockTree_1_C`) (`self.HISM_SM_MERGED_RootsRockTree_1B_B`) (`self.HISM_SM_MERGED_RootsRockTree_1B_C`) (`self.HISM_SM_MERGED_RootsRockTree_2_A`) (`self.HISM_SM_MERGED_RootsRockTree_2_C`) (`self.HISM_SM_MERGED_RootsRockTree_2B_A`) (`self.HISM_SM_MERGED_RootsRockTree_2B_B`) (`self.HISM_SM_MERGED_RootsRockTree_3_A`) (`self.HISM_SM_MERGED_RootsRockTree_3B_A`) (`self.HISM_SM_MERGED_RootsRockTree_4_A`) (`self.HISM_SM_MERGED_RootsRockTree_4B_A`))))

(event `CheckAllAssetsAndConvertToHISM`
  (`/Game/Pump/Core/BP_FunctionLibrary.ConvertActorToHISM` "/Game/Pump/BadPaul/LevelBuildingRessources/ChouRomanesco/BP_ChouRomanesco.BP_ChouRomanesco_C" (`self.HISM_ChouRomanesco`))
  (for _array_element (`self.AllHISM`)
    (`/Game/Pump/Core/BP_FunctionLibrary.ConvertMeshesToHISM` _array_element)))

(fn `UserConstructionScript`)