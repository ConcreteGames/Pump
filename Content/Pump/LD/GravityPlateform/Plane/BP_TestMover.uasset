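; BP_TestMover is a test actor in the gravity platform level design folder that oscillates around its starting position.
; On BeginPlay it stores its location, sets a five-second timeline length and plays the timeline.
; Each update offsets the actor along its combined right and up vectors by a sine wave of timeline progress, without sweeping.
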(event `self.ReceiveBeginPlay`
  (bind _timeline_0 (`self.Timeline_0`))
  (set `self.NewVar_0` (`self.K2_GetActorLocation`))
  (`TimelineComponent.SetTimelineLength` _timeline_0 5.0)
  (`Timeline|Timeline_0` :!via `PlayFromStart`
    (:`Update`
      (`self.K2_SetActorLocation` (+ (`self.NewVar_0`) (* (+ (`self.GetActorRightVector`) (`self.GetActorUpVector`)) (* (`KismetMathLibrary.Sin` (* (`/Game/Pump/Core/BP_FunctionLibrary.GetTimelinePercentage` _timeline_0) (`KismetMathLibrary.GetPI`) 2.0)) 1000.0 1.0)))))))

(fn `UserConstructionScript`)