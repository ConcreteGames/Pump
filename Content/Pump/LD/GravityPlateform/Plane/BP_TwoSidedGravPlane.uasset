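; Two-sided gravity platform built from two child-actor gravity planes, each with its own force, priority, direction and gravity zone scale.
; The construction script pushes per-side array values, shared material, surface type and tags into both planes, falling back to the first scale when one is zero.
; It disables tile spawning on the second plane and tints its selector visual green, relying on running after the children's construction scripts to override them.
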(fn `SpawnTilesOnlyForTopPlane`
  (bind _asbp_gravity_plateform_plane (cast `/Game/Pump/LD/GravityPlateform/Plane/BP_GravityPlateform_Plane` (`ChildActorComponent.ChildActor` (`self.ChildActor`))))
  (set `/Game/Pump/LD/GravityPlateform/Plane/BP_GravityPlateform_Plane.NeedToSpawnTiles` false _asbp_gravity_plateform_plane)
  (bind _returnvalue (`PrimitiveComponent.CreateDynamicMaterialInstance` (`/Game/Pump/LD/GravityPlateform/Plane/BP_GravityPlateform_Plane.OnlyVisual_Selector` _asbp_gravity_plateform_plane) 0 null "None"))
  (`MaterialInstanceDynamic.SetVectorParameterValue` _returnvalue "DiffuseColor" (struct :`R` 0.57836 :`G` 0.713542 :`B` 0.25723 :`A` 1.0)))

(fn `UserConstructionScript`
  (bind _scales (`self.Scales`))
  (`self.SpawnTilesOnlyForTopPlane`)
  (for (_array_element _array_index) (`|MakeArray` (`self.BP_GravityPlateform_Plane`) (`self.ChildActor`))
    (bind _childactor (`ChildActorComponent.ChildActor` _array_element))
    (bind _asbp_gravity_plateform (cast `/Game/Pump/LD/GravityPlateform/BP_GravityPlateform` _childactor :!pure true))
    (set `/Game/Pump/LD/GravityPlateform/BP_GravityPlateform.Force` (`|GetArrayItem` (`self.Forces`) _array_index) _asbp_gravity_plateform)
    (set `/Game/Pump/LD/GravityPlateform/BP_GravityPlateform.Priority` (`|GetArrayItem` (`self.Priority`) _array_index) _asbp_gravity_plateform)
    (set `/Game/Pump/LD/GravityPlateform/BP_GravityPlateform.Plane_LocalDirection` (`|GetArrayItem` (`self.Directions`) _array_index) _asbp_gravity_plateform)
    (bind _asbp_gravity_plateform_plane (cast `/Game/Pump/LD/GravityPlateform/Plane/BP_GravityPlateform_Plane` _childactor :!pure true))
    (bind _output (`|GetArrayItem` _scales _array_index))
    (`/Game/Pump/LD/GravityPlateform/Plane/BP_GravityPlateform_Plane.SetGravityZoneScale` _asbp_gravity_plateform_plane (select `bool` (== _output 0.0) :`false` _output :`true` (`|GetArrayItem` _scales))) ; Il semblerait qu'il suffise de faire ça\ncar on dirait que ce construction script se joue après celui de l'objet en question\ndu coup ça l'override bien comme on veut !
    (`/Game/Pump/LD/GravityPlateform/Plane/BP_GravityPlateform_Plane.Set MID` _asbp_gravity_plateform_plane (`self.SourceMaterial`) (`self.SurfaceType`))
    (set `Actor.Tags` (`self.Tags`) (`ChildActorComponent.ChildActor` (`self.BP_GravityPlateform_Plane`)))
    (set `Actor.Tags` (`self.Tags`) (`ChildActorComponent.ChildActor` (`self.ChildActor`)))))