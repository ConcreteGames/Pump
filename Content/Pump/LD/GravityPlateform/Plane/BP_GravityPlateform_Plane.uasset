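; Flat gravity platform: a gravity volume with a walkable tiled floor that reacts to player landings.
; Construction sets dynamic materials per surface type, scales the gravity zone and configures under-collision and optional blocking walls.
; BeginPlay can fill the arrow-bounded area with jittered instanced tiles, randomly thinning edges, deferred to avoid construction-time scale issues.
; Landing velocity drives timeline shader waves, with a one-time walked coloration and particle burst before first walk.
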(event `self.CharacterFirstStep`
  ;[1 1 1] Bases
  (`parent.CharacterFirstStep`))

(event `self.ReceiveBeginPlay`
  ;[1 1 1] Bases
  (`parent.ReceiveBeginPlay`)
  (`self.SpawnTileIfNeeded`))

(event `self.ReceiveTick`
  (params (DeltaSeconds :type "Float (single-precision)"))
  ;[1 1 1] Bases
  (`parent.ReceiveTick` DeltaSeconds))

(event `Set MID`
  (params (SurfaceType :type "/Game/Pump/LD/GravityPlateform/ESurfaceType Enum" :default "NewEnumerator5"))
  (bind _hism_tile (`self.HISM_Tile`))
  (bind _midlod0 (`self.MIDLOD0`))
  (bind _hism_tile_2 (`self.HISM_Tile`))
  ;[1 0.9402 0] Set Dynamic Material for all types of surfaces
  (bind _output_get (set `self.SurfaceType` SurfaceType))
  (set `self.SourceMaterialLOD0` (select `/Game/Pump/LD/GravityPlateform/ESurfaceType` _output_get :`NewEnumerator3` (`|GetArrayItem` (`self.PreMineralMat`) (`KismetMathLibrary.RandomInteger` 0)) :`NewEnumerator12` "/Game/Pump/LD/GravityPlateform/Materials/Azulejos/M_WalkableFloorAzulejos_Inst.M_WalkableFloorAzulejos_Inst"))
  (set `self.SourceMaterialLOD1` (select `/Game/Pump/LD/GravityPlateform/ESurfaceType` _output_get :`NewEnumerator5` "/Game/Pump/LD/GravityPlateform/Materials/LOD01/M_WalkableFloorBaseLOD1_Inst.M_WalkableFloorBaseLOD1_Inst" :`NewEnumerator3` "/Game/Pump/LD/GravityPlateform/Materials/LOD01/M_WalkableFloorBaseLOD1_Inst.M_WalkableFloorBaseLOD1_Inst" :`NewEnumerator6` "/Game/Pump/LD/GravityPlateform/Materials/LOD01/M_WalkableFloorBaseLOD1_Inst.M_WalkableFloorBaseLOD1_Inst" :`NewEnumerator7` "/Game/Pump/LD/GravityPlateform/Materials/LOD01/M_WalkableFloorBaseLOD1_Inst.M_WalkableFloorBaseLOD1_Inst" :`NewEnumerator4` "/Game/Pump/LD/GravityPlateform/Materials/LOD01/M_WalkableFloorBaseLOD1_Inst.M_WalkableFloorBaseLOD1_Inst" :`NewEnumerator8` "/Game/Pump/LD/GravityPlateform/Materials/LOD01/M_WalkableFloorBaseLOD1_Inst.M_WalkableFloorBaseLOD1_Inst" :`NewEnumerator9` "/Game/Pump/LD/GravityPlateform/Materials/LOD01/M_WalkableFloorBaseLOD1_Inst.M_WalkableFloorBaseLOD1_Inst" :`NewEnumerator1` "/Game/Pump/LD/GravityPlateform/Materials/LOD01/M_WalkableFloorBaseLOD1_Inst.M_WalkableFloorBaseLOD1_Inst" :`NewEnumerator10` "/Game/Pump/LD/GravityPlateform/Materials/LOD01/M_WalkableFloorBaseLOD1_Inst.M_WalkableFloorBaseLOD1_Inst" :`NewEnumerator11` "/Game/Pump/LD/GravityPlateform/Materials/LOD01/M_WalkableFloorBaseLOD1_Inst.M_WalkableFloorBaseLOD1_Inst" :`NewEnumerator12` "/Game/Pump/LD/GravityPlateform/Materials/LOD01/M_WalkableFloorBaseLOD1_Inst.M_WalkableFloorBaseLOD1_Inst" :!type "MaterialInterface Object Reference"))
  (bind _returnvalue (`PrimitiveComponent.CreateDynamicMaterialInstance` _hism_tile_2 0 (`self.SourceMaterialLOD0`) "None"))
  (bind _output_get_2 (set `self.MIDLOD0` _returnvalue))
  (`PrimitiveComponent.SetMaterial` _hism_tile_2 0 _output_get_2)
  (bind _returnvalue_2 (`PrimitiveComponent.CreateDynamicMaterialInstance` _hism_tile 1 (`self.SourceMaterialLOD1`) "None"))
  (bind _output_get_3 (set `self.MIDLOD1` _returnvalue_2))
  (`PrimitiveComponent.SetMaterial` _hism_tile 1 _output_get_3)
  (switch `/Game/Pump/LD/GravityPlateform/ESurfaceType` (`self.SurfaceType`)
    (:`NewEnumerator5`
      _)
    (:`NewEnumerator3`
      _)
    (:`NewEnumerator6`
      _)
    (:`NewEnumerator7`
      _)
    (:`NewEnumerator4`
      _)
    (:`NewEnumerator8`
      _)
    (:`NewEnumerator9`
      _)
    (:`NewEnumerator1`
      _)
    (:`NewEnumerator10`
      _)
    (:`NewEnumerator11`
      _))
  (`MaterialInstanceDynamic.SetScalarParameterValue` _midlod0 "Offset" (`KismetMathLibrary.RandomFloatInRange` 0.0 100.0))
  (`MaterialInstanceDynamic.SetScalarParameterValue` _midlod0 "Rotation" (`KismetMathLibrary.RandomFloatInRange` 0.0 1.0))
  (`MaterialInstanceDynamic.SetScalarParameterValue` _midlod0 "NTiles" (`KismetMathLibrary.Conv_IntToDouble` (`self.NOfTiles`))))

(event `/Game/Pump/Core/Beacons/BI_Events.HitGroundPlateform`
  (params (Velocity :type "Float (single-precision)") (IsWalkedOnce :type Boolean))
  ;[1 1 1] Hit Ground Event
  (set `self.PlayerVelocity` Velocity)
  (`self.HitGoundShaderFx`)
  (`self.HitGroundParticlesEvent`))

(event `HitGoundShaderFx`
  (bind _plateformwavespower (`self.PlateformWavesPower`))
  (bind _midlod0 (`self.MIDLOD0`))
  ;[0.6663 1 0] Hit Ground Shader Movement
  (set `self.PlateformWavesPower` (`KismetMathLibrary.MapRangeClamped` (`self.PlayerVelocity`) 500.0 3000.0 1.5 8.0))
  (bind (_direction _cosinepower _distancefromplayer _alpha _vectorlength) (`Timeline|TilesTimeline` :!via `PlayFromStart`)
    (:`Update`
      (`MaterialInstanceDynamic.SetScalarParameterValue` _midlod0 "Cosine" (* _cosinepower (`self.PlateformWavesPower`)))
      (`MaterialInstanceDynamic.SetScalarParameterValue` _midlod0 "DistanceImpact" (* _plateformwavespower 100.0))
      (`MaterialInstanceDynamic.SetScalarParameterValue` _midlod0 "AlphaForImpact" (* _alpha (`KismetMathLibrary.MapRangeClamped` _plateformwavespower 1.5 6.0 0.5 1.0)))
      (bind _returnvalue (* _vectorlength (`KismetMathLibrary.MapRangeClamped` (`self.PlateformWavesPower`) 1.5 6.0 1.0 2.0)))
      (`MaterialInstanceDynamic.SetScalarParameterValue` _midlod0 "VectorLength" _returnvalue)
      (`MaterialInstanceDynamic.SetScalarParameterValue` _midlod0 "VectorLengthEnd" (- _returnvalue (`KismetMathLibrary.MapRangeClamped` 0.0 1.5 6.0 (`self.MinWaveSize`) (`self.MaxWaveSize`))))
      ;[1 0.9775 0.6161] Tiles Coloration
      (if (not (`self.bHasStartedColoring`))
        (set `self.bHasStartedColoring` true)
        (bind (_direction_2 _cosinepower_2 _distancefromplayer_2 _alpha_2 _vectorlength_2) (`Timeline|FirstWalkColoration` :!via `PlayFromStart`)
          (:`Update`
            (`MaterialInstanceDynamic.SetScalarParameterValue` _midlod0 "VectorLengthMiddle" (* _vectorlength_2 (`KismetMathLibrary.MapRangeClamped` (`self.PlateformWavesPower`) 1.5 6.0 1.0 2.0))))
          (:`Finished`
            (`self.EndEventColoured` (`self.MIDLOD0`))))))))

(event `HitGroundParticlesEvent`
  (bind _pcharacter (`self.PCharacter`))
  (bind _pparticlemanager (`self.PParticleManager`))
  (bind _ischaracterlocation (`/Game/Pump/Core/Beacons/BP_ParticleManager.IsCharacterLocation` _pparticlemanager))
  ;[1 1 1] Hit Ground Particle Event
  (if (and (not (`self.IsWalkedOnce`)) (`self.SpawnParticles`))
    (`NiagaraFunctionLibrary.SpawnSystemAtLocation` (`/Game/Pump/Core/Beacons/BP_ParticleManager.VFX_ParticleSystem` _pparticlemanager) (select `bool` _ischaracterlocation :`false` (`/Game/Pump/Core/Beacons/BP_ParticleManager.ParticleLocation` _pparticlemanager) :`true` (`self.K2_GetActorLocation` _pcharacter)) (select `bool` _ischaracterlocation :`false` (`/Game/Pump/Core/Beacons/BP_ParticleManager.ParticleRotation` _pparticlemanager) :`true` (`self.K2_GetActorRotation` _pcharacter)))))

(fn `ActivateWallForClonePlane`
  (if (`self.ActivateWalls`)
    (for _array_element (`|MakeArray` (`self.WallBack`) (`self.WallLeft`) (`self.WallRight`) (`self.WallFront`))
      (`PrimitiveComponent.SetCollisionEnabled` _array_element "QueryAndPhysics")
      (`PrimitiveComponent.SetCollisionObjectType` _array_element "ECC_WorldStatic")
      (`PrimitiveComponent.SetCollisionProfileName` _array_element "BlockAll"))))

(fn `ConfigureUnderCollisions`
  (bind _undercone (`self.UnderCone`))
  (bind _undercube (`self.UnderCube`))
  (bind _undercone_2 (`self.UnderCone`))
  (bind (_returnvalue_x _returnvalue_y) (`KismetMathLibrary.BreakVector` (`SceneComponent.K2_GetComponentScale` _undercube)))
  (bind (_returnvalue_x_2 _returnvalue_y_2) (`KismetMathLibrary.BreakVector` (`SceneComponent.K2_GetComponentScale` _undercone_2)))
  (`SceneComponent.SetWorldScale3D` _undercube (`KismetMathLibrary.MakeVector` _returnvalue_x _returnvalue_y 1.0)) ; Normalize collision scale Z
  (`SceneComponent.K2_SetWorldLocation` _undercone (+ (`SceneComponent.K2_GetComponentLocation` _undercone) (* (`SceneComponent.GetUpVector` _undercube) -50.0)) false false)
  (`SceneComponent.SetWorldScale3D` _undercone_2 (`KismetMathLibrary.MakeVector` _returnvalue_x_2 _returnvalue_y_2 2.0)))

(fn `DistanceBetweenTwoPoints`
  (params (A :type "Vector Structure") (B :type "Vector Structure"))
  (returns (AbsoluteDistance :type "Float (double-precision)"))
  (return (`KismetMathLibrary.Abs` (`KismetMathLibrary.VSize` (- A B)))))

(fn `EndEventColoured`
  (params (MID :type "MaterialInstanceDynamic Object Reference"))
  (if (not (`self.bColoured`))
    (set `self.bColoured` true)
    (`MaterialInstanceDynamic.SetScalarParameterValue` MID "Walked" 1.0)))

(fn `GetAzulejosManager`
  (returns (AzulejosManager :type "/Game/Pump/LD/GravityPlateform/BP_AzulejosManager Object Reference"))
  (`/Engine/EditorBlueprintResources/StandardMacros.IsValid` (`self.pHISM_Tile`)
    (:`Is Valid`
      (return (stale _output_get)))
    (:`Is Not Valid`
      (bind _outactors (`GameplayStatics.GetAllActorsOfClass` "/Game/Pump/LD/GravityPlateform/BP_AzulejosManager.BP_AzulejosManager_C"))
      (bind _output (`|GetArrayItem` _outactors))
      (`/Engine/EditorBlueprintResources/StandardMacros.IsValid` _output
        (:`Is Valid`
          (bind _output_get (set `self.pAzulejosManager` _output))
          (return _output_get))
        (:`Is Not Valid`
          (`/Game/Pump/Core/BP_FunctionLibrary.LogErerror` "NEED in the LEVEL : BP_AzulejosManager"))))))

(fn `MSpaceColorParameters`)

(fn `SetGravityZoneScale`
  (params (NewScale_Z :type "Float (double-precision)"))
  (bind _defaultsceneroot (`self.DefaultSceneRoot`))
  (bind (_returnvalue_x _returnvalue_y) (`KismetMathLibrary.BreakVector` (`SceneComponent.K2_GetComponentScale` _defaultsceneroot)))
  (`SceneComponent.SetWorldScale3D` _defaultsceneroot (`KismetMathLibrary.MakeVector` _returnvalue_x _returnvalue_y NewScale_Z)))

(fn `SizeCalculation`
  (returns (XDistance :type "Float (double-precision)") (YDistance :type "Float (double-precision)") (ZDistance :type "Float (double-precision)") (CenterLocation :type "Vector Structure") (LocalDirection :type "Vector Structure") (Force :type "Float (double-precision)"))
  (bind _bp_gravityvolumecomponent (`self.BP_GravityVolumeComponent`))
  (return (`self.DistanceBetweenTwoPoints` (`SceneComponent.K2_GetComponentLocation` (`self.ArrowFrontLeft`)) (`SceneComponent.K2_GetComponentLocation` (`self.ArrowBackLeft`))) (`self.DistanceBetweenTwoPoints` (`SceneComponent.K2_GetComponentLocation` (`self.ArrowLeft`)) (`SceneComponent.K2_GetComponentLocation` (`self.ArrowRight`))) (`self.DistanceBetweenTwoPoints` (`SceneComponent.K2_GetComponentLocation` (`self.ArrowBackRight`)) (`SceneComponent.K2_GetComponentLocation` (`self.ArrowTop`))) (`SceneComponent.K2_GetComponentLocation` (`self.ArrowCenter`)) (`/Game/Pump/LD/GravityPlateform/BP_GravityVolumeComponent.LocalDirection` _bp_gravityvolumecomponent) (`/Game/Pump/LD/GravityPlateform/BP_GravityVolumeComponent.Force` _bp_gravityvolumecomponent)))

(fn `SpawnTileIfNeeded`
  (if (`self.NeedToSpawnTiles`)
    (`self.SpawnTiles`) ; On le met ici, sinon si on le met dans le construction script\nil se tape le scale du construction script de Cube
  ))

(fn `SpawnTiles`
  (locals (XLength :type Integer :default 0) (YLength :type Integer :default 0))
  (bind (_returnvalue_x _returnvalue_y) (`KismetMathLibrary.BreakVector` (`self.GetActorScale3D`)))
  (bind _onetilelength (`self.OneTileLength`))
  (bind _arrowbackleft (`self.ArrowBackLeft`))
  (bind _returnvalue (/ (`self.OneTileLength`) 4.0))
  (bind _returnvalue_2 (- (`local.YLength`) 1))
  (bind _returnvalue_3 (- (`local.XLength`) 1))
  (bind _returnvalue_4 (/ (`KismetMathLibrary.Conv_IntToDouble` (`KismetMathLibrary.Round` (`/Game/Pump/Core/BP_FunctionLibrary.DistanceBetweenTwoArrows` (`self.ArrowBackLeft`) (`self.ArrowFrontLeft`)))) (`self.OneTileLength`)))
  (bind _returnvalue_5 (/ (`KismetMathLibrary.Conv_IntToDouble` (`KismetMathLibrary.Round` (`/Game/Pump/Core/BP_FunctionLibrary.DistanceBetweenTwoArrows` (`self.ArrowBackLeft`) (`self.ArrowBackRight`)))) (`self.OneTileLength`)))
  (set `local.XLength` (`KismetMathLibrary.FFloor` _returnvalue_4))
  (set `local.YLength` (`KismetMathLibrary.FFloor` _returnvalue_5))
  ;[1 1 1] Décalage si le scale de la plateforme n'est pas pair
  (`SceneComponent.K2_AddRelativeLocation` (`self.ArrowBackLeft`) (`KismetMathLibrary.MakeVector` (/ (select `bool` (!= (mod _returnvalue_4 1.0) 0.0) :`true` _returnvalue) _returnvalue_x) (/ (select `bool` (!= (mod _returnvalue_5 1.0) 0.0) :`true` _returnvalue) _returnvalue_y)) false true)
  (for _index (range (+ _returnvalue_3 1))
    (for _index_2 (range (+ _returnvalue_2 1))
      (if (select `bool` (or (or (== _index 0) (== _index _returnvalue_3)) (or (== _index_2 0) (== _index_2 _returnvalue_2))) :`false` true :`true` (`KismetMathLibrary.RandomBoolWithWeight` 0.5))
        (`InstancedStaticMeshComponent.AddInstanceWorldSpace` (`self.HISM_Tile`) (`KismetMathLibrary.MakeTransform` (+ (+ (`SceneComponent.K2_GetComponentLocation` _arrowbackleft) (* (`SceneComponent.GetRightVector` _arrowbackleft) (+ (* _index_2 _onetilelength) (/ _onetilelength 2.0))) (* (`SceneComponent.GetForwardVector` _arrowbackleft) (+ (* _index _onetilelength) (/ _onetilelength 2.0)))) (* (`SceneComponent.GetUpVector` _arrowbackleft) (`KismetMathLibrary.RandomFloatInRange` -5.0 5.0))) (`SceneComponent.K2_GetComponentRotation` _arrowbackleft) (2.0 2.0 2.0)))
        (set `self.NOfTiles` (+ (`self.NOfTiles`) 1))))))

(fn `ToggleCollisions`
  (params (Reactivate :type Boolean))
  (bind _undercube (`self.UnderCube`))
  (bind _undercone (`self.UnderCone`))
  (if Reactivate
    (`PrimitiveComponent.SetCollisionEnabled` _undercube (`self.PlaneInitColl`))
    (`PrimitiveComponent.SetCollisionEnabled` _undercone (`self.PlaneInitColl`))
    (for _array_element (`|MakeArray` (`self.WallBack`) (`self.WallLeft`) (`self.WallRight`) (`self.WallFront`))
      (`PrimitiveComponent.SetCollisionEnabled` _array_element (`self.WallsInitColl`)))
    (else
      (set `self.PlaneInitColl` (`PrimitiveComponent.GetCollisionEnabled` _undercube))
      (`PrimitiveComponent.SetCollisionEnabled` _undercube "NoCollision")
      (`PrimitiveComponent.SetCollisionEnabled` _undercone "NoCollision")
      (set `self.WallsInitColl` (`PrimitiveComponent.GetCollisionEnabled` (`self.WallFront`)))
      (for _array_element_2 (`|MakeArray` (`self.WallBack`) (`self.WallLeft`) (`self.WallRight`) (`self.WallFront`))
        (`PrimitiveComponent.SetCollisionEnabled` _array_element_2 "NoCollision")))))

(fn `UserConstructionScript`
  (`parent.UserConstructionScript`)
  (set `self.GravityCollider` (`self.Box`))
  (`self.Set MID` (`self.SurfaceType`))
  (`self.SetGravityZoneScale` (`self.Plane_Scale`))
  (`SceneComponent.SetRelativeScale3D` (`self.Anchor_OnlyVisual_Selector`) (`KismetMathLibrary.MakeVector` 1.0 1.0 (/ 1.0 (`self.Plane_Scale`))) :!pinned true) ; Normalize OnlyVisual_Selector
  (`self.ConfigureUnderCollisions`)
  (`self.ActivateWallForClonePlane`))