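; BP_Mover is a level-design actor that spins a set of child actors around their yaw axis.
; On BeginPlay it attaches each actor in the ChildActor array to itself, keeping world transforms.
; A timeline named Tick then adds a fixed local yaw rotation to each child on every update, so the step is not scaled by delta time.
; An unconnected timeline chain for sinusoidal right-and-up movement of the actor never runs.
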(event `self.ReceiveBeginPlay`
  (for _array_element (`self.ChildActor`)
    (`self.K2_AttachToActor` _array_element self "None" "KeepWorld" "KeepWorld" "KeepWorld" true))
  (`Timeline|Tick` :!via `PlayFromStart`
    (:`Update`
      (for _array_element_2 (`self.ChildActor`)
        (`self.K2_AddActorLocalRotation` _array_element_2 (`KismetMathLibrary.MakeRotator` 0.0 0.0 1.0) false false)))))

(fn `UserConstructionScript`)