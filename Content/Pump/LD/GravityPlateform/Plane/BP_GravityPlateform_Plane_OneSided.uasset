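; One-sided plane gravity platform that can oscillate in position and rotation around its starting relative transform.
; On BeginPlay, optional move and rotate events start per-axis timelines with random durations and optional random phase.
; The X timelines' updates apply sine offsets to both anchors on all axes, though yaw reads the Y rotation timeline, not Z.
; The construction script normalizes the below-collision anchor's Z scale against PlaneScale.
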(event `self.ReceiveBeginPlay`
  (`parent.ReceiveBeginPlay`)
  (`self.MoveLoc`)
  (`self.MoveRot`))

(event `self.ReceiveTick`
  (params (DeltaSeconds :type "Float (single-precision)"))
  (`parent.ReceiveTick` DeltaSeconds))

(event `MoveRot`
  (bind (_startrot_roll _startrot_pitch _startrot_yaw) (`KismetMathLibrary.BreakRotator` (`self.StartRot`)))
  (bind _oscrot_y (`self.OscRot_Y`))
  (bind _oscrot_x (`self.OscRot_X`))
  (bind _oscrot_z (`self.OscRot_Z`))
  (if (`self.MoveRotation`)
    (set `self.StartRot` (`SceneComponent.RelativeRotation` (`self.AnchorForRotation`)))
    (`|ExecutionSequence`
      (:`then_0`
        (`TimelineComponent.SetTimelineLength` _oscrot_x (`KismetMathLibrary.RandomFloatInRange` (`self.OscRotMinDuration`) (`self.OscRotMaxDuration`)))
        (`TimelineComponent.SetPlaybackPosition` _oscrot_x (select `bool` (`self.RandomInitialRotation`) :`true` (`KismetMathLibrary.RandomFloatInRange` 0.0 (`TimelineComponent.GetTimelineLength` _oscrot_x))) false true)
        (`Timeline|OscRot_X`
          (:`Update`
            (`SceneComponent.K2_SetRelativeRotation` (`self.AnchorForRotation`) (`KismetMathLibrary.MakeRotator` (`self.GetDynamicRotAxisValue` (`self.OscRot_X`) (`self.DeltaRotationX`) _startrot_roll) (`self.GetDynamicRotAxisValue` (`self.OscRot_Y`) (`self.DeltaRotationY`) _startrot_pitch) (`self.GetDynamicRotAxisValue` (`self.OscRot_Y`) (`self.DeltaRotationZ`) _startrot_yaw)) false false)
            (`SceneComponent.K2_SetRelativeRotation` (`self.Anchor_BelowColl`) (`KismetMathLibrary.MakeRotator` (`self.GetDynamicRotAxisValue` (`self.OscRot_X`) (`self.DeltaRotationX`) _startrot_roll) (`self.GetDynamicRotAxisValue` (`self.OscRot_Y`) (`self.DeltaRotationY`) _startrot_pitch) (`self.GetDynamicRotAxisValue` (`self.OscRot_Y`) (`self.DeltaRotationZ`) _startrot_yaw)) false false))))
      (:`then_1`
        (`TimelineComponent.SetTimelineLength` _oscrot_y (`KismetMathLibrary.RandomFloatInRange` (`self.OscRotMinDuration`) (`self.OscRotMaxDuration`)))
        (`TimelineComponent.SetPlaybackPosition` _oscrot_y (select `bool` (`self.RandomInitialRotation`) :`true` (`KismetMathLibrary.RandomFloatInRange` 0.0 (`TimelineComponent.GetTimelineLength` _oscrot_y))) false true)
        (`Timeline|OscRot_Y`))
      (:`then_2`
        (`TimelineComponent.SetTimelineLength` _oscrot_z (`KismetMathLibrary.RandomFloatInRange` (`self.OscRotMinDuration`) (`self.OscRotMaxDuration`)))
        (`TimelineComponent.SetPlaybackPosition` _oscrot_z (select `bool` (`self.RandomInitialRotation`) :`true` (`KismetMathLibrary.RandomFloatInRange` 0.0 (`TimelineComponent.GetTimelineLength` _oscrot_z))) false true)
        (`Timeline|OscRot_Z`)))))

(event `MoveLoc`
  (bind _oscloc_z (`self.OscLoc_Z`))
  (bind _oscloc_x (`self.OscLoc_X`))
  (bind _oscloc_y (`self.OscLoc_Y`))
  (bind (_startloc_x _startloc_y _startloc_z) (`KismetMathLibrary.BreakVector` (`self.StartLoc`)))
  (if (`self.MoveLocation`)
    (set `self.StartLoc` (`SceneComponent.RelativeLocation` (`self.AnchorForRotation`)))
    (`|ExecutionSequence`
      (:`then_0`
        (`TimelineComponent.SetTimelineLength` _oscloc_x (`KismetMathLibrary.RandomFloatInRange` (`self.OscLocMinDuration`) (`self.OscLocMaxDuration`)))
        (`TimelineComponent.SetPlaybackPosition` _oscloc_x (select `bool` (`self.RandomInitialLocation`) :`true` (`KismetMathLibrary.RandomFloatInRange` 0.0 (`TimelineComponent.GetTimelineLength` _oscloc_x))) false true)
        (`Timeline|OscLoc_X`
          (:`Update`
            (`SceneComponent.K2_SetRelativeLocation` (`self.AnchorForRotation`) (`KismetMathLibrary.MakeVector` (`self.GetDynamicLocAxisValue` (`self.OscLoc_X`) (`self.DeltaLocX`) _startloc_x) (`self.GetDynamicLocAxisValue` (`self.OscLoc_Y`) (`self.DeltaLocY`) _startloc_y) (`self.GetDynamicLocAxisValue` (`self.OscLoc_Z`) (`self.DeltaLocZ`) _startloc_z)) false false)
            (`SceneComponent.K2_SetRelativeLocation` (`self.Anchor_BelowColl`) (`KismetMathLibrary.MakeVector` (`self.GetDynamicLocAxisValue` (`self.OscLoc_X`) (`self.DeltaLocX`) _startloc_x) (`self.GetDynamicLocAxisValue` (`self.OscLoc_Y`) (`self.DeltaLocY`) _startloc_y) (`self.GetDynamicLocAxisValue` (`self.OscLoc_Z`) (`self.DeltaLocZ`) _startloc_z)) false false))))
      (:`then_1`
        (`TimelineComponent.SetTimelineLength` _oscloc_y (`KismetMathLibrary.RandomFloatInRange` (`self.OscLocMinDuration`) (`self.OscLocMaxDuration`)))
        (`TimelineComponent.SetPlaybackPosition` _oscloc_y (select `bool` (`self.RandomInitialLocation`) :`true` (`KismetMathLibrary.RandomFloatInRange` 0.0 (`TimelineComponent.GetTimelineLength` _oscloc_y))) false true)
        (`Timeline|OscLoc_Y`))
      (:`then_2`
        (`TimelineComponent.SetTimelineLength` _oscloc_z (`KismetMathLibrary.RandomFloatInRange` (`self.OscLocMinDuration`) (`self.OscLocMaxDuration`)))
        (`TimelineComponent.SetPlaybackPosition` _oscloc_z (select `bool` (`self.RandomInitialLocation`) :`true` (`KismetMathLibrary.RandomFloatInRange` 0.0 (`TimelineComponent.GetTimelineLength` _oscloc_z))) false true)
        (`Timeline|OscLoc_Z`)))))

(fn `GetDynamicLocAxisValue`
  (params (Timeline :type "TimelineComponent Object Reference") (DeltaLocValue :type "Float (double-precision)") (StartLocValue :type "Float (double-precision)"))
  (returns (ReturnValue :type "Float (double-precision)"))
  (return (+ StartLocValue (* (`KismetMathLibrary.Sin` (* (`/Game/Pump/Core/BP_FunctionLibrary.GetTimelinePercentage` Timeline) (`KismetMathLibrary.GetPI`) 2.0)) DeltaLocValue))))

(fn `GetDynamicRotAxisValue`
  (params (OscTimeline :type "TimelineComponent Object Reference") (DeltaRotValue :type "Float (double-precision)") (StartRotValue :type "Float (double-precision)"))
  (returns (ReturnValue :type "Float (double-precision)"))
  (return (+ StartRotValue (* (`KismetMathLibrary.Sin` (* (`/Game/Pump/Core/BP_FunctionLibrary.GetTimelinePercentage` OscTimeline) (`KismetMathLibrary.GetPI`) 2.0)) DeltaRotValue))))

(fn `UserConstructionScript`
  (`parent.UserConstructionScript`)
  ;[1 1 1] Normalize BelowColl
  (`SceneComponent.SetRelativeScale3D` (`self.Anchor_BelowColl`) (`KismetMathLibrary.MakeVector` 1.0 1.0 (/ 1.0 (`self.Plane_Scale`)))))