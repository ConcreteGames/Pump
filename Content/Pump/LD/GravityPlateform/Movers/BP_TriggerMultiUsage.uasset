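; Multi-purpose level-design trigger volume that applies scripted game changes when the gravity character enters it.
; Begin overlap runs a sequence of independent actions, each gated by an Edit flag: player movement, camera and controls, time dilation, fog and bloom, asset cleanup, level unloading, tutorials and mover triggers.
; Most actions reach their targets through class searches or the player reference, with bloom blended by timeline.
; End overlap can only change the jump permission.
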(event `self.Collider.OnComponentBeginOverlap`
  (params (OverlappedComponent :type "PrimitiveComponent Object Reference") (OtherActor :type "Actor Object Reference") (OtherComp :type "PrimitiveComponent Object Reference") (OtherBodyIndex :type Integer) (bFromSweep :type Boolean) (SweepResult :type "HitResult Structure (by ref)"))
  (bind _character (`/Game/Pump/Core/BP_FunctionLibrary.GetCharMatter`))
  (bind _t_bloom (`self.T_Bloom`))
  (bind _tutotype (`self.TutoType`))
  (bind _myclone (`/Game/Pump/Core/Character/BP_GravityCharacter_Pump.MyClone` (`self.pChar`)))
  (bind _asbp_gravity_character_pump (cast `/Game/Pump/Core/Character/BP_GravityCharacter_Pump` OtherActor))
  (set `self.pChar` _asbp_gravity_character_pump)
  (if (`self.BEGIN_DoOnce`)
    (`/Engine/EditorBlueprintResources/StandardMacros.DoOnce` false
      (:`Completed`
        _)))
  (`|ExecutionSequence`
    (:`then_0`
      (if (`self.--Edit--SetFinalSkySpheres`)
        (bind _outactors (`GameplayStatics.GetAllActorsOfClass` "/Game/Pump/LD/Environnement/Lights/BP_SkySphere.BP_SkySphere_C"))
        (for _array_element _outactors
          (if (`self.ActorHasTag` _array_element "2")
            (`/Game/Pump/Core/BP_FunctionLibrary.LogErer` (`KismetSystemLibrary.GetDisplayName` _array_element) "Hide")
            (`self.SetActorHiddenInGame` _array_element false)
            (else
              (`/Game/Pump/Core/BP_FunctionLibrary.LogErer` (`KismetSystemLibrary.GetDisplayName` _array_element) "Destroy")
              (`self.K2_DestroyActor` _array_element))))))
    (:`then_1`
      (if (`self.--Edit--GodMode`)
        (set `/Game/Pump/Core/Character/BP_GravityCharacter_Pump.GodMode` (`self.GodMode`) (`self.pChar`))))
    (:`then_2`
      (if (`self.--Edit--CanJump`)
        (set `/Game/Pump/Core/Character/BP_GravityCharacter_Pump.CanJump` (`self.CanJump`) (`self.pChar`))))
    (:`then_3`
      (if (`self.--Edit--CharSpeed`)
        (set `/Game/Pump/Core/Character/BP_GravityCharacter_Pump.WalkMaxSpeed` (select `bool` (`self.CharSpeedResetDefault`) :`false` (`self.WalkMaxSpeed`) :`true` 745.0) _myclone)
        (set `/Game/Pump/Core/Character/BP_GravityCharacter_Pump.WalkAcceleration` (select `bool` (`self.CharSpeedResetDefault`) :`false` (`self.WalkAcceleration`) :`true` 6000.0) _myclone)))
    (:`then_4`
      (if (`self.--Edit--TimeDilation`)
        (`GameplayStatics.SetGlobalTimeDilation` (`self.TimeDilation`))))
    (:`then_5`
      (if (`self.--Edit--FogDensity`)
        (bind _outactors_2 (`GameplayStatics.GetAllActorsOfClass` "/Script/Engine.ExponentialHeightFog"))
        (bind _output (`|GetArrayItem` _outactors_2))
        (`ExponentialHeightFogComponent.SetFogDensity` (`ExponentialHeightFog.Component` _output) (`self.FogDensity`))
        ;[1 1 1] test, mais on dirait que ça fait rien
        (`ExponentialHeightFogComponent.SetVolumetricFogExtinctionScale` (`ExponentialHeightFog.Component` _output) 0.0)))
    (:`then_6`
      (if (`self.--Edit--FinalCleanAssets`)
        (`|ExecutionSequence`
          (:`then_0`
            (bind _outactors_3 (`GameplayStatics.GetAllActorsOfClass` "/Game/Pump/BadPaul/LevelBuildingRessources/Clouds/BP_Cloud.BP_Cloud_C"))
            (for _array_element_2 _outactors_3
              (`self.SetActorHiddenInGame` _array_element_2 true)
              (`self.K2_DestroyActor` _array_element_2)))
          (:`then_1`
            (bind _outactors_4 (`GameplayStatics.GetAllActorsOfClass` "/Game/Pump/LD/FlyingRocksSpawner/BP_SlineSpawner_BigRocks.BP_SlineSpawner_BigRocks_C"))
            (for _array_element_3 _outactors_4
              (`self.SetActorHiddenInGame` _array_element_3 true)))
          (:`then_2`
            (`self.DestroyLongPlateform`)
            (bind _outactors_5 (`GameplayStatics.GetAllActorsOfClass` "/Game/Pump/LD/GravityPlateform/Plane/BP_CubesInAirManager.BP_CubesInAirManager_C"))
            (`InstancedStaticMeshComponent.ClearInstances` (`/Game/Pump/LD/GravityPlateform/Plane/BP_CubesInAirManager.HISM_CubeInAir_2` (`|GetArrayItem` _outactors_5)))
            (`InstancedStaticMeshComponent.ClearInstances` (`/Game/Pump/LD/GravityPlateform/Plane/BP_CubesInAirManager.HISM_CubeInAir_1` (`|GetArrayItem` _outactors_5)))
            (`InstancedStaticMeshComponent.ClearInstances` (`/Game/Pump/LD/GravityPlateform/Plane/BP_CubesInAirManager.HISM_CubeInAir_3` (`|GetArrayItem` _outactors_5)))
            (`InstancedStaticMeshComponent.ClearInstances` (`/Game/Pump/LD/GravityPlateform/Plane/BP_CubesInAirManager.HISM_CubeInAir_Full` (`|GetArrayItem` _outactors_5))))
          (:`then_3`
            (bind _outactors_6 (`GameplayStatics.GetAllActorsOfClass` "/Game/Pump/LD/GravityPlateform/Sphere/Steps/BP_GravityPlateform_Sphere_Step_3.BP_GravityPlateform_Sphere_Step_3_C"))
            (bind _output_2 (`|GetArrayItem` _outactors_6))
            (`/Engine/EditorBlueprintResources/StandardMacros.IsValid` _output_2
              (:`Is Valid`
                (`/Game/Pump/LD/GravityPlateform/Sphere/Steps/BP_GravityPlateform_Sphere_Step_3.SetMeshesCastShadow` _output_2 false)))))))
    (:`then_7`
      (if (`self.--Edit--Bloom`)
        (set `self.InitialBloom` (`/Game/Pump/Core/Character/BP_GravityCharacter_Pump.PP_MaxBloomIntensity` (`self.pChar`)))
        (`TimelineComponent.SetTimelineLength` _t_bloom 10.0)
        (`Timeline|T_Bloom` :!via `PlayFromStart`
          (:`Update`
            (set `/Game/Pump/Core/Character/BP_GravityCharacter_Pump.PP_MaxBloomIntensity` (`KismetMathLibrary.Lerp` (`self.InitialBloom`) (`self.Bloom`) (`/Game/Pump/Core/BP_FunctionLibrary.GetTimelinePercentage` _t_bloom)) (`self.pChar`))))))
    (:`then_8`
      (if (`self.--Edit--ReduceLastPlanetRadius`)
        (bind _outactors_7 (`GameplayStatics.GetAllActorsOfClass` "/Game/Pump/LD/GravityPlateform/Sphere/BP_GravityPlateform_Sphere.BP_GravityPlateform_Sphere_C"))
        (for _array_element_4 _outactors_7
          (`SphereComponent.SetSphereRadius` (`/Game/Pump/LD/GravityPlateform/Sphere/BP_GravityPlateform_Sphere.SphereCollision` _array_element_4) 1.0 false))))
    (:`then_9`
      (if (`self.--Edit--FullMoonTest`)
        (bind _outactors_8 (`GameplayStatics.GetAllActorsOfClass` "/Game/Pump/LD/TutoTriggers/BP_EndingManager.BP_EndingManager_C"))
        (set `/Game/Pump/LD/TutoTriggers/BP_EndingManager.TestFullMoon` true (`|GetArrayItem` _outactors_8))))
    (:`then_10`
      (if (`self.--Edit--KillSpeedParticles`)
        (`SceneComponent.SetHiddenInGame` (`/Game/Pump/Core/Character/BP_GravityCharacter_Pump.SpeedParticle` (`/Game/Pump/Core/BP_FunctionLibrary.GetCharMatter`)) true false)))
    (:`then_11`
      (if (`self.--Edit--SmoothCam`)
        (set `/Game/Pump/Core/Character/BP_GravityCharacter_Pump.CameraSmooth` (`self.CameraSmooth`) _character)
        (set `/Game/Pump/Core/Character/BP_GravityCharacter_Pump.AxisValueMultiplicatorByTriggerMultiUsage` (`self.AxisValueMultiplicator`) _character)))
    (:`then_12`
      (if (`self.--Edit--HideCloudIntro`)
        (bind _outactors_9 (`GameplayStatics.GetAllActorsOfClass` "/Game/Pump/BadPaul/LevelBuildingRessources/Clouds/BP_Cloud.BP_Cloud_C"))
        (for _array_element_5 _outactors_9
          (if (`self.ActorHasTag` _array_element_5 "cloud9")
            (`self.SetActorHiddenInGame` _array_element_5 true)
            (`self.SetLifeSpan` _array_element_5 0.01)))))
    (:`then_13`
      (if (`self.--Edit--EnableReverse`)
        (set `/Game/Pump/Core/Character/BP_GravityCharacter_Pump.IntroIsOver` true (`/Game/Pump/Core/BP_FunctionLibrary.GetCharMatter`))))
    (:`then_14`
      (if (`self.--Edit--ActivateRollerCoaster`)
        (`KismetSystemLibrary.Delay` 0.3)
        (`/Game/Pump/LD/GravityPlateform/Movers/BP_SplineMover.StartNavette` (`self.RollerCoasterSpline`))))
    (:`then_15`
      (if (`self.--Edit--InventoryAllPF`)
        (bind _outactors_10 (`GameplayStatics.GetAllActorsOfClass` "/Game/Pump/Core/BP_NextPFManager.BP_NextPFManager_C"))
        (`/Game/Pump/Core/BP_NextPFManager.InventoryAllPF` (`|GetArrayItem` _outactors_10))))
    (:`then_16`
      (if (`self.--Edit--MoveToActorModifier`)
        (`/Game/Pump/LD/GravityPlateform/Movers/BP_MoveToActor.OrderMoveToActor` (`self.MoveToActorToEdit`) (`self.IDToGo`))))
    (:`then_17`
      (if (`self.--Edit--DisplayATuto`)
        (`KismetSystemLibrary.Delay` (`self.DelayBeforeShowingTuto`))
        (bind _foundwidgets (`WidgetBlueprintLibrary.GetAllWidgetsOfClass` "/Game/Pump/UI/UI_TutoWidget.UI_TutoWidget_C"))
        (bind _output_3 (`|GetArrayItem` _foundwidgets))
        (`/Engine/EditorBlueprintResources/StandardMacros.IsValid` _output_3
          (:`Is Valid`
            (`/Game/Pump/UI/UI_TutoWidget.DisplayTuto` _output_3 _tutotype 0.0)
            (if (`|EnumEquality` _tutotype "NewEnumerator5")
              (set `/Game/Pump/Core/Character/BP_GravityCharacter_Pump.NeedToTestKillMoveTuto` true (`/Game/Pump/Core/BP_FunctionLibrary.GetCharMatter`)))))))
    (:`then_18`
      (if (`self.--Edit--UnloadLevels`)
        (for _array_element_6 (`self.LevelsToUnload`)
          (`GameplayStatics.UnloadStreamLevel` _array_element_6))))
    (:`then_19`
      (if (`self.--Edit--UnBlockControls`)
        (set `/Game/Pump/Core/BP_GameInstance.BlockControls` false (`/Game/Pump/Core/BP_FunctionLibrary.GetGI`))))))

(event `self.Collider.OnComponentEndOverlap`
  (params (OverlappedComponent :type "PrimitiveComponent Object Reference") (OtherActor :type "Actor Object Reference") (OtherComp :type "PrimitiveComponent Object Reference") (OtherBodyIndex :type Integer))
  (bind _asbp_gravity_character_pump (cast `/Game/Pump/Core/Character/BP_GravityCharacter_Pump` OtherActor))
  (set `self.pChar` _asbp_gravity_character_pump)
  (if (`self.END_DoOnce`)
    (`/Engine/EditorBlueprintResources/StandardMacros.DoOnce` false
      (:`Completed`
        _)))
  (if (`self.END_--Edit--CanJump`)
    (set `/Game/Pump/Core/Character/BP_GravityCharacter_Pump.CanJump` (`self.END_CanJum`) (`self.pChar`))))

(fn `UserConstructionScript`
  (`SceneComponent.SetWorldScale3D` (`self.Selector`) (10.0 100.0 100.0)))