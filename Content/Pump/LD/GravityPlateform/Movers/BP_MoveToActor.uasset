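; BP_MoveToActor is a mover that travels to target actors from an indexed list, triggered by sphere overlap or by an order giving the index.
; A timeline scaled to MovementDuration interpolates location along an inverted float curve, teleporting without sweep and snapping to the target at the end.
; A DoOnce blocks retriggering until arrival, when the index advances or wraps to zero.
; An invalid target logs an error and leaves the gate closed.
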(event `OrderMoveToActor`
  (params (IDToGo :type Integer))
  (bind _output (`|GetArrayItem` (`self.NewActorToGoOn`) (`self.ID`)))
  (bind _returnvalue (`self.K2_GetActorLocation` _output))
  (set `self.ID` IDToGo)
  (`/Engine/EditorBlueprintResources/StandardMacros.DoOnce` false :!label _label
    (:`Completed`
      (set `self.LocatioAtMovementStart` (`self.K2_GetActorLocation`))
      (`/Engine/EditorBlueprintResources/StandardMacros.IsValid` _output
        (:`Is Valid`
          (`TimelineComponent.SetTimelineLength` (`self.T_Movement`) (`self.MovementDuration`))
          (`Timeline|T_Movement` :!via `PlayFromStart`
            (:`Update`
              (`self.K2_SetActorLocation` (`KismetMathLibrary.VLerp` (`self.LocatioAtMovementStart`) _returnvalue (- 1.0 (`CurveFloat.GetFloatValue` (`self.CRV_MoveOnce`) (`/Game/Pump/Core/BP_FunctionLibrary.GetTimelinePercentage` (`self.T_Movement`))))) false true))
            (:`Finished`
              ;[1 1 1] secu
              (`self.K2_SetActorLocation` _returnvalue false true)
              (`self.Ready`)
              (set `self.ID` (+ (`self.ID`) 1))
              ;[1 1 1] reset
              (`/Engine/EditorBlueprintResources/StandardMacros.IsValid` (`|GetArrayItem` (`self.NewActorToGoOn`) (`self.ID`))
                (:`Is Not Valid`
                  (set `self.ID` 0))))))
        (:`Is Not Valid`
          (`/Game/Pump/Core/BP_FunctionLibrary.LogErerror` "Y'a rien dans le MoveToActor"))))))

(event `CollideThenMoveToActor`
  (goto _label))

(event `self.SphereColl.OnComponentBeginOverlap`
  (params (OverlappedComponent :type "PrimitiveComponent Object Reference") (OtherActor :type "Actor Object Reference") (OtherComp :type "PrimitiveComponent Object Reference") (OtherBodyIndex :type Integer) (bFromSweep :type Boolean) (SweepResult :type "HitResult Structure (by ref)"))
  (`self.CollideThenMoveToActor`))

(event `Ready`
  (goto _label :!via `Reset`))

(fn `UserConstructionScript`
  (set `self.InitBTransform` (`self.GetTransform`)))