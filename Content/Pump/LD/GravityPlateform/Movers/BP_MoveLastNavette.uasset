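; BP_MoveLastNavette is a mover that slides the last shuttle once to an editable end point while warping game speed.
; MoveOnce fires a single time, stretches a timeline to MovementDuration, and teleports the actor along a float curve toward the End component.
; A second curve drives global time dilation during the move; on finish it snaps to the target and restores normal speed.
; The construction script places and scales End from exposed values.
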(event `MoveOnce`
  (bind _targetlocation (`self.TargetLocation`))
  (`/Engine/EditorBlueprintResources/StandardMacros.DoOnce` false
    (:`Completed`
      (set `self.LocatioAtMovementStart` (`self.K2_GetActorLocation`))
      (set `self.TargetLocation` (`SceneComponent.K2_GetComponentLocation` (`self.End`)))
      (`TimelineComponent.SetTimelineLength` (`self.T_Movement`) (`self.MovementDuration`))
      (`Timeline|T_Movement` :!via `PlayFromStart`
        (:`Update`
          (`self.K2_SetActorLocation` (`KismetMathLibrary.VLerp` (`self.LocatioAtMovementStart`) _targetlocation (`CurveFloat.GetFloatValue` (`self.CRV_MoveLastNavette`) (`/Game/Pump/Core/BP_FunctionLibrary.GetTimelinePercentage` (`self.T_Movement`)))) false true)
          (`GameplayStatics.SetGlobalTimeDilation` (`CurveFloat.GetFloatValue` (`self.CRV_LastNavetteTimeDilation`) (`/Game/Pump/Core/BP_FunctionLibrary.GetTimelinePercentage` (`self.T_Movement`)))))
        (:`Finished`
          ;[1 1 1] secu
          (`self.K2_SetActorLocation` _targetlocation false true)
          (`GameplayStatics.SetGlobalTimeDilation` 1.0))))))

(fn `UserConstructionScript`
  (bind _end (`self.End`))
  (bind _endlocationarrowscale (`self.EndLocationArrowScale`))
  (`SceneComponent.K2_SetRelativeLocation` _end (`self.EndLocation`) false false)
  (`SceneComponent.SetWorldScale3D` _end (`KismetMathLibrary.MakeVector` _endlocationarrowscale _endlocationarrowscale _endlocationarrowscale)))