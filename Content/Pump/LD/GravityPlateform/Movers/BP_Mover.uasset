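; BP_Mover is a level-design mover actor that continuously rotates itself and the actors listed in its ChildActor array.
; On BeginPlay it attaches those actors keeping world transforms, then starts a Tick timeline that adds a scaled local rotation each update with teleport.
; An unconnected second timeline holds sine-based back-and-forth movement along the right and up vectors, which never runs.
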(event `self.ReceiveBeginPlay`
  (for _array_element (`self.ChildActor`)
    (`self.K2_AttachToActor` _array_element self "None" "KeepWorld" "KeepWorld" "KeepWorld" true))
  (`Timeline|Tick` :!via `PlayFromStart`
    (:`Update`
      (`self.K2_AddActorLocalRotation` (* (`self.Rotation/100`) 0.01) false true))))

(fn `UserConstructionScript`)