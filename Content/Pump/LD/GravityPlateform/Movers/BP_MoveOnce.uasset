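; BP_MoveOnce is a level mover that starts offset from its placed transform and travels back to it once when MoveOnce is called.
; The construction script caches the placed transform, and BeginPlay shifts the actor by LocationToAddAdStart.
; A DoOnce-guarded timeline, sized to MovementDuration, scales that offset with a float curve, then snaps to the placed location on finish.
; DevDisableMovement disables both the initial shift and the move.
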(event `self.ReceiveBeginPlay`
  (bind _initbtransform_location (`KismetMathLibrary.BreakTransform` (`self.InitBTransform`)))
  (if (not (`self.Dev_DisableMovement`))
    (`self.K2_SetActorLocation` (+ _initbtransform_location (`self.LocationToAddAdStart`)))))

(event `MoveOnce`
  (bind _initbtransform_location (`KismetMathLibrary.BreakTransform` (`self.InitBTransform`)))
  (bind _movementduration (`self.MovementDuration`))
  (bind _initbtransform_location_2 (`KismetMathLibrary.BreakTransform` (`self.InitBTransform`)))
  (if (not (`self.Dev_DisableMovement`))
    (`/Engine/EditorBlueprintResources/StandardMacros.DoOnce` false
      (:`Completed`
        (set `self.LocatioAtMovementStart` (`self.K2_GetActorLocation`))
        (`TimelineComponent.SetTimelineLength` (`self.T_Movement`) _movementduration)
        (`/Game/Pump/Core/BP_FunctionLibrary.LogErer` "BP_MoveOnce start movement, duration: " (`KismetStringLibrary.Conv_DoubleToString` _movementduration))
        (`Timeline|T_Movement` :!via `PlayFromStart`
          (:`Update`
            (`self.K2_SetActorLocation` (+ _initbtransform_location (* (`self.LocationToAddAdStart`) (`CurveFloat.GetFloatValue` (`self.CRV_MoveOnce`) (`/Game/Pump/Core/BP_FunctionLibrary.GetTimelinePercentage` (`self.T_Movement`))))) false true))
          (:`Finished`
            ;[1 1 1] secu
            (`self.K2_SetActorLocation` _initbtransform_location_2 false true)))))))

(fn `UserConstructionScript`
  (set `self.InitBTransform` (`self.GetTransform`)))