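; BP_MoveToActor_ChildLvl2 is a child gravity-platform mover that overrides the collide-then-move-to-actor event.
; After running the parent logic, it loops over its attached actors and teleports each to a relative location read from a Distance entry indexed by ID.
; It logs the order and each actor's name and offset along the way.
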(event `self.CollideThenMoveToActor`
  (bind _output (`|GetArrayItem` (`self.Distance`) (`self.ID`)))
  (`parent.CollideThenMoveToActor`)
  (`/Game/Pump/Core/BP_FunctionLibrary.LogErer` "Order Move to Actor")
  (for _array_element (`self.AttachedActors`)
    (`/Game/Pump/Core/BP_FunctionLibrary.LogErer` (`KismetSystemLibrary.GetDisplayName` _array_element) (`KismetStringLibrary.Conv_VectorToString` _output))
    (`self.K2_SetActorRelativeLocation` _array_element _output false true)))

(fn `UserConstructionScript`
  (`parent.UserConstructionScript`))