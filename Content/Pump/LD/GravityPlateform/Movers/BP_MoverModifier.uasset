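; BP_MoverModifier is a trigger box that eases the Rotation100 of the first BP_Mover in its list toward FinalRotation.
; On first overlap it stops the other listed modifiers, re-arming their DoOnce, then runs a timeline of configurable duration shaped by an ease-in curve.
; It also optionally swaps music events or drives sound parameters on Bp_SoundSystem along that curve, with a step parameter at completion.
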(event `self.ReceiveBeginPlay`
  (bind _outactors (`GameplayStatics.GetAllActorsOfClass` "/Game/Pump/Core/SoundSystem/Bp_SoundSystem.Bp_SoundSystem_C"))
  (set `self.PSoundManager` (`|GetArrayItem` _outactors)))

(event `self.Box.OnComponentBeginOverlap`
  (params (OverlappedComponent :type "PrimitiveComponent Object Reference") (OtherActor :type "Actor Object Reference") (OtherComp :type "PrimitiveComponent Object Reference") (OtherBodyIndex :type Integer) (bFromSweep :type Boolean) (SweepResult :type "HitResult Structure (by ref)"))
  (bind _psoundmanager (`self.PSoundManager`))
  (bind _returnvalue (`CurveFloat.GetFloatValue` (`self.CRV_EaseIn`) (`/Game/Pump/Core/BP_FunctionLibrary.GetTimelinePercentage` (`self.TTT`))))
  (bind _returnvalue_2 (select `bool` (`self.DropSoundInvert`) :`false` _returnvalue :`true` (`KismetMathLibrary.MapRangeClamped` _returnvalue 0.0 1.0 1.0)))
  (`/Engine/EditorBlueprintResources/StandardMacros.DoOnce` false :!label _label
    (:`Completed`
      (`self.SwapSoundFunction`)
      (`self.StopOtherMoverModifiers`)
      (`TimelineComponent.SetTimelineLength` (`self.TTT`) (`self.ModificationDuration`))
      (bind _asbp_mover (cast `/Game/Pump/LD/GravityPlateform/Movers/BP_Mover` (`|GetArrayItem` (`self.Movers`))))
      (bind _output_get (set `self.MyMover` _asbp_mover))
      (set `self.MyRotation ` (`/Game/Pump/LD/GravityPlateform/Movers/BP_Mover.Rotation/100` _output_get))
      (`Timeline|TTT` :!via `PlayFromStart` :!label _label_2
        (:`Update`
          (set `/Game/Pump/LD/GravityPlateform/Movers/BP_Mover.Rotation/100` (`KismetMathLibrary.RLerp` (`self.MyRotation `) (`self.FinalRotation`) _returnvalue) (`self.MyMover`))
          (if (`self.ControlsSoundCompEvent`)
            (`self.MusicPlayPauseStop` _psoundmanager "NewEnumerator3" _returnvalue_2 (`self.DropSoundParameter`))
            (elif (`self.ChangeSwapParameter`)
              (`/Game/Pump/Core/SoundSystem/Bp_SoundSystem.SwapEventFor2D` _psoundmanager "NewEnumerator3" null true null (`self.DropSoundParameter`) _returnvalue_2))))
        (:`Finished`
          (set `/Game/Pump/LD/GravityPlateform/Movers/BP_Mover.Rotation/100` (`self.FinalRotation`) (`self.MyMover`))
          (if (`self.ControlsSoundCompEvent`)
            (`self.MusicPlayPauseStop` (`self.PSoundManager`) "NewEnumerator3" (`self.StepSoundParameterValue`) (`self.StepSoundParameter`))))))))

(event `StopMove`
  (`|ExecutionSequence`
    (:`then_0`
      (goto _label_2 :!via `Stop`))
    (:`then_1`
      (goto _label :!via `Reset`))))

(event `self.Box.OnComponentEndOverlap`
  (params (OverlappedComponent :type "PrimitiveComponent Object Reference") (OtherActor :type "Actor Object Reference") (OtherComp :type "PrimitiveComponent Object Reference") (OtherBodyIndex :type Integer))
  (set `self.SwapEvent` false))

(fn `StopOtherMoverModifiers`
  (for _array_element (`self.OtherModifiersToStop`)
    (`self.StopMove` _array_element)))

(fn `SwapSoundFunction`
  (bind _psoundmanager (`self.PSoundManager`))
  (if (`self.SwapEvent`)
    (`/Game/Pump/Core/SoundSystem/Bp_SoundSystem.SwapEventFor2D` _psoundmanager "NewEnumerator5" "/Game/FMOD/Events/Music/2DMusic/Chapitre02/M_Ch02_SpecialTunnel.M_Ch02_SpecialTunnel" true null "None" 0.0)
    (elif (`self.SwapParameter`)
      (`/Game/Pump/Core/SoundSystem/Bp_SoundSystem.MusicPlayPauseStop` _psoundmanager "NewEnumerator3" (`self.SwapParameterValue`) (`self.SwapParameterName`)))))

(fn `UserConstructionScript`
  (`SceneComponent.SetWorldScale3D` (`self.AnchorScale`) (`self.ColliderScale`)))