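; BP_TriggerSetTimeDilation is a one-shot trigger volume that sets global time dilation when the gravity character overlaps its collider.
; With End set, it also enables the character's god mode, unloads the Chapter 3 planet-step streaming level, and hides rock spawners, gravity platforms, clouds and height fog.
; With SuperVitesse set, it sharply raises the walk speed and acceleration of the character's MyClone.
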(event `self.Collider.OnComponentBeginOverlap`
  (params (OverlappedComponent :type "PrimitiveComponent Object Reference") (OtherActor :type "Actor Object Reference") (OtherComp :type "PrimitiveComponent Object Reference") (OtherBodyIndex :type Integer) (bFromSweep :type Boolean) (SweepResult :type "HitResult Structure (by ref)"))
  (`/Game/Pump/Core/BP_FunctionLibrary.LogErer` (`KismetSystemLibrary.GetDisplayName` self))
  (bind _asbp_gravity_character_pump (cast `/Game/Pump/Core/Character/BP_GravityCharacter_Pump` OtherActor))
  (`/Engine/EditorBlueprintResources/StandardMacros.DoOnce` false
    (:`Completed`
      (`GameplayStatics.SetGlobalTimeDilation` (`self.TimeDilation`))
      (`|ExecutionSequence`
        (:`then_0`
          (if (`self.End`)
            (set `/Game/Pump/Core/Character/BP_GravityCharacter_Pump.GodMode` true _asbp_gravity_character_pump)
            (`GameplayStatics.UnloadStreamLevel` "Chapter_3_Animal_PlanetStep")
            (`|ExecutionSequence`
              (:`then_0`
                (bind _outactors (`GameplayStatics.GetAllActorsOfClass` "/Game/Pump/LD/FlyingRocksSpawner/BP_SlineSpawner_BigRocks.BP_SlineSpawner_BigRocks_C"))
                (for _array_element _outactors
                  (`self.SetActorHiddenInGame` _array_element true)))
              (:`then_1`
                (bind _outactors_2 (`GameplayStatics.GetAllActorsOfClass` "/Game/Pump/LD/GravityPlateform/BP_GravityPlateform.BP_GravityPlateform_C"))
                (for _array_element_2 _outactors_2
                  (`self.SetActorHiddenInGame` _array_element_2 true)))
              (:`then_2`
                (bind _outactors_3 (`GameplayStatics.GetAllActorsOfClass` "/Game/Pump/BadPaul/LevelBuildingRessources/Clouds/BP_Cloud.BP_Cloud_C"))
                (for _array_element_3 _outactors_3
                  (`self.SetActorHiddenInGame` _array_element_3 true)))
              (:`then_3`
                (bind _outactors_4 (`GameplayStatics.GetAllActorsOfClass` "/Script/Engine.ExponentialHeightFog"))
                (for _array_element_4 _outactors_4
                  (`self.SetActorHiddenInGame` _array_element_4 true))))))
        (:`then_1`
          (if (`self.SuperVitesse`)
            (`/Game/Pump/Core/BP_FunctionLibrary.LogErer` "super vitesse")
            (bind _myclone (`/Game/Pump/Core/Character/BP_GravityCharacter_Pump.MyClone` _asbp_gravity_character_pump))
            (set `/Game/Pump/Core/Character/BP_GravityCharacter_Pump.WalkMaxSpeed` 7450.0 _myclone)
            (set `/Game/Pump/Core/Character/BP_GravityCharacter_Pump.WalkAcceleration` 12000.0 _myclone)))))))

(fn `UserConstructionScript`)