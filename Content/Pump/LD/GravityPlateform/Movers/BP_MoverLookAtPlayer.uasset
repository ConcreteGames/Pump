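; BP_MoverLookAtPlayer is a gravity-platform mover that smoothly turns to face the player's camera.
; Each tick it lerps its rotation toward a look-at rotation, using the character reference cached on BeginPlay.
; When the player overlaps CollOff, it stops ticking unless CantBeDisabled is set, and always stops child BP_Circle actors' ticks.
; The construction script sets CollOff's relative location and world scale from variables.
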(event `self.ReceiveBeginPlay`
  ;[0 1 0.1514] BEGIN PLAY
  (`self.REF_Char`))

(event `self.ReceiveTick`
  (params (DeltaSeconds :type "Float (single-precision)"))
  ;[1 0.836 0] TICK
  (`self.K2_SetActorRotation` (`KismetMathLibrary.RLerp` (`self.K2_GetActorRotation`) (`KismetMathLibrary.FindLookAtRotation` (`self.K2_GetActorLocation`) (`SceneComponent.K2_GetComponentLocation` (`/Game/Pump/Core/Character/BP_GravityCharacter_Pump.Camera` (`self.pChar`)))) 0.15 true)))

(event `self.CollOff.OnComponentBeginOverlap`
  (params (OverlappedComponent :type "PrimitiveComponent Object Reference") (OtherActor :type "Actor Object Reference") (OtherComp :type "PrimitiveComponent Object Reference") (OtherBodyIndex :type Integer) (bFromSweep :type Boolean) (SweepResult :type "HitResult Structure (by ref)"))
  (cast `/Game/Pump/Core/Character/BP_GravityCharacter_Pump` OtherActor)
  (`|ExecutionSequence`
    (:`then_0`
      (if (not (`self.CantBeDisabled`))
        (`self.SetActorTickEnabled` false)))
    (:`then_1`
      (`self.SetChildrenCirclesTickEnable` false))))

(event `SetChildrenCirclesTickEnable`
  (params (bEnabled :type Boolean))
  (for _array_element (`self.GetAllChildActors` false)
    (bind _asbp_circle (cast `/Game/Pump/LD/GravityPlateform/Movers/BP_Circle` _array_element))
    (`self.SetActorTickEnabled` _asbp_circle bEnabled)))

(fn `REF_Char`
  (set `self.pChar` (`/Game/Pump/Core/BP_FunctionLibrary.GetCharMatter`)))

(fn `UserConstructionScript`
  (bind _colloff (`self.CollOff`))
  (`SceneComponent.K2_SetRelativeLocation` _colloff (`self.CollOff_RelativeLocation`) false true)
  (`SceneComponent.SetWorldScale3D` _colloff (`self.CollOff_WorldScale`)))