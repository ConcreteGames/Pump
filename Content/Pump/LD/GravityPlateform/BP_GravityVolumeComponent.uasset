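; Gravity volume component for platforms and planets that applies a prioritized gravity force to the player character's gravity receiver.
; On BeginPlay it caches the character and receiver, matching clone or normal character for one-sided plane platforms.
; ApplyGravityToActorsInCollider acts when the given collider overlaps a gravity character.
; Plane owners pull along a local direction rotated by their anchor; other owners use radial, optionally inverted, planet gravity.
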(event `self.ReceiveBeginPlay`
  (`self.REF_Char`)
  (`self.REF_CharGravityReciever`))

(event `ApplyGravityToActorsInCollider`
  (params (Collider :type "PrimitiveComponent Object Reference"))
  (if (> (`KismetArrayLibrary.Array_Length` (`PrimitiveComponent.GetOverlappingActors` Collider "/Game/Pump/Core/Character/BP_GravityCharacter_Pump.BP_GravityCharacter_Pump_C")) 0)
    (`/Game/Pump/Core/BP_GravityReceiver.ApplyGravity` (`self.pCharGravityReceiver`) (* (`self.CalculateGravityDirection` (`Actor.K2_GetActorLocation` (`self.pChar`)) (`self.GravityType`)) (`self.Force`)) (`self.Priority`) (`self.GetOwner` Collider))))

(fn `CalculateGravityDirection`
  (params (Location :type "Vector Structure") (GravityType :type "/Game/DirectionalGravity/Blueprints/GravityLogic/EGravityType Enum" :default "NewEnumerator0"))
  (returns (Direction :type "Vector Structure"))
  (bind _returnvalue (`self.GetOwner`))
  (bind _asbp_gravity_plateform_plane (cast `/Game/Pump/LD/GravityPlateform/Plane/BP_GravityPlateform_Plane` _returnvalue)
    (:`then`
      (return (`KismetMathLibrary.Normal` (`KismetMathLibrary.GreaterGreater_VectorRotator` (`self.LocalDirection`) (`SceneComponent.K2_GetComponentRotation` (`/Game/Pump/LD/GravityPlateform/Plane/BP_GravityPlateform_Plane.AnchorForRotation` _asbp_gravity_plateform_plane))))))
    (:`CastFailed`
      (return (* (`KismetMathLibrary.Normal` (- (`Actor.K2_GetActorLocation` _returnvalue) Location)) (`KismetMathLibrary.SelectFloat` -1.0 1.0 (`self.InverseGravity`)))))))

(fn `REF_Char`
  (bind _outactors (`GameplayStatics.GetAllActorsOfClass` "/Game/Pump/Core/Character/BP_GravityCharacter_Pump.BP_GravityCharacter_Pump_C"))
  (for _array_element _outactors
    (bind _asbp_gravity_plateform_plane_one_sided (cast `/Game/Pump/LD/GravityPlateform/Plane/BP_GravityPlateform_Plane_OneSided` (`self.GetOwner`))
      (:`then`
        (if (== (`/Game/Pump/Core/Character/BP_GravityCharacter_Pump.IsCLONE` _array_element) (`/Game/Pump/LD/GravityPlateform/BP_GravityPlateform.IsClonePlateform` _asbp_gravity_plateform_plane_one_sided))
          (set `self.pChar` _array_element)))
      (:`CastFailed`
        (set `self.pChar` (`/Game/Pump/Core/BP_FunctionLibrary.GetCharMatter`)) ; Sinon c'est que c'est une planet_step\ndonc pas d'histoire de clone
      ))))

(fn `REF_CharGravityReciever`
  (set `self.pCharGravityReceiver` (`/Game/Pump/Core/Character/BP_GravityCharacter_Pump.GravityReceiver` (`self.pChar`))))