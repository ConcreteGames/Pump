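; Planet gravity platform: a scalable planet mesh inside a spherical gravity field that can be inverted.
; The construction script sizes the sphere and mesh and passes force, priority and inversion to BPGravityVolumeComponent, which applies gravity every tick.
; A Niagara effect visualises the field, deriving spawn rate (unless set manually), sprite size, velocity and lifetime from clamped radius mappings.
; Inversion flips particle direction and halves their spawn radius, while gravity hardness picks the color.
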(event `self.ReceiveBeginPlay`
  (`self.InitParticleValues`))

(event `self.ReceiveTick`
  (params (DeltaSeconds :type "Float (single-precision)"))
  (`/Game/Pump/LD/GravityPlateform/BP_GravityVolumeComponent.ApplyGravity` (`self.BP_GravityVolumeComponent`)))

(fn `InitParticleValues`
  (bind _returnvalue (`self.MapGravitySphereParticleValues` 10.0 100.0))
  (bind _gravitysphereradius (`self.GravitySphereRadius`))
  (bind _particle (`self.Particle`))
  (`NiagaraComponent.SetNiagaraVariableFloat` _particle "User.SphereRadius" (select `bool` (`self.InvertGravity`) :`false` _gravitysphereradius :`true` (/ _gravitysphereradius 2.0)))
  (`NiagaraComponent.SetNiagaraVariableFloat` _particle "User.SpawnRate" (select `bool` (`self.bManualParticleSpawnRate`) :`false` (`self.MapGravitySphereParticleValues` 100.0 10000.0) :`true` (`self.ParticleSpawnRate`)))
  (`NiagaraComponent.SetNiagaraVariableVec2` _particle "User.SpriteSize" (`KismetMathLibrary.MakeVector2D` _returnvalue _returnvalue))
  (`NiagaraComponent.SetNiagaraVariableFloat` _particle "User.Velocity" (select `bool` (`self.InvertGravity`) :`false` (`self.MapGravitySphereParticleValues` -20.0 -100.0) :`true` (`self.MapGravitySphereParticleValues` 20.0 100.0)))
  (`NiagaraComponent.SetNiagaraVariableLinearColor` _particle "User.Color" (select `bool` (`self.bGravityHard`) :`false` (`self.SoftGravityColor`) :`true` (`self.HardGravityColor`)))
  (`NiagaraComponent.SetNiagaraVariableFloat` _particle "User.ParticleLifetime" (`self.MapGravityLifetime` 0.2 7.0)))

(fn `MapGravityLifetime`
  (params (Min :type "Float (double-precision)") (Max :type "Float (double-precision)"))
  (returns (ReturnValue :type "Float (double-precision)"))
  (return (`KismetMathLibrary.MapRangeClamped` (- (`self.GravitySphereRadius`) (`self.PlanetScale`)) (`self.GravitySphereMinRadius`) (`self.GravitySphereMaxRadius`) Min Max)))

(fn `MapGravitySphereParticleValues`
  (params (Min :type "Float (double-precision)") (Max :type "Float (double-precision)"))
  (returns (ReturnValue :type "Float (double-precision)"))
  (return (`KismetMathLibrary.MapRangeClamped` (`self.GravitySphereRadius`) (`self.GravitySphereMinRadius`) (`self.GravitySphereMaxRadius`) Min Max)))

(fn `UserConstructionScript`
  (bind _bp_gravityvolumecomponent (`self.BP_GravityVolumeComponent`))
  (bind _returnvalue (/ (`self.PlanetScale`) 100.0))
  (`SphereComponent.SetSphereRadius` (`self.Sphere`) (`self.GravitySphereRadius`) true)
  (`SceneComponent.SetRelativeScale3D` (`self.PlanetMesh`) (`KismetMathLibrary.MakeVector` _returnvalue _returnvalue _returnvalue))
  (set `/Game/Pump/LD/GravityPlateform/BP_GravityVolumeComponent.Force` (`self.Force`) _bp_gravityvolumecomponent)
  (set `/Game/Pump/LD/GravityPlateform/BP_GravityVolumeComponent.Priority` (`self.Priority`) _bp_gravityvolumecomponent)
  (set `/Game/Pump/LD/GravityPlateform/BP_GravityVolumeComponent.InverseGravity` (`self.InvertGravity`) _bp_gravityvolumecomponent)
  (`self.InitParticleValues`))