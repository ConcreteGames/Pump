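; Gravity platform cube that can carry a gravity volume on any of its six sides and ripples when a character hits it.
; The construction script adds a scaled BP_GravityPlateform_Plane child actor per enabled side, setting its depth, force, direction and priority.
; SpawnAzulejos tiles enabled faces with height-jittered instances in the level's BP_AzulejosManager HISM.
; OnCharacterHit maps impact velocity to wave power, which a timeline feeds into that manager's dynamic material.
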(event `OnCharacterHit`
  (params (Velocity :type "Float (double-precision)"))
  (bind _plateformwavespower (`self.PlateformWavesPower`))
  (bind _mid (`/Game/Pump/LD/GravityPlateform/BP_AzulejosManager.MID` (`self.GetAzulejosManager`)))
  ;[1 1 1] Hit Plateform VFX
  (set `self.PlateformWavesPower` (`KismetMathLibrary.MapRangeClamped` Velocity 500.0 2000.0 1.5 8.0))
  (bind (_direction _cosinepower _distancefromplayer _alpha _vectorlength) (`Timeline|WaveTimeline` :!via `PlayFromStart`)
    (:`Update`
      (`MaterialInstanceDynamic.SetScalarParameterValue` _mid "Cosine" (* _cosinepower (`self.PlateformWavesPower`)))
      (`MaterialInstanceDynamic.SetScalarParameterValue` _mid "DistanceImpact" (* _plateformwavespower 100.0))
      (`MaterialInstanceDynamic.SetScalarParameterValue` _mid "AlphaForImpact" (* _alpha (`KismetMathLibrary.MapRangeClamped` _plateformwavespower 1.5 6.0 0.5 1.0)))
      (bind _returnvalue (* _vectorlength (`KismetMathLibrary.MapRangeClamped` (`self.PlateformWavesPower`) 1.5 6.0 0.5 2.0)))
      (`MaterialInstanceDynamic.SetScalarParameterValue` _mid "VectorLength" _returnvalue)
      (`MaterialInstanceDynamic.SetScalarParameterValue` _mid "VectorLengthEnd" (- _returnvalue (`KismetMathLibrary.MapRangeClamped` (`self.PlateformWavesPower`) 1.5 6.0 (`self.MinWaveSize`) (`self.MaxWaveSize`)))))))

(event `self.ReceiveBeginPlay`)

(fn `DsitanceBetweenArrows`
  (params (ArrowEnd :type "SceneComponent Object Reference") (ArrowStart :type "SceneComponent Object Reference"))
  (returns (ReturnValue :type Integer))
  (return (`KismetMathLibrary.FTrunc` (/ (`KismetMathLibrary.VSize` (- (`SceneComponent.K2_GetComponentLocation` ArrowStart) (`SceneComponent.K2_GetComponentLocation` ArrowEnd))) (`self.TileLenght`)))))

(fn `GetAzulejosManager`
  (returns (AzulejosManager :type "/Game/Pump/LD/GravityPlateform/BP_AzulejosManager Object Reference"))
  (`/Engine/EditorBlueprintResources/StandardMacros.IsValid` (`self.pHISM_Tile`)
    (:`Is Valid`
      (return (stale _output_get)))
    (:`Is Not Valid`
      (bind _outactors (`GameplayStatics.GetAllActorsOfClass` "/Game/Pump/LD/GravityPlateform/BP_AzulejosManager.BP_AzulejosManager_C"))
      (bind _output (`|GetArrayItem` _outactors))
      (`/Engine/EditorBlueprintResources/StandardMacros.IsValid` _output
        (:`Is Valid`
          (bind _output_get (set `self.pAzulejosManager` _output))
          (return _output_get))
        (:`Is Not Valid`
          (`/Game/Pump/Core/BP_FunctionLibrary.LogErerror` "NEED in the LEVEL : BP_AzulejosManager"))))))

(fn `SpawnAzulejos`
  (bind _tilelenght (`self.TileLenght`))
  (bind _tilelenght_2 (`self.TileLenght`))
  (for _index (range (`self.DsitanceBetweenArrows` (`self.ArrowTop_FrontLeft`) (`self.ArrowTop_BackLeft`)))
    (for _index_2 (range (`self.DsitanceBetweenArrows` (`self.ArrowTop_BackRight`) (`self.ArrowTop_BackLeft`)))
      (for _index_3 (range 6)
        (if (`|GetArrayItem` (`self.SpawnGravBoxes`) _index_3)
          (bind _returnvalue (select `int` _index_3 :`0` (`self.ArrowTop_BackLeft`) :`1` (`self.ArrowBot_BackLeft`) :`2` (`self.ArrowCorner1`) :`3` (`self.ArrowCorner2`) :`4` (`self.ArrowCorner3`) :`5` (`self.ArrowCorner4`) :!type "SceneComponent Object Reference"))
          (`InstancedStaticMeshComponent.AddInstanceWorldSpace` (`/Game/Pump/LD/GravityPlateform/BP_AzulejosManager.HISM_Tile` (`self.GetAzulejosManager`)) (`KismetMathLibrary.MakeTransform` (+ (+ (`SceneComponent.K2_GetComponentLocation` _returnvalue) (* (`SceneComponent.GetRightVector` _returnvalue) (+ (* _index_2 _tilelenght) (/ _tilelenght 2.0))) (* (`SceneComponent.GetForwardVector` _returnvalue) (+ (* _index _tilelenght_2) (/ _tilelenght_2 2.0)))) (* (`SceneComponent.GetUpVector` _returnvalue) (`KismetMathLibrary.RandomFloatInRange` -5.0 5.0))) (`SceneComponent.K2_GetComponentRotation` _returnvalue))))))))

(fn `UserConstructionScript`
  (bind _gravboxesscalez (`self.GravBoxesScaleZ`))
  (bind (_returnvalue_location _returnvalue_rotation _returnvalue_scale) (`KismetMathLibrary.BreakTransform` (`SceneComponent.GetRelativeTransform` (`self.ArrowConversion`))))
  (bind (_returnvalue_x _returnvalue_y _returnvalue_z) (`KismetMathLibrary.BreakVector` (`SceneComponent.K2_GetComponentScale` (`self.SM_Cube`))))
  (bind _returnvalue (`KismetMathLibrary.MakeVector` _returnvalue_x _returnvalue_z _returnvalue_y))
  (bind _returnvalue_2 (`KismetMathLibrary.MakeVector` _returnvalue_x _returnvalue_y _returnvalue_z))
  (bind _returnvalue_3 (`KismetMathLibrary.MakeVector` _returnvalue_z _returnvalue_y _returnvalue_x))
  ;[1 1 1] For each sides
  (bind _output_get (set `self.ArrowArray` (`|MakeArray` (`self.Arrow0Top`) (`self.Arrow1Bot`) (`self.Arrow2Front`) (`self.Arrow3Back`) (`self.Arrow4Left`) (`self.Arrow5Right`))))
  (for (_array_element _array_index) _output_get
    ;[1 1 1] If box wanted
    (if (`|GetArrayItem` (`self.SpawnGravBoxes`) _array_index)
      ;[1 1 1] Custom good scale
      (`SceneComponent.SetWorldScale3D` _array_element (select `int` _array_index :`0` _returnvalue_2 :`1` _returnvalue_2 :`2` _returnvalue_3 :`3` _returnvalue_3 :`4` _returnvalue :`5` _returnvalue))
      (bind (_returnvalue_location_2 _returnvalue_rotation_2 _returnvalue_scale_2) (`KismetMathLibrary.BreakTransform` (`SceneComponent.K2_GetComponentToWorld` _array_element)))
      ;[1 1 1] Get relative transform
      (`SceneComponent.K2_SetWorldTransform` (`self.ArrowConversion`) (`KismetMathLibrary.MakeTransform` _returnvalue_location_2 _returnvalue_rotation_2 _returnvalue_scale_2) false false)
      ;[1 1 1] Add GravityCube
      (bind _returnvalue_4 (`AddComponent|NODE_AddChildActorComponent-4` :`RelativeTransform` (`KismetMathLibrary.MakeTransform` _returnvalue_location _returnvalue_rotation _returnvalue_scale)))
      (bind _asbp_gravity_plateform_plane (cast `/Game/Pump/LD/GravityPlateform/Plane/BP_GravityPlateform_Plane` (`ChildActorComponent.ChildActor` _returnvalue_4) :!pure true))
      (bind _rootcomponent (`Actor.RootComponent` _asbp_gravity_plateform_plane))
      (bind (_returnvalue_x_2 _returnvalue_y_2) (`KismetMathLibrary.BreakVector` (`SceneComponent.K2_GetComponentScale` _rootcomponent)))
      (bind _output (`|GetArrayItem` _gravboxesscalez _array_index))
      ;[1 1 1] Override Z Scale
      (`SceneComponent.SetWorldScale3D` _rootcomponent (`KismetMathLibrary.MakeVector` _returnvalue_x_2 _returnvalue_y_2 (select `bool` (!= _output 0.0) :`false` (`|GetArrayItem` _gravboxesscalez) :`true` _output)))
      (bind _bp_gravityvolumecomponent (`/Game/Pump/LD/GravityPlateform/BP_GravityPlateform.BP_GravityVolumeComponent` _asbp_gravity_plateform_plane))
      ;[1 1 1] set Params
      (bind _output_get_2 (set `/Game/Pump/LD/GravityPlateform/BP_GravityVolumeComponent.Force` (`|GetArrayItem` (`self.GravBoxesForce`) _array_index) _bp_gravityvolumecomponent))
      (set `/Game/Pump/LD/GravityPlateform/BP_GravityVolumeComponent.LocalDirection` (`|GetArrayItem` (`self.GravBoxesDirection`) _array_index) _bp_gravityvolumecomponent)
      (set `/Game/Pump/LD/GravityPlateform/BP_GravityVolumeComponent.Priority` (`|GetArrayItem` (`self.GravBoxesPriority`) _array_index) _bp_gravityvolumecomponent))))