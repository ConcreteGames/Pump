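; BP_GravityBox is a box-shaped gravity volume that calls ApplyGravity on its gravity volume component every tick.
; Its SizeCalculation function derives the X, Y and Z extents from the world distances between three pairs of opposing arrow components.
; It returns those extents with the center arrow's location and the component's local direction and force.
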(event `self.ReceiveTick`
  (params (DeltaSeconds :type "Float (single-precision)"))
  (`/Game/Pump/LD/GravityPlateform/BP_GravityVolumeComponent.ApplyGravity` (`self.BP_GravityVolumeComponent`)))

(fn `DistanceBetweenTwoPoints`
  (params (A :type "Vector Structure") (B :type "Vector Structure"))
  (returns (AbsoluteDistance :type "Float (double-precision)"))
  (return (`KismetMathLibrary.Abs` (`KismetMathLibrary.VSize` (- A B)))))

(fn `SizeCalculation`
  (returns (XDistance :type "Float (double-precision)") (YDistance :type "Float (double-precision)") (ZDistance :type "Float (double-precision)") (CenterLocation :type "Vector Structure") (LocalDirection :type "Vector Structure") (Force :type "Float (double-precision)"))
  (bind _bp_gravityvolumecomponent (`self.BP_GravityVolumeComponent`))
  (return (`self.DistanceBetweenTwoPoints` (`SceneComponent.K2_GetComponentLocation` (`self.ArrowFront`)) (`SceneComponent.K2_GetComponentLocation` (`self.ArrowBack`))) (`self.DistanceBetweenTwoPoints` (`SceneComponent.K2_GetComponentLocation` (`self.ArrowLeft`)) (`SceneComponent.K2_GetComponentLocation` (`self.ArrowRight`))) (`self.DistanceBetweenTwoPoints` (`SceneComponent.K2_GetComponentLocation` (`self.ArrowBot`)) (`SceneComponent.K2_GetComponentLocation` (`self.ArrowTop`))) (`SceneComponent.K2_GetComponentLocation` (`self.ArrowCenter`)) (`/Game/Pump/LD/GravityPlateform/BP_GravityVolumeComponent.LocalDirection` _bp_gravityvolumecomponent) (`/Game/Pump/LD/GravityPlateform/BP_GravityVolumeComponent.Force` _bp_gravityvolumecomponent)))

(fn `UserConstructionScript`)