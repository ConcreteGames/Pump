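; Gravity platform actor that applies gravity to actors inside its collider through a gravity volume component.
; BeginPlay copies the force, priority, inversion and direction settings into the component and caches the player character and particle manager; Tick applies the gravity.
; A first-step event sets a walked-once flag after a short delay, and a visibility event toggles rendering, collision and tick together.
; Impact and particle-direction events are empty stubs.
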(event `self.ReceiveBeginPlay`
  ;[0.2181 1 0] BEGIN PLAY
  (`self.SetGravityValuesInComponent`)
  (bind _asbp_gravity_character_pump (cast `/Game/Pump/Core/Character/BP_GravityCharacter_Pump` (`GameplayStatics.GetPlayerPawn` 0)))
  (set `self.PCharacter` _asbp_gravity_character_pump)
  (bind _outactors (`GameplayStatics.GetAllActorsOfClass` "/Game/Pump/Core/Beacons/BP_ParticleManager.BP_ParticleManager_C"))
  (set `self.PParticleManager` (`|GetArrayItem` _outactors)))

(event `self.ReceiveTick`
  (params (DeltaSeconds :type "Float (single-precision)"))
  ;[1 0.855 0] TICK
  (`/Game/Pump/LD/GravityPlateform/BP_GravityVolumeComponent.ApplyGravityToActorsInCollider` (`self.BP_GravityVolumeComponent`) (`self.GravityCollider`)))

(event `CharacterImpact`)

(event `CharacterFirstStep`
  (`KismetSystemLibrary.Delay` 0.1 :!pinned true) ; Delay to Allow deactivation of hit tiles (movement and sound)
  (set `self.IsWalkedOnce` true))

(event `IsWalked`
  (if (not (`self.IsWalkedOnce`))
    (`self.CharacterFirstStep`)))

(event `SetVisiblity`
  (params (`New Visibility` :type Boolean))
  (`self.SetActorHiddenInGame` (not `New Visibility`))
  (`self.SetActorEnableCollision` `New Visibility`)
  (`self.SetActorTickEnabled` `New Visibility`))

(event `UpdateParticlesDirection`
  (params (PointToLookAt :type "Vector Structure")))

(fn `SetGravityValuesInComponent`
  (bind _bp_gravityvolumecomponent (`self.BP_GravityVolumeComponent`))
  (set `/Game/Pump/LD/GravityPlateform/BP_GravityVolumeComponent.Force` (`self.Force`) _bp_gravityvolumecomponent)
  (set `/Game/Pump/LD/GravityPlateform/BP_GravityVolumeComponent.Priority` (`self.Priority`) _bp_gravityvolumecomponent)
  (set `/Game/Pump/LD/GravityPlateform/BP_GravityVolumeComponent.InverseGravity` (`self.Sphere_InvertGravity`) _bp_gravityvolumecomponent)
  (set `/Game/Pump/LD/GravityPlateform/BP_GravityVolumeComponent.LocalDirection` (`self.Plane_LocalDirection`) _bp_gravityvolumecomponent))

(fn `UserConstructionScript`)