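; Spherical gravity platform variant that carries a step bubble, which starts growing when the character first steps on the planet.
; On BeginPlay it registers its child-actor bubble with the level's first BP_BubbleManager.
; The construction script copies the platform's NextLevelIndex to the bubble, but BeginPlay then resets the bubble's value to zero.
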(event `self.ReceiveBeginPlay`
  (bind _asbp_bubble_step (cast `/Game/Pump/LD/Bubble/BP_Bubble_Step` (`ChildActorComponent.ChildActor` (`self.ChildActor_Bubble`)) :!pure true))
  (`parent.ReceiveBeginPlay`)
  (bind _outactors (`GameplayStatics.GetAllActorsOfClass` "/Game/Pump/Core/BP_BubbleManager.BP_BubbleManager_C"))
  (`/Game/Pump/Core/BP_BubbleManager.AddBubble` (`|GetArrayItem` _outactors) _asbp_bubble_step)
  (set `/Game/Pump/LD/Bubble/BP_Bubble_Step.NextLevelIndex` 0 _asbp_bubble_step))

(event `self.ReceiveTick`
  (params (DeltaSeconds :type "Float (single-precision)"))
  (`parent.ReceiveTick` DeltaSeconds))

(event `/Game/Pump/LD/GravityPlateform/BP_GravityPlateform.CharacterFirstStep`
  (`parent.CharacterFirstStep`)
  (`/Game/Pump/LD/Bubble/BP_Bubble_Step.StartGrowing` (cast `/Game/Pump/LD/Bubble/BP_Bubble_Step` (`ChildActorComponent.ChildActor` (`self.ChildActor_Bubble`)) :!pure true)))

(fn `UserConstructionScript`
  (`parent.UserConstructionScript`)
  (set `/Game/Pump/LD/Bubble/BP_Bubble_Step.NextLevelIndex` (`self.NextLevelIndex`) (cast `/Game/Pump/LD/Bubble/BP_Bubble_Step` (`ChildActorComponent.ChildActor` (`self.ChildActor_Bubble`)) :!pure true)))