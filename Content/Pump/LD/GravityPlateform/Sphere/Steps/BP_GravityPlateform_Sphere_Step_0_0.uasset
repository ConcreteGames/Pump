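; Gravity platform sphere actor for Step 0_0, extending a parent planet step with paintable meshes, step music and a tutorial collider.
; On begin play it generates painting materials for its static meshes, except the planet and those tagged "Visible", and point damage feeds the painter component.
; A music event triggers the step's FMOD part through the sound system.
; When the key bowl fills, it hides the tutorial collider and disables its child meshes' collision.
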(event `self.ReceivePointDamage`
  (params (Damage :type "Float (single-precision)") (DamageType :type "DamageType Object Reference") (HitLocation :type "Vector Structure") (HitNormal :type "Vector Structure") (HitComponent :type "PrimitiveComponent Object Reference") (BoneName :type Name) (ShotFromDirection :type "Vector Structure") (InstigatedBy :type "Controller Object Reference") (DamageCauser :type "Actor Object Reference") (HitInfo :type "HitResult Structure (by ref)"))
  ;[1 0.7688 0] Drawer
  (`/Game/Pump/LD/Environnement/PaintedMeshes/BP_Painter_Component.PointDamage` (`self.BP_Painter_Component`) Damage DamageType HitLocation HitNormal HitComponent "None" ShotFromDirection InstigatedBy DamageCauser HitInfo))

(event `self.ReceiveBeginPlay`
  (`parent.ReceiveBeginPlay`)
  ;[1 0.6515 0] Init Meshes to Paint
  (for _array_element (`self.K2_GetComponentsByClass` "/Script/Engine.StaticMeshComponent")
    (if (and (not (== _array_element (`self.PlanetMesh`))) (not (`ActorComponent.ComponentHasTag` _array_element "Visible")))
      (`/Game/Pump/LD/Environnement/PaintedMeshes/BP_Painter_Component.GeneratePaintingMaterial` (`self.BP_Painter_Component`) _array_element))))

(event `self.Music_InitAndPlayStepsPOI`
  (`/Game/Pump/Core/SoundSystem/Bp_SoundSystem.TriggerMusicPart` (`self.PSoundSytem`) true "/Game/FMOD/Events/Music/2DMusic/Step01/M_Step01.M_Step01" 0))

(event `self.OnKeyBowlIsFilled`
  (bind _tutocoll (`self.TutoColl`))
  (`parent.OnKeyBowlIsFilled`)
  (`SceneComponent.SetVisibility` _tutocoll false true)
  (for _array_element (`SceneComponent.GetChildrenComponents` _tutocoll false)
    (bind _asstatic_mesh_component (cast `StaticMeshComponent` _array_element))
    (`PrimitiveComponent.SetCollisionEnabled` _asstatic_mesh_component "NoCollision")))

(fn `UserConstructionScript`
  (`parent.UserConstructionScript`))