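; Gravity platform sphere step Blueprint that links part of itself to a look-at-player actor.
; On BeginPlay, after the parent logic, it attaches its Scene0 component to the root of the BP_LookAtPlayer child actor, keeping world transforms.
; Scene0 thus follows that child actor's transform.
; Construction only calls the parent, and the Tick and overlap events are disabled.
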(event `self.ReceiveBeginPlay`
  (`parent.ReceiveBeginPlay`)
  (`SceneComponent.K2_AttachToComponent` (`self.Scene_0`) (`Actor.RootComponent` (cast `/Game/Pump/BadPaul/LevelBuildingRessources/Actors/BP_LookAtPlayer` (`ChildActorComponent.ChildActor` (`self.LookAtPlayer0`)) :!pure true)) "None" "KeepWorld" "KeepWorld" "KeepWorld" true))

(fn `UserConstructionScript`
  (`parent.UserConstructionScript`))