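; Step 0 of the spherical gravity platform (marked OLD), a child Blueprint that forwards point damage to its painter component.
; Its music init event starts the Step01 music and a 75 BPM tempo reference through the sound system.
; When the key bowl is filled, it hides the tutorial collider hierarchy and disables collision on that component's static mesh children.
; Older music and paint-material setup logic remains unconnected.
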(event `self.ReceivePointDamage`
  (params (Damage :type "Float (single-precision)") (DamageType :type "DamageType Object Reference") (HitLocation :type "Vector Structure") (HitNormal :type "Vector Structure") (HitComponent :type "PrimitiveComponent Object Reference") (BoneName :type Name) (ShotFromDirection :type "Vector Structure") (InstigatedBy :type "Controller Object Reference") (DamageCauser :type "Actor Object Reference") (HitInfo :type "HitResult Structure (by ref)"))
  ;[1 0.7688 0] Drawer
  (`/Game/Pump/LD/Environnement/PaintedMeshes/BP_Painter_Component.PointDamage` (`self.BP_Painter_Component`) Damage DamageType HitLocation HitNormal HitComponent "None" ShotFromDirection InstigatedBy DamageCauser HitInfo))

(event `self.ReceiveBeginPlay`
  (`parent.ReceiveBeginPlay`))

(event `self.Music_InitAndPlayStepsPOI`
  (`/Game/Pump/Core/SoundSystem/Bp_SoundSystem.PlayMusicAndTemoin` (`self.PSoundSytem`) "/Game/FMOD/Events/Music/2DMusic/Step01/M_Step01.M_Step01" "/Game/FMOD/Events/Music/2DMusic/MasterTemoins/A_M_Temoin75BPM.A_M_Temoin75BPM"))

(event `OnKeyBowlIsFilled`
  (bind _tutocoll (`self.TutoColl`))
  (`SceneComponent.SetVisibility` _tutocoll false true)
  (for _array_element (`SceneComponent.GetChildrenComponents` _tutocoll false)
    (bind _asstatic_mesh_component (cast `StaticMeshComponent` _array_element))
    (`PrimitiveComponent.SetCollisionEnabled` _asstatic_mesh_component "NoCollision")))

(fn `UserConstructionScript`
  (`parent.UserConstructionScript`))