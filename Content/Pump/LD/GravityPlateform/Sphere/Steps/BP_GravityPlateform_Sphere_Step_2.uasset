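; Second-step variant of the spherical gravity platform, a small planet that sets its first-step sound, starts its music and dresses its surface with trees.
; On decor spawn, or construction with max-scale preview, it scatters random-scale instances of three tree meshes at random sphere points, testing them against TreeHoles markers.
; Optionally, construction also snaps OrientedObjects children to the fixed radius, aligns them radially and randomizes the scale of those named as trees.
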(event `self.ReceiveBeginPlay`
  (`parent.ReceiveBeginPlay`)
  (set `self.SfxFirstStep` "/Game/FMOD/Events/Narrative/NR_PlanetStep02_FirstStep.NR_PlanetStep02_FirstStep"))

(event `self.Music_InitAndPlayStepsPOI`
  (`/Game/Pump/Core/SoundSystem/Bp_SoundSystem.PlayMusicAndTemoin` (`self.PSoundSytem`) (`self.MusicEvent`) (`self.TempoTemoin`)))

(event `self.SpawnDecor`
  (`parent.SpawnDecor`)
  (`self.GenerateTrees`))

(fn `AlignToCenter`
  (params (InputPin :type "SceneComponent Object Reference"))
  (bind _relativelocation (`SceneComponent.RelativeLocation` InputPin))
  (`SceneComponent.K2_SetRelativeRotation` InputPin (`KismetMathLibrary.FindLookAtRotation` (`KismetMathLibrary.MakeVector` 0.0) _relativelocation) false false)
  (`SceneComponent.K2_AddLocalRotation` InputPin (struct :`Pitch` -90.0) false false)
  (`SceneComponent.K2_SetRelativeLocation` InputPin (* (`KismetMathLibrary.Normal` _relativelocation) 3030.0) false false)
  (if (`KismetStringLibrary.Contains` (`KismetSystemLibrary.GetDisplayName` InputPin) "tree")
    (`SceneComponent.SetRelativeScale3D` InputPin (`KismetMathLibrary.Conv_DoubleToVector` (`KismetMathLibrary.Lerp` 0.4 0.7 (`KismetMathLibrary.RandomFloat`))))))

(fn `GenerateTrees`
  (bind _returnvalue (select `int` (`KismetMathLibrary.RandomInteger` 3) :`0` (`self.Trees01`) :`1` (`self.Trees02`) :`2` (`self.Trees03`) :!type "InstancedStaticMeshComponent Object Reference"))
  (for _ (range (+ (`self.MaxAutoTrees`) 1))
    (bind _inahole (`self.GetNextPos`))
    (if (not _inahole)
      (`InstancedStaticMeshComponent.AddInstance` _returnvalue (`self.MakeInstanceTransform`))
      (`/Game/Pump/Core/BP_FunctionLibrary.LogErer` (`KismetSystemLibrary.GetDisplayName` _returnvalue)))))

(fn `GetNextPos`
  (returns (InAHole :type Boolean))
  (bind _treeholes (`self.TreeHoles`))
  (bind _output_get (set `self.NextPos` (* (`KismetMathLibrary.RandomUnitVector`) 3030.0)))
  (`SceneComponent.K2_SetRelativeLocation` (`self.Arrow`) _output_get false false)
  (set `self.InAHole` false)
  (for _index (range (`SceneComponent.GetNumChildrenComponents` _treeholes))
    (bind _returnvalue (<= (`KismetMathLibrary.VSize` (- (`SceneComponent.K2_GetComponentLocation` (`SceneComponent.GetChildComponent` _treeholes _index)) (`SceneComponent.K2_GetComponentLocation` (`self.Arrow`)))) 500.0))
    (if _returnvalue
      (bind _output_get_2 (set `self.NextPos` (* (`KismetMathLibrary.RandomUnitVector`) 3030.0)))
      (`SceneComponent.K2_SetRelativeLocation` (`self.Arrow`) _output_get_2 false false)
      (if (not _returnvalue)
        (set `self.InAHole` true))))
  (return (`self.InAHole`)))

(fn `MakeInstanceTransform`
  (returns (ReturnValue :type "Transform Structure"))
  (return (`KismetMathLibrary.MakeTransform` (`self.NextPos`) (`KismetMathLibrary.NormalizedDeltaRotator` (`KismetMathLibrary.FindLookAtRotation` (`KismetMathLibrary.MakeVector` 0.0) (`self.NextPos`)) (struct :`Pitch` 90.0)) (`KismetMathLibrary.Conv_DoubleToVector` (`KismetMathLibrary.Lerp` 0.4 0.7 (`KismetMathLibrary.RandomFloat`))))))

(fn `OrientateObjects`
  (bind _orientedobjects (`self.OrientedObjects`))
  (if (`self.OrientateTrees`)
    (for _index (range (`SceneComponent.GetNumChildrenComponents` _orientedobjects))
      (`self.AlignToCenter` (`SceneComponent.GetChildComponent` _orientedobjects _index)))))

(fn `UserConstructionScript`
  (`parent.UserConstructionScript`)
  (`self.OrientateObjects`)
  (if (`self.PreviewMaxScale`)
    (`self.GenerateTrees`)))