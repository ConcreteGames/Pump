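; Spherical gravity platform: a planet mesh inside a radius-driven gravity volume that can be inverted.
; The construction script sizes the collision sphere and mesh, assigns the sphere as gravity collider and passes inversion to the gravity volume component.
; InitParticleValue, also run on BeginPlay, drives the Niagara effect, scaling spawn rate (unless manual), size, velocity and lifetime from the radii.
; Inversion flips particle velocity and halves radius and lifetime; hard or soft gravity picks the color.
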(event `self.ReceiveBeginPlay`
  (`parent.ReceiveBeginPlay`)
  (`self.InitParticleValue`))

(fn `InitParticleValue`
  (bind _returnvalue (`self.MapGravitySphereParticleValues` 10.0 100.0))
  (bind _gravitysphereradius (`self.GravitySphereRadius`))
  (bind _particle (`self.Particle`))
  (`NiagaraComponent.SetNiagaraVariableFloat` _particle "User.SphereRadius" (select `bool` (`self.InvertGravity`) :`false` _gravitysphereradius :`true` (/ _gravitysphereradius 2.0)))
  (`NiagaraComponent.SetNiagaraVariableFloat` _particle "User.SpawnRate" (select `bool` (`self.bManualParticleSpawnRate`) :`false` (`self.MapGravitySphereParticleValues` 100.0 10000.0) :`true` (`self.ParticleSpawnRate`)))
  (`NiagaraComponent.SetNiagaraVariableVec2` _particle "User.SpriteSize" (`KismetMathLibrary.MakeVector2D` _returnvalue _returnvalue))
  (`NiagaraComponent.SetNiagaraVariableFloat` _particle "User.Velocity" (select `bool` (`self.InvertGravity`) :`false` (`self.MapGravitySphereParticleValues` -20.0 -100.0) :`true` (`self.MapGravitySphereParticleValues` 20.0 100.0)))
  (`NiagaraComponent.SetNiagaraVariableLinearColor` _particle "User.Color" (select `bool` (`self.bGravityHard`) :`false` (`self.SoftGravityColor`) :`true` (`self.HardGravityColor`)))
  (`NiagaraComponent.SetNiagaraVariableFloat` _particle "User.ParticleLifetime" (`self.MapGravityLifetime` 0.2 7.0)))

(fn `MapGravityLifetime`
  (params (Min :type "Float (double-precision)") (Max :type "Float (double-precision)"))
  (returns (ReturnValue :type "Float (double-precision)"))
  (bind _returnvalue (`KismetMathLibrary.MapRangeClamped` (- (`self.GravitySphereRadius`) (`self.PlanetScale`)) (`self.GravitySphereMinRadius`) (`self.GravitySphereMaxRadius`) Min Max))
  (return (select `bool` (`self.InvertGravity`) :`false` _returnvalue :`true` (/ _returnvalue 2.0))))

(fn `MapGravitySphereParticleValues`
  (params (Min :type "Float (double-precision)") (Max :type "Float (double-precision)"))
  (returns (ReturnValue :type "Float (double-precision)"))
  (return (`KismetMathLibrary.MapRangeClamped` (`self.GravitySphereRadius`) (`self.GravitySphereMinRadius`) (`self.GravitySphereMaxRadius`) Min Max)))

(fn `UserConstructionScript`
  (bind _returnvalue (/ (`self.PlanetScale`) 100.0))
  (`parent.UserConstructionScript`)
  (set `self.GravityCollider` (`self.SphereCollision`))
  (`SphereComponent.SetSphereRadius` (`self.SphereCollision`) (`self.GravitySphereRadius`) true)
  (`SceneComponent.SetRelativeScale3D` (`self.PlanetMesh`) (`KismetMathLibrary.MakeVector` _returnvalue _returnvalue _returnvalue))
  (set `/Game/Pump/LD/GravityPlateform/BP_GravityVolumeComponent.InverseGravity` (`self.InvertGravity`) (`self.BP_GravityVolumeComponent`))
  (`self.InitParticleValue`))