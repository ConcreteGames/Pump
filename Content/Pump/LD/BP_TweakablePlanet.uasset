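; BP_TweakablePlanet is a level-design planet actor that pairs a planet mesh with a gravity sphere, tunable per instance.
; The Construction Script uniformly scales the mesh (relative) and the BP_GravitySphere child actor component (world) from separate scale variables.
; It then casts the child actor and pushes Force and Priority into it.
; The event graph holds only disabled stub events.
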(fn `UserConstructionScript`
  (bind _gravityspherescale (`self.GravitySphereScale`))
  (bind _planetscale (`self.PlanetScale`))
  (bind _bp_gravitysphere (`self.BP_GravitySphere`))
  (`SceneComponent.SetRelativeScale3D` (`self.SM_Planet`) (`KismetMathLibrary.MakeVector` _planetscale _planetscale _planetscale))
  (`SceneComponent.SetWorldScale3D` _bp_gravitysphere (`KismetMathLibrary.MakeVector` _gravityspherescale _gravityspherescale _gravityspherescale))
  (bind _asbp_gravity_sphere (cast `/Game/Pump/LD/BP_GravitySphere` (`ChildActorComponent.ChildActor` _bp_gravitysphere)))
  (set `/Game/DirectionalGravity/Blueprints/GravityLogic/BP_GravityVolumeBase.Force` (`self.Force`) _asbp_gravity_sphere)
  (set `/Game/DirectionalGravity/Blueprints/GravityLogic/BP_GravityVolumeBase.Priority` (`self.Priority`) _asbp_gravity_sphere))