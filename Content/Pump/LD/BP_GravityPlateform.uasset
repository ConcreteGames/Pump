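; Cube platform that builds optional gravity volumes on any of its six faces, each with particle feedback.
; The construction script spawns a BP_GravityBox child actor per enabled face arrow, converting transforms through a helper arrow and swapping scale axes per side.
; Per-face arrays set depth, force, direction and priority, with zero depth falling back to the first entry.
; Niagara effects follow box footprint, with force driving velocity and color, and depth driving lifetime and spawn rate.
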(fn `UserConstructionScript`
  (bind _gravboxesscalez (`self.GravBoxesScaleZ`))
  (bind (_returnvalue_location _returnvalue_rotation _returnvalue_scale) (`KismetMathLibrary.BreakTransform` (`SceneComponent.GetRelativeTransform` (`self.ArrowConversion`))))
  (bind (_returnvalue_x _returnvalue_y _returnvalue_z) (`KismetMathLibrary.BreakVector` (`SceneComponent.K2_GetComponentScale` (`self.SM_Cube`))))
  (bind _returnvalue (`KismetMathLibrary.MakeVector` _returnvalue_x _returnvalue_z _returnvalue_y))
  (bind _returnvalue_2 (`KismetMathLibrary.MakeVector` _returnvalue_x _returnvalue_y _returnvalue_z))
  (bind _returnvalue_3 (`KismetMathLibrary.MakeVector` _returnvalue_z _returnvalue_y _returnvalue_x))
  ;[1 1 1] For each sides
  (bind _output_get (set `self.ArrowArray` (`|MakeArray` (`self.Arrow0Top`) (`self.Arrow1Bot`) (`self.Arrow2Front`) (`self.Arrow3Back`) (`self.Arrow4Left`) (`self.Arrow5Right`))))
  (for (_array_element _array_index) _output_get
    ;[1 1 1] If box wanted
    (if (`|GetArrayItem` (`self.SpawnGravBoxes`) _array_index)
      ;[1 1 1] Custom good scale
      (`SceneComponent.SetWorldScale3D` _array_element (select `int` _array_index :`0` _returnvalue_2 :`1` _returnvalue_2 :`2` _returnvalue_3 :`3` _returnvalue_3 :`4` _returnvalue :`5` _returnvalue))
      (bind (_returnvalue_location_2 _returnvalue_rotation_2 _returnvalue_scale_2) (`KismetMathLibrary.BreakTransform` (`SceneComponent.K2_GetComponentToWorld` _array_element)))
      ;[1 1 1] Get relative transform
      (`SceneComponent.K2_SetWorldTransform` (`self.ArrowConversion`) (`KismetMathLibrary.MakeTransform` _returnvalue_location_2 _returnvalue_rotation_2 _returnvalue_scale_2) false false)
      ;[1 1 1] Add GravityCube
      (bind _returnvalue_4 (`AddComponent|NODE_AddChildActorComponent-3` :`RelativeTransform` (`KismetMathLibrary.MakeTransform` _returnvalue_location _returnvalue_rotation _returnvalue_scale)))
      (bind (_returnvalue_x_2 _returnvalue_y_2) (`KismetMathLibrary.BreakVector` (`SceneComponent.K2_GetComponentScale` _returnvalue_4)))
      (bind _output (`|GetArrayItem` _gravboxesscalez _array_index))
      (bind _returnvalue_5 (select `bool` (!= _output 0.0) :`false` (`|GetArrayItem` _gravboxesscalez) :`true` _output))
      ;[1 1 1] Override Z Scale
      (`SceneComponent.SetWorldScale3D` _returnvalue_4 (`KismetMathLibrary.MakeVector` _returnvalue_x_2 _returnvalue_y_2 _returnvalue_5))
      (bind _asbp_gravity_box (cast `/Game/Pump/LD/BP_GravityBox` (`ChildActorComponent.ChildActor` _returnvalue_4) :!pure true))
      (bind _bp_gravityvolumecomponent (`/Game/Pump/LD/BP_GravityBox.BP_GravityVolumeComponent` _asbp_gravity_box))
      ;[1 1 1] set Params
      (bind _output_get_2 (set `/Game/Pump/LD/BP_GravityVolumeComponent.Force` (`|GetArrayItem` (`self.GravBoxesForce`) _array_index) _bp_gravityvolumecomponent))
      (set `/Game/Pump/LD/BP_GravityVolumeComponent.LocalDirection` (`|GetArrayItem` (`self.GravBoxesDirection`) _array_index) _bp_gravityvolumecomponent)
      (set `/Game/Pump/LD/BP_GravityVolumeComponent.Priority` (`|GetArrayItem` (`self.GravBoxesPriority`) _array_index) _bp_gravityvolumecomponent)
      ;[1 1 1] Particles
      (bind _returnvalue_6 (`AddComponent|NODE_AddNiagaraComponent-1` :`bManualAttachment` true))
      (`SceneComponent.K2_SetWorldRotation` _returnvalue_6 (`self.K2_GetActorRotation` _asbp_gravity_box) false false)
      (`SceneComponent.K2_SetWorldLocation` _returnvalue_6 (`SceneComponent.K2_GetComponentLocation` (`/Game/Pump/LD/BP_GravityBox.ArrowTop` _asbp_gravity_box)) false false)
      (bind (_xdistance _ydistance) (`/Game/Pump/LD/BP_GravityBox.SizeCalculation` _asbp_gravity_box))
      (bind _returnvalue_7 (/ _xdistance 2.0))
      (bind _returnvalue_8 (/ _ydistance 2.0))
      (`NiagaraComponent.SetNiagaraVariableVec2` _returnvalue_6 "User.PlainSize" (`KismetMathLibrary.MakeVector2D` _returnvalue_7 _returnvalue_8))
      (`NiagaraComponent.SetNiagaraVariableVec2` _returnvalue_6 "User.RainPlateSize" (`KismetMathLibrary.MakeVector2D` _returnvalue_7 _returnvalue_8))
      (`NiagaraComponent.SetNiagaraVariableVec3` _returnvalue_6 "User.RainVelocity" (`KismetMathLibrary.MakeVector` 0.0 0.0 (`KismetMathLibrary.MapRangeClamped` _output_get_2 100.0 10000.0 -20.0 -1000.0)))
      (`NiagaraComponent.SetNiagaraVariableVec3` _returnvalue_6 "User.InitColor" (`KismetMathLibrary.Conv_LinearColorToVector` (`CurveLinearColor.GetLinearColorValue` (`self.CRV_GravityColorCurve`) (`KismetMathLibrary.MapRangeClamped` _output_get_2 100.0 10000.0 0.0 1.0)))) ; Set Color For Particle
      (`NiagaraComponent.SetNiagaraVariableFloat` _returnvalue_6 "User.RainLifetime" (`KismetMathLibrary.MapRangeClamped` _returnvalue_5 0.5 20.0 1.5 5.0))
      (`NiagaraComponent.SetNiagaraVariableFloat` _returnvalue_6 "User.RainSpawnRate" (`KismetMathLibrary.MapRangeClamped` _returnvalue_5 0.5 20.0 30.0 100.0)))))