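; BP_Creatures is a decorative-looking actor that continuously spins groups of child components around several pivots.
; The construction script places children of PivotUp in a cross and children of Scene at diagonal corners, applying a shared scale to all but Scene.
; Each Tick rotates PivotUp steadily, while PivotRight and Scene yaw and add curve-driven pitch or roll sampled from a two-second Sine timeline.
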(event `self.ReceiveBeginPlay`
  (`TimelineComponent.SetTimelineLength` (`self.Sine`) 2.0)
  (`Timeline|Sine` :!via `PlayFromStart`))

(event `self.ReceiveTick`
  (params (DeltaSeconds :type "Float (single-precision)"))
  (bind _returnvalue (`CurveFloat.GetFloatValue` (`self.SineCurve`) (`/Game/Pump/Core/BP_FunctionLibrary.GetTimelinePercentage` (`self.Sine`))))
  (set `self.Time` (+ DeltaSeconds (`self.Time`)))
  (`SceneComponent.K2_AddWorldRotation` (`self.PivotUp`) (struct :`Roll` 1.0) false false)
  (set `self.NewVar_0` (mod (+ (/ (* DeltaSeconds 360.0) 2.0) (`self.NewVar_0`)) 360.0))
  (`SceneComponent.K2_AddWorldRotation` (`self.PivotRight`) (`KismetMathLibrary.MakeRotator` 0.0 (* _returnvalue 1.0) 1.0) false false)
  (`SceneComponent.K2_AddWorldRotation` (`self.Scene`) (`KismetMathLibrary.MakeRotator` (* _returnvalue 1.0) 0.0 1.0) false false))

(fn `UserConstructionScript`
  (bind _output_get (set `self.PUChilds` (`SceneComponent.GetChildrenComponents` (`self.PivotUp`) false)))
  (for (_array_element _array_index) _output_get
    (set `self.SSLoc` (select `int` _array_index :`0` (0.0 200.0 0.0) :`1` (0.0 0.0 200.0) :`2` (0.0 -200.0 0.0) :`3` (0.0 0.0 -200.0) :!type "Vector Structure"))
    (`SceneComponent.K2_SetRelativeLocation` _array_element (`self.SSLoc`) false false)
    (if (!= _array_element (`self.Scene`))
      (`SceneComponent.SetWorldScale3D` _array_element (`self.NewVar_1`))))
  (bind _output_get_2 (set `self.VChilds` (`SceneComponent.GetChildrenComponents` (`self.Scene`) false)))
  (for (_array_element_2 _array_index_2) _output_get_2
    (`SceneComponent.K2_SetRelativeLocation` _array_element_2 (select `int` _array_index_2 :`0` (0.0 150.0 150.0) :`1` (0.0 -150.0 -150.0) :`2` (0.0 150.0 -150.0) :`3` (0.0 -150.0 150.0) :!type "Vector Structure") false false)
    (`SceneComponent.SetWorldScale3D` _array_element_2 (`self.NewVar_1`))))