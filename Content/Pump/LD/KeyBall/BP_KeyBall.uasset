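; Key ball pickup that guides the player toward a target bowl with visual feedback.
; Until picked up, it bobs and turns a pulsing child component toward the player, scaled by proximity, while timeline spins quicken as the player nears.
; With a target set, Niagara velocity points at the bowl, and once held, glow material parameters follow hand aim and bowl distance.
; Pickup disables collision and shrinks the visual; dropping stops particles and Tick.
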(event `self.ReceiveTick`
  (params (DeltaSeconds :type "Float (single-precision)"))
  (`self.UpdatePlayerProximityFeedback`)
  (`self.UpdateKeyFloating`)
  (`/Engine/EditorBlueprintResources/StandardMacros.IsValid` (`self.CurrentTargetBowl`)
    (:`Is Valid`
      (`self.UpdateParticleDirection`)
      (`self.UpdatePlayerDirectionFeedback`))))

(event `IsPickedUp`
  (`PrimitiveComponent.SetCollisionEnabled` (`self.Collision`) "NoCollision")
  (`SceneComponent.SetRelativeScale3D` (`self.Visual`) (0.5 0.5 0.5))
  (set `self.PickedUp` true)
  (`MaterialInstanceDynamic.SetScalarParameterValue` (`self.DynamicMaterialInstance`) "Speed" 0.5)
  (`SceneComponent.SetVisibility` (`self.Scene1`) false true)
  (`self.K2_SetActorRelativeRotation` (struct)))

(event `SetTargetBowl`
  (params (NewParam :type "/Game/Pump/LD/KeyBall/BP_KeyBowl Object Reference"))
  (set `self.CurrentTargetBowl` NewParam))

(event `UpdateParticleDirection`
  (`NiagaraComponent.SetNiagaraVariableVec3` (`self.Niagara`) "User.Velocity" (* (`KismetMathLibrary.Normal` (- (`SceneComponent.K2_GetComponentLocation` (`/Game/Pump/LD/KeyBall/BP_KeyBowl.BallAttachPoint` (`self.CurrentTargetBowl`))) (`self.K2_GetActorLocation`))) 100.0)))

(event `IsDropped`
  (`ActorComponent.Deactivate` (`self.Niagara`))
  (set `self.PickedUp` false)
  (`self.SetActorTickEnabled` false))

(event `UpdatePlayerProximityFeedback`
  (bind _returnvalue (`KismetMathLibrary.MapRangeClamped` (`self.GetDistanceToPlayer`) 300.0 400.0 1.0 0.0))
  (if (not (`self.PickedUp`))
    (`SceneComponent.K2_SetWorldRotation` (`self.Scene1`) (`KismetMathLibrary.RLerp` (`KismetMathLibrary.FindLookAtRotation` (`self.K2_GetActorLocation`) (`self.K2_GetActorLocation` (cast `/Game/Pump/Core/Character/BP_GravityCharacter_Pump` (`GameplayStatics.GetPlayerPawn` 0) :!pure true))) (`SceneComponent.K2_GetComponentRotation` (`self.Scene1`)) 0.9) false false)
    (`SceneComponent.SetRelativeScale3D` (`self.Scene1`) (`KismetMathLibrary.VLerp` (`KismetMathLibrary.VLerp` (1.0 1.0 1.0) (1.8 1.8 1.8) _returnvalue) (`KismetMathLibrary.VLerp` (1.2 1.2 1.2) (2.0 2.0 2.0) _returnvalue) (`self.SinusPerTime` 1.0)))))

(event `UpdatePlayerDirectionFeedback`
  (bind _dynamicmaterialinstance (`self.DynamicMaterialInstance`))
  (bind _returnvalue (- (`self.K2_GetActorLocation`) (`SceneComponent.K2_GetComponentLocation` (`/Game/Pump/LD/KeyBall/BP_KeyBowl.BallAttachPoint` (`self.CurrentTargetBowl`)))))
  (bind _returnvalue_2 (`KismetMathLibrary.Dot_VectorVector` (`SceneComponent.GetForwardVector` (`/Game/Pump/Core/Character/BP_GravityCharacter_Pump.CharacterHands` (cast `/Game/Pump/Core/Character/BP_GravityCharacter_Pump` (`GameplayStatics.GetPlayerPawn` 0) :!pure true))) (`KismetMathLibrary.Normal` _returnvalue)))
  (if (`self.PickedUp`)
    (`MaterialInstanceDynamic.SetScalarParameterValue` _dynamicmaterialinstance "MinPower" (`KismetMathLibrary.MapRangeClamped` _returnvalue_2 -1.0 0.0 10.0 5.0))
    (`MaterialInstanceDynamic.SetScalarParameterValue` _dynamicmaterialinstance "MaxPower" (`KismetMathLibrary.MapRangeClamped` _returnvalue_2 -1.0 0.0 15.0 5.0))
    (`MaterialInstanceDynamic.SetScalarParameterValue` (`self.DynamicMaterialInstance`) "PowerBooster" (`KismetMathLibrary.MapRangeClamped` (`KismetMathLibrary.VSize` _returnvalue) 100.0 500.0 1000.0))))

(event `UpdateKeyFloating`
  (bind _returnvalue (`self.GetDistanceToPlayer`))
  (bind _timeline_rotateweirdly (`self.Timeline_RotateWeirdly`))
  (bind __ (`/Game/Pump/Core/BP_FunctionLibrary.GetTimelinePercentage` (`self.Timeline_RotateWeirdly`)))
  (bind _returnvalue_2 (`KismetMathLibrary.MapRangeClamped` _returnvalue 400.0 600.0 0.3 1.0))
  (`SceneComponent.K2_SetRelativeLocation` (`self.Scene`) (select `bool` (`self.PickedUp`) :`false` (`KismetMathLibrary.VLerp` (0.0 0.0 -5.0) (0.0 0.0 5.0) (`self.SinusPerTime` 0.5))) false false)
  (`self.WaitDuration` (`KismetMathLibrary.MapRangeClamped` _returnvalue 400.0 1000.0 0.0 5.0)
    (:`TimeIsElapsed`
      (if (not (`TimelineComponent.IsPlaying` _timeline_rotateweirdly))
        (`TimelineComponent.SetTimelineLength` _timeline_rotateweirdly _returnvalue_2)
        (set `self.UseEaseInOutCurve` (>= _returnvalue_2 1.0))
        (`Timeline|Timeline_RotateWeirdly` :`NewTime` 0.0 :!via `PlayFromStart`
          (:`Update`
            (`SceneComponent.K2_SetRelativeRotation` (`self.Scene`) (`KismetMathLibrary.RLerp` (struct) (struct :`Yaw` 360.0) (select `bool` (`self.UseEaseInOutCurve`) :`false` __ :`true` (`CurveFloat.GetFloatValue` (`self.CRV_EaseInOut`) __))) false false)))))))

(fn `GetDistanceToPlayer`
  (returns (ReturnValue :type "Float (double-precision)"))
  (return (`KismetMathLibrary.VSize` (- (`self.K2_GetActorLocation` (`GameplayStatics.GetPlayerPawn` 0)) (`self.K2_GetActorLocation`)))))

(fn `SinusPerTime`
  (params (Speed :type "Float (double-precision)"))
  (returns (Value :type "Float (double-precision)"))
  (return (/ (+ (`KismetMathLibrary.Sin` (* (`self.GetGameTimeSinceCreation`) Speed)) 1.0) 2.0)))

(fn `UserConstructionScript`
  (bind _returnvalue (`PrimitiveComponent.CreateDynamicMaterialInstance` (`self.Sphere`) 0 "/Game/Pump/LD/KeyBall/M_GlowBase_Animated_KeyBall.M_GlowBase_Animated_KeyBall" "None"))
  (set `self.DynamicMaterialInstance` _returnvalue))