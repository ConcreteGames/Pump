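; BP_KeyBowl is a receptacle for a KeyBall that reports to its planet step once it is filled.
; When a ball is given, it attaches and snaps it to an attach point, flags it as dropped, marks itself filled and notifies MyPlanetStep.
; Three feedback components start hidden: one shows this bowl's fill, two reveal progressively from the filled-bowl count passed to UpdateFillFeedbacks.
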(event `self.ReceiveBeginPlay`
  (`SceneComponent.SetVisibility` (`self.Feedback_This`) false false)
  (`SceneComponent.SetVisibility` (`self.Feedback_0`) false false)
  (`SceneComponent.SetVisibility` (`self.Feedback_1`) false false))

(event `OnBallIsGiven`
  (params (KeyBall :type "/Game/Pump/LD/KeyBall/BP_KeyBall Object Reference"))
  (`self.K2_AttachToComponent` KeyBall (`self.BallAttachPoint`) "None" "KeepWorld" "KeepWorld" "KeepWorld" true)
  (`self.K2_SetActorRelativeLocation` KeyBall (0.0 0.0 0.0) false false)
  (`/Game/Pump/LD/KeyBall/BP_KeyBall.IsDropped` KeyBall)
  (set `self.IsFilled` true)
  (`/Game/Pump/LD/GravityPlateform/Sphere/BP_GravityPlateform_Sphere_Step.OnKeyBowlIsFilled` (`self.MyPlanetStep`))
  (`KismetSystemLibrary.PrintString` "Hello")
  (`SceneComponent.SetVisibility` (`self.Feedback_This`) true false))

(event `UpdateFillFeedbacks`
  (params (FilledBowls :type Integer))
  (if (> FilledBowls 0)
    (if (>= FilledBowls 2)
      (`SceneComponent.SetVisibility` (`self.Feedback_1`) true false))
    (`SceneComponent.SetVisibility` (`self.Feedback_0`) true false)))

(fn `UserConstructionScript`)