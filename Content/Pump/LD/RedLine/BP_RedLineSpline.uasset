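; Spline actor that draws a "red line" as a chain of spline meshes with particles and an animated pulsing thickness.
; The construction script splits the spline into equal-length segments, with scaled and optionally normalized tangents.
; GenerateParticles then adds a Niagara component at each segment start, aimed along its tangent.
; Tick applies a phase-offset sine to each segment's end scale and copies it to the next segment's start, keeping joints continuous.
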(event `self.ReceiveBeginPlay`)

(event `self.ReceiveTick`
  (params (DeltaSeconds :type "Float (single-precision)"))
  (`self.AnimateStartEndScale`))

(event `AnimateStartEndScale`
  (bind _splinemeshcomponent (`self.SplineMeshComponent`))
  (for (_array_element _array_index) (`self.SplineMeshComponent`)
    (`/Engine/EditorBlueprintResources/StandardMacros.IsValid` _array_element
      (:`Is Valid`
        (bind _returnvalue (* (`KismetMathLibrary.Sin` (+ (`self.GetGameTimeSinceCreation`) (* (`KismetMathLibrary.MultiplyByPi` (`KismetMathLibrary.Conv_IntToDouble` _array_index)) 0.5))) (`self.ScaleAnimDelta`)))
        (bind _returnvalue_2 (+ (`self.BaseScale`) (`KismetMathLibrary.MakeVector2D` _returnvalue _returnvalue)))
        (`SplineMeshComponent.SetEndScale` _array_element _returnvalue_2 true)
        (bind _returnvalue_3 (+ _array_index 1))
        (if (< _returnvalue_3 (`KismetArrayLibrary.Array_Length` _splinemeshcomponent))
          (`SplineMeshComponent.SetStartScale` (`|GetArrayItem` _splinemeshcomponent _returnvalue_3) _returnvalue_2 true))))))

(fn `GenerateParticles`
  (for _array_element (`self.SplineMeshComponent`)
    (`/Engine/EditorBlueprintResources/StandardMacros.IsValid` _array_element
      (:`Is Valid`
        (bind _returnvalue (`AddComponent|NODE_AddNiagaraComponent-1` :`bManualAttachment` true))
        (`SceneComponent.K2_AttachToComponent` _returnvalue (`self.DefaultSceneRoot`) "None" "KeepRelative" "KeepRelative" "KeepRelative" true)
        (bind _returnvalue_2 (`SplineMeshComponent.GetStartPosition` _array_element))
        (`SceneComponent.K2_SetRelativeLocationAndRotation` _returnvalue _returnvalue_2 (`KismetMathLibrary.FindLookAtRotation` _returnvalue_2 (+ _returnvalue_2 (`SplineMeshComponent.GetStartTangent` _array_element))) false false)))))

(fn `UserConstructionScript`
  (locals (NewLocalVar_0 :type "Float (double-precision)" :default 0.0))
  (bind _lengthpermesh (`self.LengthPerMesh`))
  (bind _tangentscaling (`self.TangentScaling`))
  (bind _normalizetangent (`self.NormalizeTangent`))
  (bind _basescale (`self.BaseScale`))
  (bind _spline (`self.Spline`))
  (bind _returnvalue (* (`self.Idx`) _lengthpermesh))
  (bind _returnvalue_2 (* (+ (`self.Idx`) 1) _lengthpermesh))
  (bind _returnvalue_3 (`SplineComponent.GetTangentAtDistanceAlongSpline` _spline _returnvalue "Local"))
  (bind _returnvalue_4 (`SplineComponent.GetTangentAtDistanceAlongSpline` _spline _returnvalue_2 "Local"))
  (set `self.SplineMeshComponent` (`|MakeArray` null :!type "SplineMeshComponent Object Reference"))
  (set `self.LengthPerMesh` (/ (`SplineComponent.GetSplineLength` _spline) (`KismetMathLibrary.Conv_IntToDouble` (`self.Segments`))))
  (for _index (range (`self.Segments`))
    (set `self.Idx` _index)
    (bind _returnvalue_5 (`AddComponent|NODE_AddSplineMeshComponent-1`))
    (`SplineMeshComponent.SetStartAndEnd` _returnvalue_5 (`SplineComponent.GetLocationAtDistanceAlongSpline` _spline _returnvalue "Local") (select `bool` _normalizetangent :`false` (* _returnvalue_3 _tangentscaling) :`true` (* (`KismetMathLibrary.Normal` _returnvalue_3) _tangentscaling)) (`SplineComponent.GetLocationAtDistanceAlongSpline` _spline _returnvalue_2 "Local") (select `bool` _normalizetangent :`false` (* _returnvalue_4 _tangentscaling) :`true` (* (`KismetMathLibrary.Normal` _returnvalue_4) _tangentscaling)) true)
    (`SplineMeshComponent.SetStartScale` _returnvalue_5 _basescale true)
    (`SplineMeshComponent.SetEndScale` _returnvalue_5 _basescale true)
    (`KismetArrayLibrary.Array_AddUnique` (`self.SplineMeshComponent`) _returnvalue_5))
  (`self.GenerateParticles`))