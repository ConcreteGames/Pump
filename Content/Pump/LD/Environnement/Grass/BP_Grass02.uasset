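; BP_Grass02 is a grass environment actor whose static mesh becomes visible when something begins overlapping its box and hides when an overlap ends.
; The overlap events set visibility directly, with no actor filter or overlap count.
; The construction script applies the box extent, mesh asset and mesh world scale from variables.
; A custom event, apparently for debugging, prints the attach parent actor's scale.
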(event `self.Box.OnComponentBeginOverlap`
  (params (OverlappedComponent :type "PrimitiveComponent Object Reference") (OtherActor :type "Actor Object Reference") (OtherComp :type "PrimitiveComponent Object Reference") (OtherBodyIndex :type Integer) (bFromSweep :type Boolean) (SweepResult :type "HitResult Structure (by ref)"))
  (`SceneComponent.SetVisibility` (`self.StaticMesh`) true false))

(event `self.Box.OnComponentEndOverlap`
  (params (OverlappedComponent :type "PrimitiveComponent Object Reference") (OtherActor :type "Actor Object Reference") (OtherComp :type "PrimitiveComponent Object Reference") (OtherBodyIndex :type Integer))
  (`SceneComponent.SetVisibility` (`self.StaticMesh`) false false))

(event `CustomEvent_0`
  (`KismetSystemLibrary.PrintString` (`KismetStringLibrary.Conv_VectorToString` (`self.GetActorScale3D` (`self.GetAttachParentActor`)))))

(fn `UserConstructionScript`
  (`BoxComponent.SetBoxExtent` (`self.Box`) (`self.BoxExtent`) true)
  (`SceneComponent.SetWorldScale3D` (`self.StaticMesh`) (`self.PlaneScale`))
  (`StaticMeshComponent.SetStaticMesh` (`self.StaticMesh`) (`self.Mesh`)))