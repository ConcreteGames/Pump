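; Phantom mesh environment actor that starts at zero initial opacity and reveals itself once, typically when a platform ground hit is received.
; BeginPlay applies dynamic phantom materials to a static mesh and/or randomly scattered instances, kept outside a safe zone and optionally aimed at the center.
; HitGroundPlateform maps impact velocity to wave power, scaling the timeline-driven VectorLengthMiddle reveal on all materials.
; When the timeline finishes, the materials are permanently flagged as Walked.
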(event `self.ReceiveBeginPlay`
  (bind _instancedstaticmesh (`self.InstancedStaticMesh`))
  (bind _returnvalue (+ (`self.K2_GetActorLocation`) (`self.PopInstancesZone` (`self.Distance`) (`self.SafeZone`))))
  (if (`self.HasSM`)
    (`KismetArrayLibrary.Array_Clear` (`self.SMMid`))
    (for _index (range (+ (`PrimitiveComponent.GetNumMaterials` (`self.StaticMesh`)) 1))
      (bind _returnvalue_2 (`PrimitiveComponent.CreateDynamicMaterialInstance` (`self.StaticMesh`) _index "/Game/Pump/LD/Environnement/PhantomMeshes/M_PhantomMeshes_Inst.M_PhantomMeshes_Inst" "None"))
      (`KismetArrayLibrary.Array_AddUnique` (`self.SMMid`) _returnvalue_2)
      (`MaterialInstanceDynamic.SetTextureParameterValue` _returnvalue_2 "Texture" (`self.SmTexture`))
      (`MaterialInstanceDynamic.SetTextureParameterValue` _returnvalue_2 "Normal" (`self.SmNormal`))
      (`MaterialInstanceDynamic.SetTextureParameterValue` _returnvalue_2 "RoughnessTexture" (`self.SmRoughness`))
      (`MaterialInstanceDynamic.SetScalarParameterValue` _returnvalue_2 "Metallic" (`self.SmMetal`))
      (`MaterialInstanceDynamic.SetScalarParameterValue` _returnvalue_2 "InitOpacity" 0.0)))
  (if (`self.HasInstance`)
    (`KismetArrayLibrary.Array_Clear` (`self.Mids`))
    (`StaticMeshComponent.SetStaticMesh` (`self.InstancedStaticMesh`) (`self.SetStaticMesh`))
    (for _index_2 (range (+ (`PrimitiveComponent.GetNumMaterials` _instancedstaticmesh) 1))
      (bind _returnvalue_3 (`PrimitiveComponent.CreateDynamicMaterialInstance` _instancedstaticmesh _index_2 "/Game/Pump/LD/Environnement/PhantomMeshes/M_PhantomMeshes_Inst.M_PhantomMeshes_Inst" "None"))
      (`KismetArrayLibrary.Array_AddUnique` (`self.Mids`) _returnvalue_3))
    (for _array_element (`self.Mids`)
      (`MaterialInstanceDynamic.SetTextureParameterValue` _array_element "Texture" (`self.Texture`))
      (`MaterialInstanceDynamic.SetTextureParameterValue` _array_element "Normal" (`self.NormalMap`))
      (`MaterialInstanceDynamic.SetTextureParameterValue` _array_element "RoughnessTexture" (`self.RoughnessTexture`))
      (`MaterialInstanceDynamic.SetScalarParameterValue` _array_element "Metallic" (`self.Metalic`)))
    (set `self.PParent` (`SceneComponent.GetAttachParent` (`self.Billboard`)))
    (for _ (range (+ (`self.NumberOfInstances`) 1))
      (`InstancedStaticMeshComponent.AddInstanceWorldSpace` (`self.InstancedStaticMesh`) (`KismetMathLibrary.MakeTransform` _returnvalue (`self.GetInstanceRotation` _returnvalue) (`KismetMathLibrary.Conv_DoubleToVector` (`KismetMathLibrary.RandomFloatInRange` (`self.ScaleMin`) (`self.ScaleMax`))))))
    (for _array_element_2 (`self.Mids`)
      (`MaterialInstanceDynamic.SetScalarParameterValue` _array_element_2 "InitOpacity" 0.0))))

(event `/Game/Pump/Core/Beacons/BI_Events.HitGroundPlateform`
  (params (Velocity :type "Float (single-precision)") (IsWalkedOnce :type Boolean))
  ;[1 1 1] Hit Ground Message
  (set `self.PlateformWavesPower` (`KismetMathLibrary.MapRangeClamped` Velocity 500.0 3000.0 1.5 8.0))
  (`self.RevealMesh`))

(event `RevealMesh`
  ;[1 1 1] Reveal Mesh
  (`/Engine/EditorBlueprintResources/StandardMacros.DoOnce` false
    (:`Completed`
      (bind (_direction _cosinepower _distancefromplayer _alpha _vectorlength) (`Timeline|Timeline_0` :!via `PlayFromStart`)
        (:`Update`
          (`|ExecutionSequence`
            (:`then_0`
              (for _array_element (`self.Mids`)
                (bind _returnvalue (* _vectorlength (`KismetMathLibrary.MapRangeClamped` (`self.PlateformWavesPower`) 1.5 6.0 1.0 2.0)))
                (`MaterialInstanceDynamic.SetScalarParameterValue` _array_element "VectorLengthMiddle" _returnvalue)))
            (:`then_1`
              (for _array_element_2 (`self.SMMid`)
                (`MaterialInstanceDynamic.SetScalarParameterValue` _array_element_2 "VectorLengthMiddle" _returnvalue)))))
        (:`Finished`
          (if (not (`self.bColoured`))
            (set `self.bColoured` true)
            (`|ExecutionSequence`
              (:`then_0`
                (for _array_element_3 (`self.Mids`)
                  (`MaterialInstanceDynamic.SetScalarParameterValue` _array_element_3 "Walked" 1.0)))
              (:`then_1`
                (for _array_element_4 (`self.SMMid`)
                  (`MaterialInstanceDynamic.SetScalarParameterValue` _array_element_4 "Walked" 1.0))))))))))

(fn `GetInstanceRotation`
  (params (InstanceLocation :type "Vector Structure"))
  (returns (ReturnValue :type "Rotator Structure"))
  (return (select `bool` (`self.LookAtCenter`) :`false` (`KismetMathLibrary.RandomRotator` true) :`true` (`KismetMathLibrary.FindLookAtRotation` InstanceLocation (`self.K2_GetActorLocation`)))))

(fn `PopInstancesZone`
  (params (Distance :type "Float (double-precision)") (SafeZone :type "Float (double-precision)"))
  (returns (Vector :type "Vector Structure"))
  (locals (LocalSafeZone :type "Float (double-precision)") (NegativeValue :type "Float (double-precision)"))
  (bind _distance (`local.Distance`))
  (bind _negativevalue (`local.NegativeValue`))
  (bind _localsafezone (`local.LocalSafeZone`))
  (bind _localsafezone_2 (`local.LocalSafeZone`))
  (bind _negativevalue_2 (`local.NegativeValue`))
  (bind _distance_2 (`local.Distance`))
  (set `local.NegativeValue` (* Distance -1.0))
  (set `local.LocalSafeZone` (- Distance SafeZone))
  (return (`KismetMathLibrary.MakeVector` (select `bool` (`KismetMathLibrary.RandomBool`) :`false` (`KismetMathLibrary.RandomFloatInRange` _negativevalue_2 (+ _negativevalue_2 _localsafezone_2)) :`true` (`KismetMathLibrary.RandomFloatInRange` (- _distance _localsafezone_2) _distance)) (select `bool` (`KismetMathLibrary.RandomBool`) :`false` (`KismetMathLibrary.RandomFloatInRange` _negativevalue (+ _negativevalue _localsafezone)) :`true` (`KismetMathLibrary.RandomFloatInRange` (- _distance_2 _localsafezone) _distance_2)) (select `bool` (`KismetMathLibrary.RandomBool`) :`false` (`KismetMathLibrary.RandomFloatInRange` _negativevalue (+ _negativevalue _localsafezone)) :`true` (`KismetMathLibrary.RandomFloatInRange` (- _distance_2 _localsafezone) _distance_2)))))

(fn `UserConstructionScript`)