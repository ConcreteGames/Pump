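; Trigger actor that transitions the level's exponential height fog to a desired density when something overlaps its collider.
; On each overlap, INIT grabs the first ExponentialHeightFog actor's component and stores its current density as the starting value.
; The FogTransition timeline, resized to TransitionDuration, then linearly blends density toward DesiredFogDensity using its playback percentage.
; The overlapping actor is not filtered, and exiting does not restore the fog.
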(event `self.Collider.OnComponentBeginOverlap`
  (params (OverlappedComponent :type "PrimitiveComponent Object Reference") (OtherActor :type "Actor Object Reference") (OtherComp :type "PrimitiveComponent Object Reference") (OtherBodyIndex :type Integer) (bFromSweep :type Boolean) (SweepResult :type "HitResult Structure (by ref)"))
  (`self.INIT`)
  (`TimelineComponent.SetTimelineLength` (`self.FogTransition`) (`self.TransitionDuration`))
  (`Timeline|FogTransition` :!via `PlayFromStart`
    (:`Update`
      (`ExponentialHeightFogComponent.SetFogDensity` (`self.pExponensialHeightFogComponent`) (+ (`self.InitialFogDensity`) (* (- (`self.DesiredFogDensity`) (`self.InitialFogDensity`)) (`/Game/Pump/Core/BP_FunctionLibrary.GetTimelinePercentage` (`self.FogTransition`))))))))

(fn `INIT`
  (bind _outactors (`GameplayStatics.GetAllActorsOfClass` "/Script/Engine.ExponentialHeightFog"))
  (bind _component (`ExponentialHeightFog.Component` (`|GetArrayItem` _outactors)))
  (set `self.pExponensialHeightFogComponent` _component)
  (set `self.InitialFogDensity` (`ExponentialHeightFogComponent.FogDensity` _component)))

(fn `UserConstructionScript`)