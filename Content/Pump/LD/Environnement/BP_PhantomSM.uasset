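; BP_PhantomSM is an environment static mesh with phantom materials that reveals itself when it receives a ground-hit message.
; Construction applies the configurable mesh and builds a dynamic phantom material per slot, whose initial opacity is zeroed at BeginPlay.
; Impact velocity sets a wave power that scales a timeline-driven reveal radius parameter in those materials.
; When the first reveal finishes, the mesh is permanently flagged as walked and coloured.
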(event `self.ReceiveBeginPlay`
  (set `self.PParent` (`SceneComponent.GetAttachParent` (`self.DefaultSceneRoot`)))
  (for _array_element (`self.Mids`)
    (`MaterialInstanceDynamic.SetScalarParameterValue` _array_element "InitOpacity" 0.0)))

(event `/Game/Pump/Core/Beacons/BI_Events.HitGroundPlateform`
  (params (Velocity :type "Float (single-precision)") (IsWalkedOnce :type Boolean))
  ;[1 1 1] Hit Ground Message
  (set `self.PlateformWavesPower` (`KismetMathLibrary.MapRangeClamped` Velocity 500.0 3000.0 1.5 8.0))
  (`self.RevealMesh`))

(event `RevealMesh`
  ;[1 1 1] Reveal Mesh
  (bind (_direction _cosinepower _distancefromplayer _alpha _vectorlength) (`Timeline|Timeline_0` :!via `PlayFromStart`)
    (:`Update`
      (for _array_element (`self.Mids`)
        (`MaterialInstanceDynamic.SetScalarParameterValue` _array_element "VectorLengthMiddle" (* _vectorlength (`KismetMathLibrary.MapRangeClamped` (`self.PlateformWavesPower`) 1.5 6.0 1.0 2.0)))))
    (:`Finished`
      (if (not (`self.bColoured`))
        (set `self.bColoured` true)
        (for _array_element_2 (`self.Mids`)
          (`MaterialInstanceDynamic.SetScalarParameterValue` _array_element_2 "Walked" 1.0))))))

(fn `UserConstructionScript`
  (bind _staticmesh (`self.StaticMesh`))
  (`KismetArrayLibrary.Array_Clear` (`self.Mids`))
  (`StaticMeshComponent.SetStaticMesh` (`self.StaticMesh`) (`self.SetStaticMesh`))
  (for _index (range (+ (`PrimitiveComponent.GetNumMaterials` _staticmesh) 1))
    (bind _returnvalue (`PrimitiveComponent.CreateDynamicMaterialInstance` _staticmesh _index "/Game/Pump/LD/Environnement/M_PhantomMeshes_Inst.M_PhantomMeshes_Inst" "None"))
    (`KismetArrayLibrary.Array_AddUnique` (`self.Mids`) _returnvalue)))