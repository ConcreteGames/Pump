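; BP_PaintedDecal is a level-design decal actor that gets painted at runtime when it receives point damage.
; Construction creates dynamic decal and paint materials, applying texture, base color, metallic and roughness.
; BeginPlay feeds a new render target to the decal and zeroes OpacityInit, which keeps it visible in the editor.
; PointDamage passes ShotFromDirection as the paint material's Position, then draws it into that render target.
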(event `self.ReceiveBeginPlay`
  (bind _mid (`self.Mid`))
  (bind _returnvalue (`KismetRenderingLibrary.CreateRenderTarget2D` 512 512))
  (bind _output_get (set `self.RenderTarget` _returnvalue))
  (`MaterialInstanceDynamic.SetTextureParameterValue` _mid "RenderTarget" _output_get)
  (`MaterialInstanceDynamic.SetScalarParameterValue` _mid "OpacityInit" 0.0) ; SetInitOpacity (to see meshes in LD)
)

(event `self.ReceiveTick`
  (params (DeltaSeconds :type "Float (single-precision)")))

(event `self.ReceivePointDamage`
  (params (Damage :type "Float (single-precision)") (DamageType :type "DamageType Object Reference") (HitLocation :type "Vector Structure") (HitNormal :type "Vector Structure") (HitComponent :type "PrimitiveComponent Object Reference") (BoneName :type Name) (ShotFromDirection :type "Vector Structure") (InstigatedBy :type "Controller Object Reference") (DamageCauser :type "Actor Object Reference") (HitInfo :type "HitResult Structure (by ref)"))
  (bind _paintmat (`self.PaintMat`))
  (`MaterialInstanceDynamic.SetVectorParameterValue` _paintmat "Position" (`KismetMathLibrary.Conv_VectorToLinearColor` ShotFromDirection))
  (`KismetRenderingLibrary.DrawMaterialToRenderTarget` (`self.RenderTarget`) _paintmat))

(fn `UserConstructionScript`
  (bind _returnvalue (`DecalComponent.CreateDynamicMaterialInstance` (`self.Decal`)))
  (set `self.Mid` _returnvalue)
  (`DecalComponent.SetDecalMaterial` (`self.Decal`) _returnvalue)
  (bind _returnvalue_2 (`KismetMaterialLibrary.CreateDynamicMaterialInstance` "/Game/Pump/LD/Environnement/PaintedMeshes/M_Paint_Inst.M_Paint_Inst"))
  (set `self.PaintMat` _returnvalue_2)
  (`MaterialInstanceDynamic.SetScalarParameterValue` _returnvalue "Metallic" (`self.Metalic`))
  (`MaterialInstanceDynamic.SetScalarParameterValue` _returnvalue "Roughness" (`self.Roughness`))
  (`MaterialInstanceDynamic.SetTextureParameterValue` _returnvalue "Texture" (`self.Texture`))
  (`MaterialInstanceDynamic.SetVectorParameterValue` _returnvalue "BaseColor" (`self.BaseColor`)))