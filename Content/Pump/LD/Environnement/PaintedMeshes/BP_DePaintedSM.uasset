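; Placeable static mesh that gets de-painted when it takes point damage, with selectable opacity, color, texture and burn looks.
; The construction script applies a dynamic material per slot, picked by PaintType, and sets its surface parameters.
; BeginPlay creates a render target, feeds it to those materials and sets their initial opacity.
; Point damage passes ShotFromDirection as Position to the DePaint material, which is drawn into that target.
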(event `self.ReceiveBeginPlay`
  (bind _returnvalue (`KismetRenderingLibrary.CreateRenderTarget2D` 512 512))
  (bind _output_get (set `self.RenderTarget` _returnvalue))
  (for _array_element (`self.Mid`)
    (`MaterialInstanceDynamic.SetTextureParameterValue` _array_element "RenderTarget" _output_get)
    (`MaterialInstanceDynamic.SetScalarParameterValue` _array_element "OpacityInit" 1.0) ; SetInitOpacity (to see meshes in LD)
  ))

(event `self.ReceiveTick`
  (params (DeltaSeconds :type "Float (single-precision)")))

(event `self.ReceivePointDamage`
  (params (Damage :type "Float (single-precision)") (DamageType :type "DamageType Object Reference") (HitLocation :type "Vector Structure") (HitNormal :type "Vector Structure") (HitComponent :type "PrimitiveComponent Object Reference") (BoneName :type Name) (ShotFromDirection :type "Vector Structure") (InstigatedBy :type "Controller Object Reference") (DamageCauser :type "Actor Object Reference") (HitInfo :type "HitResult Structure (by ref)"))
  (bind _paintmat (`self.PaintMat`))
  (`MaterialInstanceDynamic.SetVectorParameterValue` _paintmat "Position" (`KismetMathLibrary.Conv_VectorToLinearColor` ShotFromDirection))
  (`KismetRenderingLibrary.DrawMaterialToRenderTarget` (`self.RenderTarget`) _paintmat))

(fn `UserConstructionScript`
  (bind _staticmesh (`self.StaticMesh`))
  (`StaticMeshComponent.SetStaticMesh` _staticmesh (`self.StaticMeshInstance`))
  (for _index (range (+ (`PrimitiveComponent.GetNumMaterials` _staticmesh) 1))
    (bind _returnvalue (`PrimitiveComponent.CreateDynamicMaterialInstance` _staticmesh _index (select `/Game/Pump/LD/Environnement/PaintedMeshes/EPaintedMeshesTypes` (`self.PaintType`) :`NewEnumerator0` "/Game/Pump/LD/Environnement/PaintedMeshes/M_PaintCanvasDepaint.M_PaintCanvasDepaint" :`NewEnumerator1` "/Game/Pump/LD/Environnement/PaintedMeshes/M_PaintCanvasTextureOpacity_Inst.M_PaintCanvasTextureOpacity_Inst" :`NewEnumerator2` "/Game/Pump/LD/Environnement/PaintedMeshes/M_PaintCanvasTextureBurnOpacity_Inst.M_PaintCanvasTextureBurnOpacity_Inst" :`NewEnumerator3` "/Game/Pump/LD/Environnement/PaintedMeshes/M_PaintCanvasDepaint.M_PaintCanvasDepaint" :`NewEnumerator5` "/Game/Pump/LD/Environnement/PaintedMeshes/M_PaintCanvasColorsBurn_Inst.M_PaintCanvasColorsBurn_Inst" :!type "MaterialInterface Object Reference") "None"))
    (`PrimitiveComponent.SetMaterial` _staticmesh _index _returnvalue)
    (`KismetArrayLibrary.Array_AddUnique` (`self.Mid`) _returnvalue))
  (bind _returnvalue_2 (`KismetMaterialLibrary.CreateDynamicMaterialInstance` "/Game/Pump/LD/Environnement/PaintedMeshes/M_DePaint_Inst.M_DePaint_Inst"))
  (set `self.PaintMat` _returnvalue_2)
  (for _array_element (`self.Mid`)
    (`MaterialInstanceDynamic.SetScalarParameterValue` _array_element "Metallic" (`self.Metal`))
    (`MaterialInstanceDynamic.SetScalarParameterValue` _array_element "Roughness" (`self.Roughness`))
    (switch `/Game/Pump/LD/Environnement/PaintedMeshes/EPaintedMeshesTypes` (`self.PaintType`)
      (:`NewEnumerator0`
        (`MaterialInstanceDynamic.SetVectorParameterValue` _array_element "BaseColor" (`self.BaseColor`) :!label _label)
        (`MaterialInstanceDynamic.SetVectorParameterValue` _array_element "PaintedColor" (`self.PaintedColor`))
        (switch `/Game/Pump/LD/Environnement/PaintedMeshes/EPaintedMeshesTypes` (`self.PaintType`)
          (:`NewEnumerator2`
            _)
          (:`NewEnumerator5`
            _)))
      (:`NewEnumerator1`
        _)
      (:`NewEnumerator2`
        (goto _label))
      (:`NewEnumerator3`
        (goto _label))
      (:`NewEnumerator5`
        (goto _label)))
    (`MaterialInstanceDynamic.SetTextureParameterValue` _array_element "Normal" (`self.NormalMap`))
    (`MaterialInstanceDynamic.SetTextureParameterValue` _array_element "Texture" (`self.Texture`))))