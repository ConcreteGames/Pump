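; Painter component that makes registered meshes paintable by point damage, with variants for custom colors, textures, burn and opacity.
; Each registered mesh gets a custom collision channel, dynamic canvas materials chosen by paint type, and its own render target.
; On a hit, the shot direction value becomes the brush material's Position, and that material is drawn into the hit mesh's render target, which feeds its canvas materials.
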(event `self.ReceiveBeginPlay`
  ;[1 1 1] Begin Play
  (`KismetArrayLibrary.Array_Clear` (`self.StrPaintMeshes`))
  (bind _returnvalue (`KismetMaterialLibrary.CreateDynamicMaterialInstance` "/Game/Pump/LD/Environnement/PaintedMeshes/M_Paint_Inst.M_Paint_Inst"))
  (set `self.PaintMat` _returnvalue))

(event `GeneratePaintingMaterial`
  (params (SmRef :type "StaticMeshComponent Object Reference"))
  ;[1 1 1] Make Array of Painted meshes
  (`self.MakePaintedMeshes` SmRef))

(event `PointDamage`
  (params (Damage :type "Float (double-precision)") (DamageType :type "DamageType Object Reference") (HitLocation :type "Vector Structure") (HitNormal :type "Vector Structure") (HitComponent :type "PrimitiveComponent Object Reference") (BoneName :type Name) (ShotFromDirection :type "Vector Structure") (InstigatedBy :type "Controller Object Reference") (DamageCauser :type "Actor Object Reference") (HitInfo :type "HitResult Structure (by ref)"))
  (bind _paintmat (`self.PaintMat`))
  ;[1 1 1] Paint
  (set `self.PointerPosition` ShotFromDirection)
  (for _array_element (`self.StrPaintMeshes`)
    (bind (_meshcomponents _rendertarget) (break `/Game/Pump/LD/Environnement/PaintedMeshes/STR_PaintMesh` _array_element))
    (if (== HitComponent _meshcomponents)
      (`MaterialInstanceDynamic.SetVectorParameterValue` _paintmat "Position" (`KismetMathLibrary.Conv_VectorToLinearColor` (`self.PointerPosition`)))
      (`KismetRenderingLibrary.DrawMaterialToRenderTarget` _rendertarget _paintmat))))

(fn `MakePaintedMeshes`
  (params (MeshComponents :type "StaticMeshComponent Object Reference"))
  (locals (Mid :type "Array of MaterialInstanceDynamic Object Reference"))
  (bind _structindex (`self.StructIndex`))
  (bind _strpaintmeshes (`self.StrPaintMeshes`))
  (bind _strpaintmeshes_2 (`self.StrPaintMeshes`))
  (bind ((`MeshComponents_5_3C8F78414F4A9FC6F1922ABD4056DDF5` _meshcomponents)) (break `/Game/Pump/LD/Environnement/PaintedMeshes/STR_PaintMesh` (`|GetArrayItem` (`self.StrPaintMeshes`) (`self.StructIndex`))))
  (bind (_meshcomponents_2 _rendertarget _mids) (break `/Game/Pump/LD/Environnement/PaintedMeshes/STR_PaintMesh` (`|GetArrayItem` _strpaintmeshes_2 _structindex)))
  (bind (_meshcomponents_3 _rendertarget_2 _mids_2) (break `/Game/Pump/LD/Environnement/PaintedMeshes/STR_PaintMesh` (`|GetArrayItem` (`self.StrPaintMeshes`) (`self.StructIndex`))))
  (bind _returnvalue (`KismetArrayLibrary.Array_AddUnique` (`self.StrPaintMeshes`) (make `/Game/Pump/LD/Environnement/PaintedMeshes/STR_PaintMesh` :`MeshComponents` MeshComponents)))
  (set `self.StructIndex` _returnvalue)
  (`PrimitiveComponent.SetCollisionObjectType` _meshcomponents "ECC_GameTraceChannel3")
  (for _index (range (+ (`PrimitiveComponent.GetNumMaterials` _meshcomponents) 1))
    (bind _returnvalue_2 (`PrimitiveComponent.CreateDynamicMaterialInstance` _meshcomponents _index (select `/Game/Pump/LD/Environnement/PaintedMeshes/EPaintedMeshesTypes` (`self.PaintType`) :`NewEnumerator0` "/Game/Pump/LD/Environnement/PaintedMeshes/M_PaintCanvasColorsOpacity_Inst.M_PaintCanvasColorsOpacity_Inst" :`NewEnumerator1` "/Game/Pump/LD/Environnement/PaintedMeshes/M_PaintCanvasTextureOpacity_Inst.M_PaintCanvasTextureOpacity_Inst" :`NewEnumerator2` "/Game/Pump/LD/Environnement/PaintedMeshes/M_PaintCanvasTextureBurnOpacity_Inst.M_PaintCanvasTextureBurnOpacity_Inst" :`NewEnumerator3` "/Game/Pump/LD/Environnement/PaintedMeshes/M_PaintCanvasColors_Inst.M_PaintCanvasColors_Inst" :`NewEnumerator5` "/Game/Pump/LD/Environnement/PaintedMeshes/M_PaintCanvasColorsBurn_Inst.M_PaintCanvasColorsBurn_Inst" :!type "MaterialInterface Object Reference") "None"))
    (`PrimitiveComponent.SetMaterial` _meshcomponents _index _returnvalue_2)
    (`KismetArrayLibrary.Array_AddUnique` (`local.Mid`) _returnvalue_2))
  (`KismetArrayLibrary.Array_Set` _strpaintmeshes (`self.StructIndex`) (make `/Game/Pump/LD/Environnement/PaintedMeshes/STR_PaintMesh` :`MeshComponents` (`.MeshComponents_5_3C8F78414F4A9FC6F1922ABD4056DDF5` (break `/Game/Pump/LD/Environnement/PaintedMeshes/STR_PaintMesh` (`|GetArrayItem` _strpaintmeshes (`self.StructIndex`)))) :`Mids` (`local.Mid`)))
  (for _array_element (`.Mids_12_69A9E7D5324BFF1A186D02B26C8DB660` (break `/Game/Pump/LD/Environnement/PaintedMeshes/STR_PaintMesh` (`|GetArrayItem` (`self.StrPaintMeshes`) (`self.StructIndex`))))
    (`MaterialInstanceDynamic.SetScalarParameterValue` _array_element "Metallic" (`self.Metal`))
    (`MaterialInstanceDynamic.SetScalarParameterValue` _array_element "Roughness" (`self.Roughness`))
    (switch `/Game/Pump/LD/Environnement/PaintedMeshes/EPaintedMeshesTypes` (`self.PaintType`)
      (:`NewEnumerator0`
        (`MaterialInstanceDynamic.SetVectorParameterValue` _array_element "BaseColor" (`self.BaseColor`) :!label _label)
        (`MaterialInstanceDynamic.SetVectorParameterValue` _array_element "PaintedColor" (`self.PaintedColor`))
        (switch `/Game/Pump/LD/Environnement/PaintedMeshes/EPaintedMeshesTypes` (`self.PaintType`)
          (:`NewEnumerator2`
            _)
          (:`NewEnumerator5`
            _)))
      (:`NewEnumerator1`
        _)
      (:`NewEnumerator2`
        (goto _label))
      (:`NewEnumerator3`
        (goto _label))
      (:`NewEnumerator5`
        (goto _label)))
    (`MaterialInstanceDynamic.SetTextureParameterValue` _array_element "Normal" (`self.NormalMap`))
    (`MaterialInstanceDynamic.SetTextureParameterValue` _array_element "Texture" (`self.Texture`)))
  (bind _returnvalue_3 (`KismetRenderingLibrary.CreateRenderTarget2D` 512 512))
  (`KismetArrayLibrary.Array_Set` _strpaintmeshes_2 _structindex (make `/Game/Pump/LD/Environnement/PaintedMeshes/STR_PaintMesh` _meshcomponents_3 _returnvalue_3 _mids_2))
  (for _array_element_2 _mids
    (`MaterialInstanceDynamic.SetTextureParameterValue` _array_element_2 "RenderTarget" _rendertarget)
    (`MaterialInstanceDynamic.SetScalarParameterValue` _array_element_2 "OpacityInit" (`self.InitOpacity`)) ; SetInitOpacity (to see meshes in LD)
  ))