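; Scene-capture actor that paints onto instanced static, static or spline mesh components at a hit location with a given brush size.
; BeginPlay creates a dynamic M_Unwrap material and clears the RT_Paint render target.
; PaintActor temporarily swaps the mesh's first material for that unwrap material, feeds it the hit location and radius, triggers the scene capture, then restores the original material.
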(event `self.ReceiveBeginPlay`
  (bind _returnvalue (`KismetMaterialLibrary.CreateDynamicMaterialInstance` "/Game/Pump/LD/Environnement/PaintedMeshes/M_Unwrap.M_Unwrap"))
  (set `self.UnwrapMaterial` _returnvalue)
  (`KismetRenderingLibrary.ClearRenderTarget2D` (`SceneCaptureComponent2D.TextureTarget` (`self.SceneCapture`)) "/Game/Pump/LD/Environnement/PaintedMeshes/RT_Paint.RT_Paint"))

(fn `PaintActor`
  (params (ComponentToPaint :type "ActorComponent Object Reference") (HitLocation :type "Vector Structure") (BrushSize :type "Float (double-precision)"))
  (bind _asinstanced_static_mesh_component (cast `InstancedStaticMeshComponent` ComponentToPaint)
    (:`then`
      (set `self.InstancedMesh` _asinstanced_static_mesh_component)
      (set `self.CompType` 0))
    (:`CastFailed`
      (bind _asstatic_mesh_component (cast `StaticMeshComponent` ComponentToPaint)
        (:`then`
          (set `self.StaticMesh` _asstatic_mesh_component)
          (set `self.CompType` 1))
        (:`CastFailed`
          (bind _asspline_mesh_component (cast `SplineMeshComponent` ComponentToPaint))
          (set `self.SplineMeshComp` _asspline_mesh_component)
          (set `self.CompType` 2)))))
  (`|ExecutionSequence`
    (:`then_0`
      (set `self.OriginalMaterial` (`PrimitiveComponent.GetMaterial` (select `int` (`self.CompType`) :`0` (`self.StaticMesh`) :`1` (`self.InstancedMesh`) :`2` (`self.SplineMeshComp`) :!type "PrimitiveComponent Object Reference") 0))
      (`PrimitiveComponent.SetMaterial` (select `int` (`self.CompType`) :`0` (`self.StaticMesh`) :`1` (`self.InstancedMesh`) :`2` (`self.SplineMeshComp`) :!type "PrimitiveComponent Object Reference") 0 (`self.UnwrapMaterial`)))
    (:`then_1`
      (`MaterialInstanceDynamic.SetVectorParameterValue` (`self.UnwrapMaterial`) "HitLocation" (`KismetMathLibrary.Conv_VectorToLinearColor` (`local.HitLocation`)))
      (`MaterialInstanceDynamic.SetScalarParameterValue` (`self.UnwrapMaterial`) "Radius" (`local.BrushSize`)))
    (:`then_2`
      (`SceneCaptureComponent2D.CaptureScene` (`self.SceneCapture`))
      (`PrimitiveComponent.SetMaterial` (select `int` (`self.CompType`) :`0` (`self.StaticMesh`) :`1` (`self.InstancedMesh`) :`2` (`self.SplineMeshComp`) :!type "PrimitiveComponent Object Reference") 0 (`self.OriginalMaterial`)))))

(fn `UserConstructionScript`)