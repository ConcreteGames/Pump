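; BP_Painting is a paintable mesh actor that records brush hits into its own render target.
; Construction gives the mesh a dynamic canvas material, and BeginPlay creates the render target shared by that material and the scene capture.
; Paint briefly swaps in an unwrap material fed with hit location and brush radius, captures the scene, then restores the original.
; The component-type casting in Paint is disconnected, so only the built-in mesh is painted.
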(event `self.ReceiveBeginPlay`
  (bind _returnvalue (`KismetMaterialLibrary.CreateDynamicMaterialInstance` "/Game/Pump/LD/Environnement/PaintedMeshes/M_Unwrap.M_Unwrap"))
  (bind _output_get (set `self.UnwrapMaterial` _returnvalue))
  (`MaterialInstanceDynamic.SetScalarParameterValue` _output_get "None" 0.0)
  (`KismetRenderingLibrary.ClearRenderTarget2D` "/Game/Pump/LD/Environnement/PaintedMeshes/RT_Paint.RT_Paint")
  (bind _returnvalue_2 (`KismetRenderingLibrary.CreateRenderTarget2D` 512 512))
  (set `self.RenderTarget` _returnvalue_2)
  (`MaterialInstanceDynamic.SetTextureParameterValue` (`self.PaintMaterial`) "RenderTarget" _returnvalue_2)
  (set `SceneCaptureComponent2D.TextureTarget` (`self.RenderTarget`) (`self.SceneCapture`)))

(fn `Paint`
  (params (Component :type "Object Object Reference") (HitLocation :type "Vector Structure") (BrushSize :type "Float (double-precision)"))
  (`|ExecutionSequence`
    (:`then_0`
      (set `self.OriginalMaterial` (`PrimitiveComponent.GetMaterial` (`self.StaticMesh1`) 0))
      (`PrimitiveComponent.SetMaterial` (`self.StaticMesh1`) 0 (`self.UnwrapMaterial`)))
    (:`then_1`
      (`MaterialInstanceDynamic.SetVectorParameterValue` (`self.UnwrapMaterial`) "HitLocation" (`KismetMathLibrary.Conv_VectorToLinearColor` (`local.HitLocation`)))
      (`MaterialInstanceDynamic.SetScalarParameterValue` (`self.UnwrapMaterial`) "Radius" (`local.BrushSize`)))
    (:`then_2`
      (`SceneCaptureComponent2D.CaptureScene` (`self.SceneCapture`))
      (`PrimitiveComponent.SetMaterial` (`self.StaticMesh1`) 0 (`self.OriginalMaterial`)))))

(fn `UserConstructionScript`
  (`PrimitiveComponent.SetMaterial` (`self.StaticMesh1`) 0 "/Game/Pump/LD/Environnement/PaintedMeshes/M_PaintCanvasCapture.M_PaintCanvasCapture")
  (bind _returnvalue (`PrimitiveComponent.CreateDynamicMaterialInstance` (`self.StaticMesh1`) 0 "/Game/Pump/LD/Environnement/PaintedMeshes/M_PaintCanvasCapture.M_PaintCanvasCapture" "None"))
  (set `self.PaintMaterial` _returnvalue))