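; Level design actor that places a row of bubble child actors along a spline.
; Starting at the SplineParser distance, it adds a bubble, then advances by a spacing read from a float curve at the normalized spline position, looping until the next step would reach the spline's end.
; The PreviewBubbles flag decides whether bubbles are built in the construction script for editor preview or at BeginPlay.
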(event `self.ReceiveBeginPlay`
  (if (not (`self.PreviewBubbles`))
    (`self.SpawnBubblesAlongSpline`)))

(fn `SpawnABubble`
  (bind _returnvalue (`AddComponent|NODE_AddChildActorComponent-2` :`bManualAttachment` true))
  (`SceneComponent.K2_SetWorldLocation` _returnvalue (`SplineComponent.GetLocationAtDistanceAlongSpline` (`self.Spline`) (`self.SplineParser`) "World") false false))

(fn `SpawnBubblesAlongSpline`
  (bind _returnvalue (+ (`self.SplineParser`) (`CurveFloat.GetFloatValue` (`self.CRV_BubbleSplineDistance`) (/ (`self.SplineParser`) (`SplineComponent.GetSplineLength` (`self.Spline`))))))
  (`self.SpawnABubble` :!label _label)
  (if (< _returnvalue (`SplineComponent.GetSplineLength` (`self.Spline`)))
    (set `self.SplineParser` _returnvalue)
    (goto _label)))

(fn `UserConstructionScript`
  (if (`self.PreviewBubbles`)
    (`self.SpawnBubblesAlongSpline`)))