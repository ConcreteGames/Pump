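; Master bubble actor: a sphere zone that notifies the Pump gravity character on enter and exit, with density-based damping.
; Construction hard-codes damping per density, derives color from it or a fixed value, and scales by radius.
; First entry swaps to a density-specific "ON" material and notifies the level manager; leaving while pumping notifies the sound manager.
; Overlap radius grows while occupied to stabilize enter/exit, and a startup delay temporarily gates entry.
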(event `self.ReceiveBeginPlay`
  ;[0 1 0.1624] BEGIN PLAY
  (`self.REF_Char`)
  (set `self.SaveInitialRadius` (`SphereComponent.SphereRadius` (`self.Sphere`))) ; for SecuEnterExitSphere
  (`self.REF_SoundManager`)
  ;[1 1 1] test fix caca
  ; ça ne résoud pas le son du début
  (`KismetSystemLibrary.Delay` 2.0)
  (set `self.BubbleIsReadyTempTestFix` true))

(event `SetDefaultState`
  (params (NewParam :type "LinearColor Structure"))
  (`MaterialInstanceDynamic.SetVectorParameterValue` (`self.MaterialInstance`) "Color" NewParam))

(event `SetBubbleManager`
  (params (NewParam :type "/Game/Pump/Core/BP_LevelManager Object Reference"))
  (set `self.LevelManager` NewParam))

(event `self.Sphere.OnComponentBeginOverlap`
  (params (OverlappedComponent :type "PrimitiveComponent Object Reference") (OtherActor :type "Actor Object Reference") (OtherComp :type "PrimitiveComponent Object Reference") (OtherBodyIndex :type Integer) (bFromSweep :type Boolean) (SweepResult :type "HitResult Structure (by ref)"))
  (bind _bubbleisreadytemptestfix (`self.BubbleIsReadyTempTestFix`))
  ;[1 1 1] test fix caca
  ; ça ne résoud pas le son du début
  (if _bubbleisreadytemptestfix
    (`/Game/Pump/Core/BP_FunctionLibrary.LogErerBool` "BubbleIsReadyTempTestFix" _bubbleisreadytemptestfix)
    (bind _asbp_gravity_character_pump (cast `/Game/Pump/Core/Character/BP_GravityCharacter_Pump` OtherActor))
    (`/Game/Pump/Core/Character/BP_GravityCharacter_Pump.EnterBubble` _asbp_gravity_character_pump self)
    (`self.SecuEnterExitSphere` true)
    (`self.OnIsEntered`)))

(event `self.Sphere.OnComponentEndOverlap`
  (params (OverlappedComponent :type "PrimitiveComponent Object Reference") (OtherActor :type "Actor Object Reference") (OtherComp :type "PrimitiveComponent Object Reference") (OtherBodyIndex :type Integer))
  (bind _asbp_gravity_character_pump (cast `/Game/Pump/Core/Character/BP_GravityCharacter_Pump` OtherActor))
  (`/Game/Pump/Core/Character/BP_GravityCharacter_Pump.ExitBubble` _asbp_gravity_character_pump self)
  (`self.SecuEnterExitSphere` false)
  (`self.OnIsLeaved`))

(event `OnIsEntered`
  (if (not (`self.HasBeenEnteredOnce`))
    (`self.OnFirstEntrance`)))

(event `OnFirstEntrance`
  (bind _returnvalue (select `bool` (`self.UseCRV`) :`false` (`self.ColorWhenEntered`) :`true` (`CurveLinearColor.GetLinearColorValue` (`self.CRV_DashZoneColorByDamping`) (`KismetMathLibrary.MapRangeUnclamped` (`self.Damping`) 0.0 35.0 0.0 1.0))))
  (`/Engine/EditorBlueprintResources/StandardMacros.IsValid` (`self.LevelManager`)
    (:`Is Valid`
      (set `self.HasBeenEnteredOnce` true)
      (set `self.ColorOfBubble` _returnvalue)
      (`self.SetMaterialInstance` (select `/Game/Pump/LD/Bubble/E_Density` (`self.BubbleDensity`) :`NewEnumerator0` "/Game/Pump/LD/Bubble/M_Bubble_Disto_Dense_ON.M_Bubble_Disto_Dense_ON" :`NewEnumerator1` "/Game/Pump/LD/Bubble/M_Bubble_Disto_Medium_ON.M_Bubble_Disto_Medium_ON" :`NewEnumerator2` "/Game/Pump/LD/Bubble/M_Bubble_Disto_Liquid_ON.M_Bubble_Disto_Liquid_ON" :!type "MaterialInterface Object Reference"))
      (`MaterialInstanceDynamic.SetVectorParameterValue` (`self.MaterialInstance`) "Color" _returnvalue)
      (`/Game/Pump/Core/BP_LevelManager.OnABubbleIsEnteredForFirstTIme` (`self.LevelManager`) self))))

(event `SetVisiblity`
  (params (`New Visibility` :type Boolean))
  (`self.SetActorHiddenInGame` (not `New Visibility`))
  (`self.SetActorEnableCollision` `New Visibility`)
  (`self.SetActorTickEnabled` `New Visibility`))

(event `OnIsLeaved`
  (bind _psoundmanager (`self.pSoundManager`))
  (bind _ispumping (`/Game/Pump/Core/Character/BP_GravityCharacter_Pump.IsPumping` (`self.pChar`)))
  ;[1 1 1] On Leave And Pump
  (if (`self.HasBeenLeavedOnce`)
    (if _ispumping
      (bind _output_get (set `self.HasBeenLeavedOnceInPump` true))
      (`/Game/Pump/Core/SoundSystem/Bp_SoundSystem.OnBubbleEnter` _psoundmanager false self _output_get))
    (else
      (set `self.HasBeenLeavedOnce` true)
      (if _ispumping
        (bind _output_get_2 (set `self.HasBeenLeavedOnceInPump` true))
        (`/Game/Pump/Core/SoundSystem/Bp_SoundSystem.OnBubbleEnter` _psoundmanager false self _output_get_2)))))

(fn `REF_Char`
  (set `self.pChar` (`/Game/Pump/Core/BP_FunctionLibrary.GetCharMatter`)))

(fn `REF_SoundManager`
  (set `self.pSoundManager` (`/Game/Pump/Core/BP_FunctionLibrary.GetSoundSystem`)))

(fn `SecuEnterExitSphere`
  (params (Enter :type Boolean))
  (bind _sphere (`self.Sphere`))
  (if (`self.DisableSecuEnterExitSphere`)
    _
    (elif Enter
      (`SphereComponent.SetSphereRadius` _sphere (+ (`SphereComponent.SphereRadius` _sphere) 10.0) false)
      (else
        (`SphereComponent.SetSphereRadius` (`self.Sphere`) (`self.SaveInitialRadius`) false)))))

(fn `SetMaterialInstance`
  (params (SourceMat :type "MaterialInterface Object Reference"))
  (bind _output_get (set `self.SourceMat` SourceMat))
  (bind _returnvalue (`PrimitiveComponent.CreateDynamicMaterialInstance` (`self.Visual`) 0 _output_get "None"))
  (set `self.MaterialInstance` _returnvalue))

(fn `SetScaleUsingRadius`
  (bind _output_get (set `self.SphereScale` (* (0.5 0.5 0.5) (`self.Radius`))))
  (`SceneComponent.SetRelativeScale3D` (`self.Sphere`) _output_get)
  (`SceneComponent.SetWorldScale3D` (`self.Visual`) _output_get))

(fn `UserConstructionScript`
  (locals (DynamicMat :type "MaterialInstanceDynamic Object Reference"))
  (set `self.Damping` (select `/Game/Pump/LD/Bubble/E_Density` (`self.BubbleDensity`) :`NewEnumerator0` 30.0 :`NewEnumerator1` 0.6 :`NewEnumerator2` 1.5 :!type "Float (single-precision)"))
  (`MaterialInstanceDynamic.SetVectorParameterValue` (`self.MaterialInstance`) "Color" (select `bool` (`self.UseCRV`) :`false` (`self.ColorWhenEntered`) :`true` (`CurveLinearColor.GetLinearColorValue` (`self.CRV_DashZoneColorByDamping`) (`KismetMathLibrary.MapRangeUnclamped` (`self.Damping`) 0.0 35.0 0.0 1.0))))
  (`self.SetScaleUsingRadius`))