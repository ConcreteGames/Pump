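; Bubble step that the player can validate to make its sphere grow, with overridable hooks for growth events.
; Once entered, its center glows brighter as the player nears and the interaction collider turns toward them.
; Overlapping that collider toggles interaction on BP_GravityCharacter_Pump.
; ValidateStep triggers camera shake and a material flash, while a curve-driven timeline scales the sphere toward a MaxRadius-based size over GrowthDuration.
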(event `self.ReceiveBeginPlay`
  (`self.SetCenterMaterialParams` 10000000.0 -1.0 -1.0))

(event `self.ReceiveTick`
  (params (DeltaSeconds :type "Float (single-precision)"))
  (`parent.ReceiveTick` DeltaSeconds)
  (if (and (`self.PlayerIsEntered`) (not (`self.IsValidated`)))
    (`self.AnimateCenterAccordingToPlayerDistance`)))

(event `ValidateStep`
  (set `self.IsValidated` true)
  (`self.OnGrowthStart`)
  (`TimelineComponent.SetTimelineLength` (`self.GrowthTimeline`) (`self.GrowthDuration`))
  (`Timeline|GrowthTimeline` :!via `PlayFromStart`
    (:`Update`
      (`SceneComponent.SetRelativeScale3D` (`self.Sphere`) (`KismetMathLibrary.VLerp` (`self.StartScale`) (* (0.5 0.5 0.5) (`self.MaxRadius`)) (`CurveFloat.GetFloatValue` (`self.CRV_Bubble_Step_Growth`) (`/Game/Pump/Core/BP_FunctionLibrary.GetTimelinePercentage` (`self.GrowthTimeline`)))))
      (`self.OnIsGrowing`))
    (:`Finished`
      (`self.OnGrowthHasEnded`))))

(event `self.OnIsEntered`
  (`parent.OnIsEntered`)
  (set `self.PlayerIsEntered` true))

(event `OnGrowthHasEnded`)

(event `OnIsGrowing`)

(event `OnGrowthStart`
  ;[1 1 1] Light Explosion Animation
  (`GameplayStatics.PlayWorldCameraShake` "/Game/Pump/Core/Character/CS_Pump.CS_Pump_C" (`self.GetCenter`) 0.0 10000000.0)
  (`TimelineComponent.SetTimelineLength` (`self.FlashOnGrowth`) 1.5)
  (`Timeline|FlashOnGrowth` :!via `PlayFromStart`
    (:`Update`
      (`self.SetCenterMaterialParams` (`KismetMathLibrary.MapRangeClamped` (`/Game/Pump/Core/BP_FunctionLibrary.GetTimelinePercentage` (`self.FlashOnGrowth`)) 0.0 1.0 0.0 10000.0)))
    (:`Finished`
      (`self.SetCenterMaterialParams` 0.0 1.0 5.0 0.2))))

(event `self.SphereColl_Interaction.OnComponentBeginOverlap`
  (params (OverlappedComponent :type "PrimitiveComponent Object Reference") (OtherActor :type "Actor Object Reference") (OtherComp :type "PrimitiveComponent Object Reference") (OtherBodyIndex :type Integer) (bFromSweep :type Boolean) (SweepResult :type "HitResult Structure (by ref)"))
  (bind _asbp_gravity_character_pump (cast `/Game/Pump/Core/Character/BP_GravityCharacter_Pump` OtherActor))
  (`/Game/Pump/Core/Character/BP_GravityCharacter_Pump.CanInteractWithBubbleStep` _asbp_gravity_character_pump true)
  (set `self.PlayerIsInValidationRadius` true))

(event `self.SphereColl_Interaction.OnComponentEndOverlap`
  (params (OverlappedComponent :type "PrimitiveComponent Object Reference") (OtherActor :type "Actor Object Reference") (OtherComp :type "PrimitiveComponent Object Reference") (OtherBodyIndex :type Integer))
  (bind _asbp_gravity_character_pump (cast `/Game/Pump/Core/Character/BP_GravityCharacter_Pump` OtherActor))
  (`/Game/Pump/Core/Character/BP_GravityCharacter_Pump.CanInteractWithBubbleStep` _asbp_gravity_character_pump false)
  (set `self.PlayerIsInValidationRadius` false))

(fn `AnimateCenterAccordingToPlayerDistance`
  (bind _spherecoll_interaction (`self.SphereColl_Interaction`))
  (bind _asbp_gravity_character_pump (cast `/Game/Pump/Core/Character/BP_GravityCharacter_Pump` (`GameplayStatics.GetPlayerPawn` 0)))
  (bind _returnvalue (`self.K2_GetActorLocation` _asbp_gravity_character_pump))
  (`self.SetCenterMaterialParams` 0.0 (`KismetMathLibrary.Lerp` 200.0 5.0 (`KismetMathLibrary.MapRangeClamped` (`KismetMathLibrary.VSize` (- _returnvalue (`self.K2_GetActorLocation`))) 200.0 600.0 0.0 1.0)) 2.0)
  (`SceneComponent.K2_SetRelativeRotation` _spherecoll_interaction (`KismetMathLibrary.FindLookAtRotation` (`SceneComponent.K2_GetComponentLocation` _spherecoll_interaction) _returnvalue) false false))

(fn `GetCenter`
  (returns (ReturnValue :type "Vector Structure"))
  (return (- (`SceneComponent.K2_GetComponentLocation` (`self.SphereColl_Interaction`)) (0.0 0.0 75.0))))

(fn `GetDynamicMaterialInstance`
  (params (Target :type "PrimitiveComponent Object Reference"))
  (returns (Output_Get :type "MaterialInstanceDynamic Object Reference"))
  (`/Engine/EditorBlueprintResources/StandardMacros.IsValid` (`self.DynamicCenterMaterial`)
    (:`Is Valid`
      _)
    (:`Is Not Valid`
      (bind _returnvalue (`PrimitiveComponent.CreateDynamicMaterialInstance` Target 0 "/Game/Pump/LD/Bubble/M_GlowBase_Animated_BubbleCenter.M_GlowBase_Animated_BubbleCenter" "None"))
      (set `self.DynamicCenterMaterial` _returnvalue)))
  (return (`self.DynamicCenterMaterial`)))

(fn `UserConstructionScript`
  (bind _returnvalue (`PrimitiveComponent.CreateDynamicMaterialInstance` (`self.Visual`) 0 (`self.SourceMat`) "None"))
  (set `self.MaterialInstance` _returnvalue)
  (`parent.UserConstructionScript`)
  (set `self.StartScale` (`SceneComponent.RelativeScale3D` (`self.Sphere`))))