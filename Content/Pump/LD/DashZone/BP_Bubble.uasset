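; BP_Bubble is a bubble volume for the dash zone that tells the gravity character when it enters and exits.
; Its sphere overlaps call EnterBubble and ExitBubble on BP_GravityCharacter_Pump, with the exit using a cached player pawn rather than the overlapping actor.
; The construction script creates a dynamic material colored from a damping-driven color curve or the entered color.
; The first entrance permanently flags the bubble and applies the entered color; external events can set its color and manager.
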(event `SetDefaultState`
  (params (NewParam :type "LinearColor Structure"))
  (`MaterialInstanceDynamic.SetVectorParameterValue` (`self.MaterialInstance`) "Color" NewParam))

(event `SetBubbleManager`
  (params (NewParam :type "/Game/Pump/Core/BP_BubbleManager Object Reference"))
  (set `self.MyBubbleManager` NewParam))

(event `self.Sphere.OnComponentBeginOverlap`
  (params (OverlappedComponent :type "PrimitiveComponent Object Reference") (OtherActor :type "Actor Object Reference") (OtherComp :type "PrimitiveComponent Object Reference") (OtherBodyIndex :type Integer) (bFromSweep :type Boolean) (SweepResult :type "HitResult Structure (by ref)"))
  (bind _asbp_gravity_character_pump (cast `/Game/Pump/Core/Character/BP_GravityCharacter_Pump` OtherActor))
  (`/Game/Pump/Core/Character/BP_GravityCharacter_Pump.EnterBubble` _asbp_gravity_character_pump self)
  (`self.OnIsEntered`))

(event `self.Sphere.OnComponentEndOverlap`
  (params (OverlappedComponent :type "PrimitiveComponent Object Reference") (OtherActor :type "Actor Object Reference") (OtherComp :type "PrimitiveComponent Object Reference") (OtherBodyIndex :type Integer))
  (`/Game/Pump/Core/Character/BP_GravityCharacter_Pump.ExitBubble` (`self.GetChar`) self))

(event `OnIsEntered`
  (if (not (`self.HasBeenEnteredOnce`))
    (`self.OnFirstEntrance`)))

(event `OnFirstEntrance`
  (set `self.HasBeenEnteredOnce` true)
  (`MaterialInstanceDynamic.SetVectorParameterValue` (`self.MaterialInstance`) "Color" (`self.ColorWhenEntered`)))

(fn `GetChar`
  (returns (Char :type "/Game/Pump/Core/Character/BP_GravityCharacter_Pump Object Reference"))
  (`/Engine/EditorBlueprintResources/StandardMacros.IsValid` (`self.Char`)
    (:`Is Valid`
      _)
    (:`Is Not Valid`
      (set `self.Char` (cast `/Game/Pump/Core/Character/BP_GravityCharacter_Pump` (`GameplayStatics.GetPlayerPawn` 0) :!pure true))))
  (return (`self.Char`)))

(fn `UserConstructionScript`
  (locals (DynamicMat :type "MaterialInstanceDynamic Object Reference"))
  (bind _returnvalue (`PrimitiveComponent.CreateDynamicMaterialInstance` (`self.Visual`) 0 (`self.SourceMat`) "None"))
  (bind _output_get (set `self.MaterialInstance` _returnvalue))
  (`MaterialInstanceDynamic.SetVectorParameterValue` _output_get "Color" (select `bool` (`self.UseCRV`) :`false` (`self.ColorWhenEntered`) :`true` (`CurveLinearColor.GetLinearColorValue` (`self.CRV_DashZoneColorByDamping`) (`KismetMathLibrary.MapRangeUnclamped` (`self.Damping`) 0.0 35.0 0.0 1.0)))))