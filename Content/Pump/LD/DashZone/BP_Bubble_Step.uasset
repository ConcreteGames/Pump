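; Bubble step in the DashZone level design that grows its sphere when first entered.
; The parent's first-entrance event triggers ValidateStep, which plays a fixed-length timeline.
; Each update lerps the sphere's scale from its construction-time value toward half of MaxRadius, eased by a float curve sampled at timeline percentage.
; Empty OnIsGrowing and OnGrowthHasEnded events act as hooks during and after growth.
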(event `ValidateStep`
  (`TimelineComponent.SetTimelineLength` (`self.GrowthTimeline`) 5.0)
  (`Timeline|GrowthTimeline` :!via `PlayFromStart`
    (:`Update`
      (`SceneComponent.SetRelativeScale3D` (`self.Sphere`) (`KismetMathLibrary.VLerp` (`self.StartScale`) (* (0.5 0.5 0.5) (`self.MaxRadius`)) (`CurveFloat.GetFloatValue` (`self.CRV_Bubble_Step_Growth`) (`/Game/Pump/Core/BP_FunctionLibrary.GetTimelinePercentage` (`self.GrowthTimeline`)))))
      (`self.OnIsGrowing`))
    (:`Finished`
      (`self.OnGrowthHasEnded`))))

(event `OnGrowthHasEnded`)

(event `OnIsGrowing`)

(event `self.OnFirstEntrance`
  (`parent.OnFirstEntrance`)
  (`self.ValidateStep`))

(fn `UserConstructionScript`
  (`parent.UserConstructionScript`)
  (set `self.StartScale` (`SceneComponent.RelativeScale3D` (`self.Sphere`))))