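; BP_DashZone is a level-design zone that notifies listeners when the player's gravity character enters its sphere.
; Sphere overlap checks the other actor against the player pawn cast to BP_GravityCharacter_Pump, then fires the OnCharacterEntersDashZone dispatcher.
; The construction script creates a dynamic material on the visual and tints it from a color curve sampled by the Damping value, so each zone's damping shows by color.
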(event `self.Sphere.OnComponentBeginOverlap`
  (params (OverlappedComponent :type "PrimitiveComponent Object Reference") (OtherActor :type "Actor Object Reference") (OtherComp :type "PrimitiveComponent Object Reference") (OtherBodyIndex :type Integer) (bFromSweep :type Boolean) (SweepResult :type "HitResult Structure (by ref)"))
  (if (== OtherActor (cast `/Game/Pump/Core/Character/BP_GravityCharacter_Pump` (`GameplayStatics.GetPlayerPawn` 0) :!pure true))
    (`self.OnCharacterEntersDashZone`)))

(fn `UserConstructionScript`
  (bind _returnvalue (`PrimitiveComponent.CreateDynamicMaterialInstance` (`self.Visual`) 0 "/Game/Pump/LD/DashZone/M_DashZone.M_DashZone" "None"))
  (`MaterialInstanceDynamic.SetVectorParameterValue` _returnvalue "Color" (`CurveLinearColor.GetLinearColorValue` (`self.CRV_DashZoneColorByDamping`) (`KismetMathLibrary.MapRangeUnclamped` (`self.Damping`) 0.0 35.0 0.0 1.0))))