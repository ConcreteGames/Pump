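; Dash-zone bubble that notifies the gravity character when it enters or leaves its sphere.
; Construction maps the density preset to a damping value, scales the sphere by radius and colours the material from a damping-driven curve or fixed colour.
; SetDefaultState can override that colour; the first entrance restores it and reports the bubble to its BubbleManager.
; End overlap always calls exit on the cached player pawn, whichever actor left.
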(event `self.ReceiveBeginPlay`)

(event `SetDefaultState`
  (params (NewParam :type "LinearColor Structure"))
  (`MaterialInstanceDynamic.SetVectorParameterValue` (`self.MaterialInstance`) "Color" NewParam))

(event `SetBubbleManager`
  (params (NewParam :type "/Game/Pump/Core/BP_BubbleManager Object Reference"))
  (set `self.MyBubbleManager` NewParam))

(event `self.Sphere.OnComponentBeginOverlap`
  (params (OverlappedComponent :type "PrimitiveComponent Object Reference") (OtherActor :type "Actor Object Reference") (OtherComp :type "PrimitiveComponent Object Reference") (OtherBodyIndex :type Integer) (bFromSweep :type Boolean) (SweepResult :type "HitResult Structure (by ref)"))
  (bind _asbp_gravity_character_pump (cast `/Game/Pump/Core/Character/BP_GravityCharacter_Pump` OtherActor))
  (`/Game/Pump/Core/Character/BP_GravityCharacter_Pump.EnterBubble` _asbp_gravity_character_pump self)
  (`self.OnIsEntered`))

(event `self.Sphere.OnComponentEndOverlap`
  (params (OverlappedComponent :type "PrimitiveComponent Object Reference") (OtherActor :type "Actor Object Reference") (OtherComp :type "PrimitiveComponent Object Reference") (OtherBodyIndex :type Integer))
  (`/Game/Pump/Core/Character/BP_GravityCharacter_Pump.ExitBubble` (`self.GetChar`) self))

(event `OnIsEntered`
  (if (not (`self.HasBeenEnteredOnce`))
    (`self.OnFirstEntrance`)))

(event `OnFirstEntrance`
  (set `self.HasBeenEnteredOnce` true)
  (`MaterialInstanceDynamic.SetVectorParameterValue` (`self.MaterialInstance`) "Color" (select `bool` (`self.UseCRV`) :`false` (`self.ColorWhenEntered`) :`true` (`CurveLinearColor.GetLinearColorValue` (`self.CRV_DashZoneColorByDamping`) (`KismetMathLibrary.MapRangeUnclamped` (`self.Damping`) 0.0 35.0 0.0 1.0))))
  (`/Game/Pump/Core/BP_BubbleManager.OnABubbleIsEnteredForFirstTIme` (`self.MyBubbleManager`) self))

(fn `GetChar`
  (returns (Char :type "/Game/Pump/Core/Character/BP_GravityCharacter_Pump Object Reference"))
  (`/Engine/EditorBlueprintResources/StandardMacros.IsValid` (`self.Char`)
    (:`Is Valid`
      _)
    (:`Is Not Valid`
      (set `self.Char` (cast `/Game/Pump/Core/Character/BP_GravityCharacter_Pump` (`GameplayStatics.GetPlayerPawn` 0) :!pure true))))
  (return (`self.Char`)))

(fn `UserConstructionScript`
  (locals (DynamicMat :type "MaterialInstanceDynamic Object Reference"))
  (set `self.Damping` (select `/Game/Pump/LD/DashZone/E_Density` (`self.BubbleDensity`) :`NewEnumerator0` 35.0 :`NewEnumerator1` 17.5 :!type "Float (single-precision)"))
  (`MaterialInstanceDynamic.SetVectorParameterValue` (`self.MaterialInstance`) "Color" (select `bool` (`self.UseCRV`) :`false` (`self.ColorWhenEntered`) :`true` (`CurveLinearColor.GetLinearColorValue` (`self.CRV_DashZoneColorByDamping`) (`KismetMathLibrary.MapRangeUnclamped` (`self.Damping`) 0.0 35.0 0.0 1.0))))
  (`SceneComponent.SetRelativeScale3D` (`self.Sphere`) (* (0.5 0.5 0.5) (`self.Radius`))))