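; Level-design spline actor for flying rocks that follows a chosen point range of the referenced red line spline.
; FitToRedLine matches its point count to that range, moves the actor to the first point, and copies locations, tangents and up vectors.
; The construction script walks a slightly wider range in distance steps, passing each segment to a rock destroyer's line trace, apparently clearing colliding HISM rocks.
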(event `FitToRedLine`
  (bind _spline (`self.Spline`))
  (bind _spline_2 (`self.Spline`))
  (bind _spline_3 (`self.Spline`))
  (bind _editredline_firstpointindex (`self.EDITRedLine_FirstPointIndex`))
  (bind _currentindex (`self.CurrentIndex`))
  (bind _returnvalue (- (`self.CurrentIndex`) (`self.EDITRedLine_FirstPointIndex`)))
  (bind _returnvalue_2 (`SplineComponent.GetNumberOfSplinePoints` _spline))
  (bind _spline_4 (`/Game/Pump/LD/RedLine/BP_RedLineSpline.Spline` (`self.pRedLine`)))
  (while (< (`SplineComponent.GetNumberOfSplinePoints` _spline_2) (+ (`self.EDITNumberOfPointsToFollow`) 1))
    (`SplineComponent.AddSplinePoint` _spline_2 (0.0 0.0 0.0) "Local" true))
  (while (> _returnvalue_2 (+ (`self.EDITNumberOfPointsToFollow`) 1))
    (`SplineComponent.RemoveSplinePoint` _spline (- _returnvalue_2 1) true))
  (for _index (range _editredline_firstpointindex (+ (+ _editredline_firstpointindex (`self.EDITNumberOfPointsToFollow`)) 1))
    (set `self.CurrentIndex` _index)
    (if (== (`self.CurrentIndex`) (`self.EDITRedLine_FirstPointIndex`))
      (bind (_returnvalue_location _returnvalue_rotation) (`KismetMathLibrary.BreakTransform` (`SplineComponent.GetTransformAtSplinePoint` (`/Game/Pump/LD/RedLine/BP_RedLineSpline.Spline` (`self.pRedLine`)) _index "World" true)))
      (`self.K2_SetActorTransform` (`KismetMathLibrary.MakeTransform` _returnvalue_location _returnvalue_rotation) false true))
    (`SplineComponent.SetTangentAtSplinePoint` _spline_3 _returnvalue (`SplineComponent.GetTangentAtSplinePoint` _spline_4 _currentindex "World") "World" true)
    (`SplineComponent.SetLocationAtSplinePoint` _spline_3 _returnvalue (`SplineComponent.GetLocationAtSplinePoint` _spline_4 _currentindex "World") "World" true)
    (`SplineComponent.SetUpVectorAtSplinePoint` _spline_3 _returnvalue (`SplineComponent.GetUpVectorAtSplinePoint` _spline_4 _currentindex "World") "World" true)))

(fn `InitParser`
  (bind _spline (`/Game/Pump/LD/RedLine/BP_RedLineSpline.Spline` (`self.pRedLine`)))
  (bind _output_get (set `self.SplineParser_Distance_Init` (`SplineComponent.GetDistanceAlongSplineAtSplinePoint` _spline (- (`self.EDITRedLine_FirstPointIndex`) 10))))
  (bind _output_get_2 (set `self.SplineParser_Distance_End` (`SplineComponent.GetDistanceAlongSplineAtSplinePoint` _spline (+ (`self.EDITRedLine_FirstPointIndex`) (`self.EDITNumberOfPointsToFollow`) 1))))
  (set `self.SplineParser_Distance_Current` (`self.SplineParser_Distance_Init`)))

(fn `KillCollidingRockHISM`
  (bind _spline (`/Game/Pump/LD/RedLine/BP_RedLineSpline.Spline` (`self.pRedLine`)))
  (`/Game/Pump/MatLab/BP_RockDestoyerAlongSpline.TraceLine` (`self.pRockDestoyerAlongSpline`) (`SplineComponent.GetLocationAtDistanceAlongSpline` _spline (`self.SplineParser_Distance_PreviousFrame`) "World") (`SplineComponent.GetLocationAtDistanceAlongSpline` _spline (`self.SplineParser_Distance_Current`) "World")))

(fn `UpdateParser`
  (set `self.SplineParser_Distance_PreviousFrame` (`self.SplineParser_Distance_Current`))
  (set `self.SplineParser_Distance_Current` (+ (`self.SplineParser_Distance_Current`) (`self.SplineParser_Distance_Step`))))

(fn `UserConstructionScript`
  (`parent.UserConstructionScript`)
  (`self.InitParser`)
  (`self.UpdateParser` :!label _label)
  (`self.KillCollidingRockHISM`)
  (if (not (> (`self.SplineParser_Distance_Current`) (`self.SplineParser_Distance_End`)))
    (goto _label)))