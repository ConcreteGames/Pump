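; Spawner that scatters flying rock decoration around the level's planet steps as instanced static meshes.
; Init takes PlanetSteps from the level manager, then adds many medium and a few huge randomly scaled rocks in a shell around each step, picking among five instance components.
; A second path places big rocks around BP_CriticalPathSpline actors with a spline clearance check, but its calling chain is disconnected, as is a random scatter around the spawner.
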(event `Init`
  (params (LevelManager :type "/Game/Pump/Core/BP_LevelManager Object Reference"))
  (bind _output_get (set `self.pLevelManager` LevelManager))
  (set `self.PlanetSteps` (`/Game/Pump/Core/BP_LevelManager.PlanetSteps` _output_get))
  (`self.SpawnRocksAroundSteps`))

(event `SpawnRocksAroundSteps`
  (bind _returnvalue (select `int` (`KismetMathLibrary.RandomIntegerInRange` 0 4) :`0` (`self.MiddleRockInstance_1`) :`1` (`self.MiddleRockInstance_2`) :`2` (`self.MiddleRockInstance_3`) :`3` (`self.MiddleRockInstance_4`) :`4` (`self.MiddleRockInstance_5`)))
  (bind _returnvalue_2 (select `int` (`KismetMathLibrary.RandomIntegerInRange` 0 4) :`0` (`self.MiddleRockInstance_1`) :`1` (`self.MiddleRockInstance_2`) :`2` (`self.MiddleRockInstance_3`) :`3` (`self.MiddleRockInstance_4`) :`4` (`self.MiddleRockInstance_5`)))
  (for _array_element (`self.PlanetSteps`)
    (for _ (range 501)
      (`/Engine/EditorBlueprintResources/StandardMacros.IsValid` _returnvalue_2
        (:`Is Valid`
          (bind _returnvalue_3 (`self.K2_GetActorLocation` _array_element))
          (bind _returnvalue_4 (+ _returnvalue_3 (* (`KismetMathLibrary.RandomUnitVector`) (`KismetMathLibrary.RandomFloatInRange` 6000.0 12000.0))))
          (bind _returnvalue_5 (`KismetMathLibrary.FindLookAtRotation` _returnvalue_3 _returnvalue_4))
          (`InstancedStaticMeshComponent.AddInstanceWorldSpace` _returnvalue_2 (`KismetMathLibrary.MakeTransform` _returnvalue_4 _returnvalue_5 (`KismetMathLibrary.VLerp` (4.0 4.0 4.0) (10.0 10.0 10.0) (`KismetMathLibrary.RandomFloat`)))))))
    (for _ (range 11)
      (`/Engine/EditorBlueprintResources/StandardMacros.IsValid` _returnvalue
        (:`Is Valid`
          (`InstancedStaticMeshComponent.AddInstanceWorldSpace` _returnvalue (`KismetMathLibrary.MakeTransform` _returnvalue_4 _returnvalue_5 (`KismetMathLibrary.VLerp` (30.0 30.0 30.0) (40.0 40.0 40.0) (`KismetMathLibrary.RandomFloat`)))))))))

(event `SpawnFloatingRocks`)

(event `CollectSplineSpawners`
  (bind _outactors (`GameplayStatics.GetAllActorsOfClass` "/Game/Pump/LD/FlyingRocksSpawner/BP_CriticalPathSpline.BP_CriticalPathSpline_C"))
  (set `self.SplineObjectSpawners` _outactors))

(event `SpawnRocksOnSplineSpawners`
  (for _array_element (`self.SplineObjectSpawners`)
    (set `self.CurrentSpline` (`/Game/Pump/LD/FlyingRocksSpawner/BP_CriticalPathSpline.Spline` _array_element))
    (set `self.CurrentQuantity` (`/Game/Pump/LD/FlyingRocksSpawner/BP_CriticalPathSpline.Quantity` _array_element))
    (`self.SpawnForCurrentSpline`)))

(event `SpawnForCurrentSpline`
  (bind _returnvalue (`self.GetRandomBigRockInstance`))
  (bind _returnvalue_2 (`KismetMathLibrary.VLerp` (3.0 3.0 3.0) (5.0 5.0 5.0) (`KismetMathLibrary.RandomFloat`)))
  (bind _returnvalue_3 (* (`SplineComponent.GetSplineLength` (`self.CurrentSpline`)) (`KismetMathLibrary.RandomFloat`)))
  (bind _returnvalue_4 (+ (`SplineComponent.GetLocationAtDistanceAlongSpline` (`self.CurrentSpline`) _returnvalue_3 "World") (* (`KismetMathLibrary.Normal` (`KismetMathLibrary.ProjectVectorOnToPlane` (`KismetMathLibrary.RandomUnitVector`) (`KismetMathLibrary.Normal` (`SplineComponent.GetTangentAtDistanceAlongSpline` (`self.CurrentSpline`) _returnvalue_3 "World")))) (+ (* (.x _returnvalue_2) 1000.0) (`KismetMathLibrary.RandomFloatInRange` 5000.0 10000.0)))))
  (for _ (range 1 (+ (`self.CurrentQuantity`) 1))
    (bind _returnvalue_5 (`self.CheckDistanceFromSpline` _returnvalue_4 3000.0))
    (if _returnvalue_5
      (`/Engine/EditorBlueprintResources/StandardMacros.IsValid` _returnvalue
        (:`Is Valid`
          (`InstancedStaticMeshComponent.AddInstanceWorldSpace` _returnvalue (`KismetMathLibrary.MakeTransform` _returnvalue_4 (struct) _returnvalue_2)))))))

(fn `CheckDistanceFromSpline`
  (params (Location :type "Vector Structure") (Distance :type "Float (double-precision)"))
  (returns (ReturnValue :type Boolean))
  (locals (NewLocalVar_0 :type Integer) (NewLocalVar_1 :type "Float (double-precision)"))
  (bind _closestpointlocation (`self.GetClosestSplinePointLocation` Location))
  (return (>= (`KismetMathLibrary.VSize` (- _closestpointlocation Location)) Distance)))

(fn `GetClosestSplinePointLocation`
  (params (WorldLocation :type "Vector Structure"))
  (returns (ClosestPointLocation :type "Vector Structure"))
  (locals (BestDistance :type "Float (double-precision)" :default 1.1515844984674714e+19) (BestIndex :type Integer))
  (bind _bestdistance (`local.BestDistance`))
  (bind _instancedstaticmesh (`self.InstancedStaticMesh`))
  (bind _returnvalue (`SplineComponent.GetLocationAtSplinePoint` (`self.CurrentSpline`) (`local.BestIndex`) "World"))
  (for _index (range (+ (`SplineComponent.GetNumberOfSplinePoints` (`self.CurrentSpline`)) 1))
    (if (<= (`KismetMathLibrary.VSize` (- (`SplineComponent.GetLocationAtSplinePoint` (`self.CurrentSpline`) _index "Local") WorldLocation)) _bestdistance)
      (set `local.BestDistance` _bestdistance)
      (set `local.BestIndex` _index)))
  (`/Engine/EditorBlueprintResources/StandardMacros.IsValid` _instancedstaticmesh
    (:`Is Valid`
      (`InstancedStaticMeshComponent.AddInstanceWorldSpace` _instancedstaticmesh (`KismetMathLibrary.MakeTransform` _returnvalue (struct) (30.0 30.0 30.0)))
      (return _returnvalue))))

(fn `GetRandomBigRockInstance`
  (returns (ReturnValue :type "InstancedStaticMeshComponent Object Reference"))
  (bind _bigrockinstance_3 (`self.BigRockInstance_3`))
  (return (select `int` (`KismetMathLibrary.RandomIntegerInRange` 0 1) :`0` _bigrockinstance_3 :`1` _bigrockinstance_3 :`2` _bigrockinstance_3)))

(fn `GetRandomMiddleRockInstance`
  (returns (ReturnValue :type "InstancedStaticMeshComponent Object Reference"))
  (return (select `int` (`KismetMathLibrary.RandomIntegerInRange` 0 4) :`0` (`self.MiddleRockInstance_1`) :`1` (`self.MiddleRockInstance_2`) :`2` (`self.MiddleRockInstance_3`) :`3` (`self.MiddleRockInstance_4`) :`4` (`self.MiddleRockInstance_5`))))

(fn `GetRandomRotator`
  (returns (ReturnValue :type "Rotator Structure"))
  (return (`KismetMathLibrary.MakeRotator` (* (`KismetMathLibrary.RandomFloat`) 360.0) (* (`KismetMathLibrary.RandomFloat`) 360.0) (* (`KismetMathLibrary.RandomFloat`) 360.0))))

(fn `RecursiveDistanceCheck`
  (params (Iteration :type Integer) (StartTime :type "Float (double-precision)") (EndTime :type "Float (double-precision)") (Location :type "Vector Structure"))
  (returns (BestTime :type "Float (double-precision)"))
  (locals (Start :type "Float (double-precision)") (End :type "Float (double-precision)") (Best :type "Float (double-precision)") (Num :type Integer) (StartDistance :type "Float (double-precision)") (EndDistance :type "Float (double-precision)") (DistanceThreshold :type "Float (double-precision)" :default 100.0))
  (bind _currentspline (`self.CurrentSpline`))
  (bind _location (`local.Location`))
  (bind _returnvalue (`KismetMathLibrary.Lerp` (`local.Start`) (`local.End`) 0.5))
  (set `local.Num` Iteration)
  (set `local.Start` StartTime)
  (set `local.End` EndTime)
  (set `local.StartDistance` (`KismetMathLibrary.VSize` (- (`SplineComponent.GetLocationAtTime` _currentspline (`local.Start`) "World" true) _location)))
  (set `local.EndDistance` (`KismetMathLibrary.VSize` (- (`SplineComponent.GetLocationAtTime` _currentspline (`local.End`) "World" true) _location)))
  (if (< (`local.StartDistance`) (`local.EndDistance`))
    (if (<= (`local.Num`) 0)
      (set `local.Best` (`local.Start`) :!label _label)
      (else
        (`/Engine/EditorBlueprintResources/StandardMacros.DecrementInt` (`local.Num`)
          (:`  `
            (if (<= (`local.StartDistance`) (`local.DistanceThreshold`))
              (goto _label)
              (else
                (bind _besttime (`self.RecursiveDistanceCheck` (`local.Num`) (`local.Start`) _returnvalue (`local.Location`)))
                (set `local.Best` _besttime)))))))
    (elif (<= (`local.Num`) 0)
      (set `local.Best` (`local.End`) :!label _label_2)
      (else
        (`/Engine/EditorBlueprintResources/StandardMacros.DecrementInt` (`local.Num`)
          (:`  `
            (if (<= (`local.EndDistance`) (`local.DistanceThreshold`))
              (goto _label_2)
              (else
                (bind _besttime_2 (`self.RecursiveDistanceCheck` (`local.Num`) _returnvalue (`local.End`) (`local.Location`)))
                (set `local.Best` _besttime_2))))))))
  (return (`local.Best`)))

(fn `UserConstructionScript`)