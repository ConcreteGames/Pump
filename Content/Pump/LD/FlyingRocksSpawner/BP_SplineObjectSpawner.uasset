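; Spawns flying rocks around a spline at BeginPlay as instances of one InstancedStaticMesh.
; About a thousand attempts each pick a random spline point, offset it perpendicular to the tangent by a scale-derived radius, and face it outward.
; An instance is added only when the closest-spline distance is below that radius, and each check is logged.
; Random pure nodes re-roll per executed node, so logged, tested and spawned points differ.
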(event `self.ReceiveBeginPlay`
  (`self.SpawnRocksAlongSpline`))

(event `SpawnRocksAlongSpline`
  (bind _spline (`self.Spline`))
  (bind _returnvalue (`KismetMathLibrary.VLerp` (40.0 40.0 120.0) (40.0 40.0 120.0) (`KismetMathLibrary.RandomFloat`)))
  (bind _returnvalue_2 (* (`SplineComponent.GetSplineLength` (`self.Spline`)) (`KismetMathLibrary.RandomFloat`)))
  (bind _returnvalue_3 (`SplineComponent.GetLocationAtDistanceAlongSpline` _spline _returnvalue_2 "World"))
  (bind _returnvalue_4 (+ (* (.x _returnvalue) 100.0) (`KismetMathLibrary.RandomFloatInRange` 0.0 0.0)))
  (bind _returnvalue_5 (+ _returnvalue_3 (* (`KismetMathLibrary.Normal` (`KismetMathLibrary.ProjectVectorOnToPlane` (`KismetMathLibrary.RandomUnitVector`) (`KismetMathLibrary.Normal` (`SplineComponent.GetTangentAtDistanceAlongSpline` _spline _returnvalue_2 "World")))) _returnvalue_4)))
  (bind _returnvalue_6 (`KismetMathLibrary.VSize` (- (`SplineComponent.FindLocationClosestToWorldLocation` (`self.Spline`) _returnvalue_5 "World") _returnvalue_5)))
  (for _ (range 1001)
    (`/Game/Pump/Core/BP_FunctionLibrary.LogErer` "" (`KismetStringLibrary.Conv_DoubleToString` _returnvalue_6))
    (if (not (>= _returnvalue_6 _returnvalue_4))
      (`InstancedStaticMeshComponent.AddInstanceWorldSpace` (`self.InstancedStaticMesh`) (`KismetMathLibrary.MakeTransform` _returnvalue_5 (`KismetMathLibrary.FindLookAtRotation` _returnvalue_3 _returnvalue_5) _returnvalue)))))

(fn `UserConstructionScript`)