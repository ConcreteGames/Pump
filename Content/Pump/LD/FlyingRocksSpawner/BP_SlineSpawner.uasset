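; Spline-based scatter tool that places instanced meshes along a spline, apparently for flying rocks in level dressing.
; The construction script creates a shadowless HISM component per mesh, then adds each instance to a randomly picked one.
; Instances are spaced evenly or randomly, offset vertically or around the spline tangent, with configurable rotation and random scale.
; A VisualHelper instance marks each spline point, and the event graph is empty.
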(fn `DisplayEditorHelpers`
  (bind _spline (`self.Spline`))
  (for _index (range (+ (`SplineComponent.GetNumberOfSplinePoints` _spline) 1))
    (`InstancedStaticMeshComponent.AddInstanceWorldSpace` (`self.VisualHelper`) (`KismetMathLibrary.MakeTransform` (`SplineComponent.GetLocationAtSplinePoint` _spline _index "World") (struct) (100.0 100.0 100.0)))))

(fn `GetRandomRotator`
  (returns (ReturnValue :type "Rotator Structure"))
  (return (`KismetMathLibrary.MakeRotator` (* (`KismetMathLibrary.RandomFloat`) 360.0) (* (`KismetMathLibrary.RandomFloat`) 360.0) (* (`KismetMathLibrary.RandomFloat`) 360.0))))

(fn `SetInstanciatedMeshes`
  (locals (NewHISM :type "HierarchicalInstancedStaticMeshComponent Object Reference"))
  (for _array_element (`self.Meshes`)
    (bind _returnvalue (`AddComponent|NODE_AddHierarchicalInstancedStaticMeshComponent-1`))
    (set `local.NewHISM` _returnvalue)
    (`StaticMeshComponent.SetStaticMesh` (`local.NewHISM`) _array_element)
    (`PrimitiveComponent.SetCastShadow` (`local.NewHISM`) false)
    (`KismetArrayLibrary.Array_AddUnique` (`self.HInstanciatedStaticMeshes`) (`local.NewHISM`))))

(fn `UserConstructionScript`
  (locals (CurIndex :type Integer))
  (bind _hinstanciatedstaticmeshes (`self.HInstanciatedStaticMeshes`))
  (bind _returnvalue (select `bool` (`self.RandomDistribution`) :`false` (* (/ (`SplineComponent.GetSplineLength` (`self.Spline`)) (`KismetMathLibrary.Conv_IntToDouble` (`self.Quantity`))) (`KismetMathLibrary.Conv_IntToDouble` (`local.CurIndex`))) :`true` (* (`SplineComponent.GetSplineLength` (`self.Spline`)) (`KismetMathLibrary.RandomFloat`))))
  (bind _returnvalue_2 (`SplineComponent.GetLocationAtDistanceAlongSpline` (`self.Spline`) _returnvalue "World"))
  (bind _returnvalue_3 (+ _returnvalue_2 (* (select `bool` (`self.OnlyVerticalDistanceRandom`) :`false` (`KismetMathLibrary.Normal` (`KismetMathLibrary.ProjectVectorOnToPlane` (`KismetMathLibrary.RandomUnitVector`) (`KismetMathLibrary.Normal` (`SplineComponent.GetTangentAtDistanceAlongSpline` (`self.Spline`) _returnvalue "World")))) :`true` (select `bool` (`KismetMathLibrary.RandomBool`) :`false` (`self.GetActorUpVector`) :`true` (* (`self.GetActorUpVector`) -1.0))) (`KismetMathLibrary.RandomFloatInRange` (`self.MinDistance`) (`self.MaxDistance`)))))
  (`self.SetInstanciatedMeshes`)
  (`self.DisplayEditorHelpers`)
  (for _index (range (+ (`self.Quantity`) 1))
    (set `local.CurIndex` _index)
    (`InstancedStaticMeshComponent.AddInstanceWorldSpace` (`|GetArrayItem` _hinstanciatedstaticmeshes (`KismetMathLibrary.RandomIntegerInRange` 0 (`KismetArrayLibrary.Array_LastIndex` _hinstanciatedstaticmeshes))) (`KismetMathLibrary.MakeTransform` _returnvalue_3 (select `bool` (`self.LookAtSpline`) :`false` (select `bool` (`self.RandomRotation`) :`false` (select `bool` (`self.LocalRotation`) :`true` (`self.K2_GetActorRotation`)) :`true` (`self.GetRandomRotator`)) :`true` (`KismetMathLibrary.FindLookAtRotation` _returnvalue_2 _returnvalue_3)) (select `bool` (`self.UniformScale`) :`false` (`KismetMathLibrary.MakeVector` (`KismetMathLibrary.Lerp` (.x (`self.MinScale`)) (.x (`self.MaxScale`)) (`KismetMathLibrary.RandomFloat`)) (`KismetMathLibrary.Lerp` (.y (`self.MinScale`)) (.y (`self.MaxScale`)) (`KismetMathLibrary.RandomFloat`)) (`KismetMathLibrary.Lerp` (.z (`self.MinScale`)) (.z (`self.MaxScale`)) (`KismetMathLibrary.RandomFloat`))) :`true` (`KismetMathLibrary.VLerp` (`self.MinScale`) (`self.MaxScale`) (`KismetMathLibrary.RandomFloat`)))))))