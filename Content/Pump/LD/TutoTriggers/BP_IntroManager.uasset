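; Intro manager that launches the player's Pump character from the actor's location toward the world origin at level start, unless a dev flag disables it.
; During the flight, character collision with world static and dynamic channels is ignored and gravity-platform planes' security collisions are on.
; Tick uses distance to origin to blend character and camera rotations along a curve from values saved on entering range, then restores both collision states near the origin.
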(event `self.ReceiveBeginPlay`
  (bind _returnvalue (`self.K2_GetActorLocation`))
  (bind _character (`/Game/Pump/Core/BP_FunctionLibrary.GetCharPump`))
  (if (not (`self.Dev_DisableIntro`))
    (`self.K2_SetActorLocationAndRotation` _character _returnvalue (`KismetMathLibrary.FindLookAtRotation` _returnvalue (0.0 0.0 0.0)) false true)
    (set `/Game/Pump/Core/Character/BP_GravityCharacter_Pump.IsInIntro` true _character)
    (`/Game/Pump/Core/Character/BP_GravityCharacter_Pump.Pump` _character)
    ;[1 1 1] Remove collision
    (`self.SetCharCollResponse` "ECR_Ignore")
    (`self.SetSecuStateOfAllPlanes` true)))

(event `self.ReceiveTick`
  (params (DeltaSeconds :type "Float (single-precision)"))
  (bind _character (`/Game/Pump/Core/BP_FunctionLibrary.GetCharPump`))
  (bind _returnvalue (+ 40000.0 0.0))
  (bind _camera (`/Game/Pump/Core/Character/BP_GravityCharacter_Pump.Camera` _character))
  (bind _returnvalue_2 (`KismetMathLibrary.VSize` (`self.K2_GetActorLocation` (`/Game/Pump/Core/BP_FunctionLibrary.GetCharPump`))))
  (bind _returnvalue_3 (`CurveFloat.GetFloatValue` (`self.CRV_IntroRot`) (`KismetMathLibrary.MapRangeClamped` _returnvalue_2 _returnvalue 1000.0 0.0 1.0)))
  (if (not (`self.Dev_DisableIntro`))
    (`|ExecutionSequence`
      (:`then_0`
        (`/Game/Pump/Core/Character/BP_ActorMacroLibrary.BranchTrigger` (< _returnvalue_2 _returnvalue)
          (:`TriggerTrue`
            (set `self.InitCharPumpRot` (`self.K2_GetActorRotation` _character))
            (set `self.InitCameraRot` (`SceneComponent.RelativeRotation` _camera))
            (`/Game/Pump/Core/BP_FunctionLibrary.LogErer` "save rots"))
          (:`True`
            (`self.K2_SetActorRotation` _character (`KismetMathLibrary.RLerp` (`self.InitCharPumpRot`) (struct :`Yaw` 180.0) _returnvalue_3 true) true)
            (`SceneComponent.K2_SetRelativeRotation` _camera (`KismetMathLibrary.RLerp` (`self.InitCameraRot`) (struct :`Roll` -5.0) _returnvalue_3 true) false true)
            (`/Game/Pump/Core/BP_FunctionLibrary.LogErer` "lerping rots"))))
      (:`then_1`
        (`/Game/Pump/Core/Character/BP_ActorMacroLibrary.BranchTrigger` (< (`KismetMathLibrary.VSize` (`self.K2_GetActorLocation` (`/Game/Pump/Core/BP_FunctionLibrary.GetCharPump`))) 1000.0)
          (:`TriggerTrue`
            (`/Game/Pump/Core/BP_FunctionLibrary.LogErer` "sqdsqd")
            ;[1 1 1] Reset collision
            (`self.SetCharCollResponse` "ECR_Block")
            (`self.SetSecuStateOfAllPlanes` false)))))))

(event `SetSecuStateOfAllPlanes`
  (params (ActivateSecu :type Boolean))
  (bind _outactors (`GameplayStatics.GetAllActorsOfClass` "/Game/Pump/LD/GravityPlateform/Plane/BP_GravityPlateform_Plane.BP_GravityPlateform_Plane_C"))
  (for _array_element _outactors
    (if ActivateSecu
      (`/Game/Pump/LD/GravityPlateform/Plane/BP_GravityPlateform_Plane.SecuCollON` _array_element)
      (else
        (`/Game/Pump/LD/GravityPlateform/Plane/BP_GravityPlateform_Plane.SecuCollOFF` _array_element)))))

(fn `SetCharCollResponse`
  (params (NewResponse :type "ECollisionResponse Enum" :default "ECR_Ignore"))
  (bind _walkcollision (`/Game/Pump/Core/Character/BP_GravityCharacter_Pump.WalkCollision` (`/Game/Pump/Core/BP_FunctionLibrary.GetCharPump`)))
  (`PrimitiveComponent.SetCollisionResponseToChannel` _walkcollision "ECC_WorldStatic" NewResponse)
  (`PrimitiveComponent.SetCollisionResponseToChannel` (`/Game/Pump/Core/Character/BP_GravityCharacter_Pump.SideCollision` (`/Game/Pump/Core/BP_FunctionLibrary.GetCharPump`)) "ECC_WorldStatic" NewResponse)
  (`PrimitiveComponent.SetCollisionResponseToChannel` _walkcollision "ECC_WorldDynamic" NewResponse)
  (`PrimitiveComponent.SetCollisionResponseToChannel` (`/Game/Pump/Core/Character/BP_GravityCharacter_Pump.SideCollision` (`/Game/Pump/Core/BP_FunctionLibrary.GetCharPump`)) "ECC_WorldDynamic" NewResponse))

(fn `UserConstructionScript`)