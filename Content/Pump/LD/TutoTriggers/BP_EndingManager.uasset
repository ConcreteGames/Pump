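; Ending manager actor that triggers the final sequence once its four trigger components, laid out in a cross by the construction script, are all on screen.
; While TestFullMoon is set, Tick runs this check, then starts a timeline animating the player's bloom along a curve.
; Past halfway, it spawns randomly placed moon child actors, destroys gravity plane platforms, slowly rotates itself and calls the player's FinalOxy after a delay.
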(event `self.ReceiveTick`
  (params (DeltaSeconds :type "Float (single-precision)"))
  (bind _spawnmoonlocationhelper (`self.SpawnMoonLocationHelper`))
  (bind _t_bloom (`self.T_Bloom`))
  (bind _returnvalue (* 0.02 (`GameplayStatics.GetGlobalTimeDilation`)))
  (if (`self.TestFullMoon`)
    (set `self.NumberOfOnScreenElements` 0)
    (for _array_element (`|MakeArray` (`self.OnScreenTrigger1`) (`self.OnScreenTrigger2`) (`self.OnScreenTrigger3`) (`self.OnScreenTrigger4`))
      (if (`/Game/Pump/Core/BP_FunctionLibrary.IsOnScreen` _array_element)
        (set `self.NumberOfOnScreenElements` (+ (`self.NumberOfOnScreenElements`) 1))))
    (if (== (`self.NumberOfOnScreenElements`) 4)
      (`/Engine/EditorBlueprintResources/StandardMacros.DoOnce` false
        (:`Completed`
          ;[1 1 1] Bloo animation
          (set `self.InitialBloom` (`/Game/Pump/Core/Character/BP_GravityCharacter_Pump.PP_MaxBloomIntensity` (`/Game/Pump/Core/BP_FunctionLibrary.GetCharPump`)))
          (`TimelineComponent.SetTimelineLength` _t_bloom (`self.BloomVariationDuration`))
          (`Timeline|T_Bloom` :!via `PlayFromStart`
            (:`Update`
              (set `/Game/Pump/Core/Character/BP_GravityCharacter_Pump.PP_MaxBloomIntensity` (`KismetMathLibrary.Lerp` (`self.InitialBloom`) (`self.DesiredFinalBloom`) (`CurveFloat.GetFloatValue` (`self.CRV_SkySphereBloom`) (`/Game/Pump/Core/BP_FunctionLibrary.GetTimelinePercentage` _t_bloom))) (`/Game/Pump/Core/BP_FunctionLibrary.GetCharPump`))
              (if (> (`/Game/Pump/Core/BP_FunctionLibrary.GetTimelinePercentage` (`self.T_Bloom`)) 0.5)
                (`/Engine/EditorBlueprintResources/StandardMacros.DoOnce` false
                  (:`Completed`
                    (`|ExecutionSequence`
                      (:`then_0`
                        ;[1 1 1] spawn moons
                        (for _ (range 1 (+ (`self.NumberOfMoons`) 1))
                          (`SceneComponent.K2_SetWorldRotation` _spawnmoonlocationhelper (`KismetMathLibrary.RandomRotator` false) false false)
                          (`AddComponent|NODE_AddChildActorComponent-1` :`RelativeTransform` (`KismetMathLibrary.MakeTransform` (* (`SceneComponent.GetForwardVector` _spawnmoonlocationhelper) (`KismetMathLibrary.RandomFloatInRange` (`self.MoonMinDistance`) (`self.MoonMaxDistance`)))))))
                      (:`then_1`
                        ;[1 1 1] destroy plateform
                        (bind _outactors (`GameplayStatics.GetAllActorsOfClass` "/Game/Pump/LD/GravityPlateform/Plane/BP_GravityPlateform_Plane.BP_GravityPlateform_Plane_C"))
                        (for _array_element_2 _outactors
                          (`self.K2_DestroyActor` _array_element_2)
                          (`|ExecutionSequence`
                            (:`then_0`
                              (`Timeline|Loop` :!via `PlayFromStart`
                                (:`Update`
                                  (`self.K2_SetActorRotation` (`KismetMathLibrary.ComposeRotators` (`self.K2_GetActorRotation`) (`KismetMathLibrary.MakeRotator` _returnvalue _returnvalue _returnvalue))))))
                            (:`then_1`
                              (`KismetSystemLibrary.Delay` 10.0)
                              (`/Game/Pump/Core/Character/BP_GravityCharacter_Pump.FinalOxy` (`/Game/Pump/Core/BP_FunctionLibrary.GetCharPump`)))))))))))
            (:`Finished`
              (set `self.TestFullMoon` false))))))))

(fn `UserConstructionScript`
  (bind _cubedistance (`self.CubeDistance`))
  (bind _returnvalue (* _cubedistance -1.0))
  (`SceneComponent.K2_SetRelativeLocation` (`self.OnScreenTrigger1`) (`KismetMathLibrary.MakeVector` _cubedistance) false false)
  (`SceneComponent.K2_SetRelativeLocation` (`self.OnScreenTrigger2`) (`KismetMathLibrary.MakeVector` _returnvalue) false false)
  (`SceneComponent.K2_SetRelativeLocation` (`self.OnScreenTrigger3`) (`KismetMathLibrary.MakeVector` 0.0 0.0 _cubedistance) false false)
  (`SceneComponent.K2_SetRelativeLocation` (`self.OnScreenTrigger4`) (`KismetMathLibrary.MakeVector` 0.0 0.0 _returnvalue) false false))