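; One-shot tutorial trigger that redirects the gravity character toward a target point, logged as going to a planet.
; On the first collider overlap by BP_GravityCharacter_Pump, it re-aims the WalkCollision physics velocity at VelocityTargetPoint, preserving speed, and rotates that point along the new direction.
; The construction script positions the target from VelocityTargetPointLocation.
; An unconnected stop-and-delay branch remains unused.
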(event `self.Collider.OnComponentBeginOverlap`
  (params (OverlappedComponent :type "PrimitiveComponent Object Reference") (OtherActor :type "Actor Object Reference") (OtherComp :type "PrimitiveComponent Object Reference") (OtherBodyIndex :type Integer) (bFromSweep :type Boolean) (SweepResult :type "HitResult Structure (by ref)"))
  (`/Game/Pump/Core/BP_FunctionLibrary.LogErer` "col")
  (bind _asbp_gravity_character_pump (cast `/Game/Pump/Core/Character/BP_GravityCharacter_Pump` OtherActor))
  (`/Engine/EditorBlueprintResources/StandardMacros.DoOnce` false
    (:`Completed`
      (`/Game/Pump/Core/BP_FunctionLibrary.LogErer` "GO TO PLANET!!!!")
      (bind _walkcollision (`/Game/Pump/Core/Character/BP_GravityCharacter_Pump.WalkCollision` _asbp_gravity_character_pump))
      (bind _returnvalue (`PrimitiveComponent.GetPhysicsLinearVelocity` _walkcollision "None"))
      (bind _output_get (set `self.CurrentCharVelocityLenght` (`KismetMathLibrary.VSize` _returnvalue)))
      (bind _returnvalue_2 (* (`KismetMathLibrary.Normal` (- (`SceneComponent.K2_GetComponentLocation` (`self.VelocityTargetPoint`)) (`SceneComponent.K2_GetComponentLocation` _walkcollision))) _output_get))
      (`PrimitiveComponent.SetAllPhysicsLinearVelocity` _walkcollision _returnvalue_2 false)
      (`SceneComponent.K2_SetWorldRotation` (`self.VelocityTargetPoint`) (`KismetMathLibrary.Conv_VectorToRotator` _returnvalue_2) false false))))

(fn `UserConstructionScript`
  (bind _velocitytargetpoint (`self.VelocityTargetPoint`))
  (`SceneComponent.K2_SetRelativeLocation` _velocitytargetpoint (`self.VelocityTargetPointLocation`) false false)
  (`SceneComponent.SetWorldScale3D` _velocitytargetpoint (2.0 1.0 1.0)))