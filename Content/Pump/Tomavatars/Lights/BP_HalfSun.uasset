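; BP_HalfSun is a sun light Blueprint that continuously rotates a RectLight and a DirectionalLight in pitch.
; BeginPlay stores each light's initial world pitch.
; Every Tick adds that stored pitch plus a small constant as a world rotation delta, so spin speed depends on starting pitch and frame rate.
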(event `self.ReceiveBeginPlay`
  (bind (_returnvalue_roll _returnvalue_pitch) (`KismetMathLibrary.BreakRotator` (`SceneComponent.K2_GetComponentRotation` (`self.RectLight`))))
  (bind (_returnvalue_roll_2 _returnvalue_pitch_2) (`KismetMathLibrary.BreakRotator` (`SceneComponent.K2_GetComponentRotation` (`self.DirectionalLight`))))
  (set `self.RectLightY` _returnvalue_pitch)
  (set `self.DirLightY` _returnvalue_pitch_2))

(event `self.ReceiveTick`
  (params (DeltaSeconds :type "Float (single-precision)"))
  ;[0.502 1 0.1636] Tick
  ;[1 1 1] Rotate Sun
  (`SceneComponent.K2_AddWorldRotation` (`self.RectLight`) (`KismetMathLibrary.MakeRotator` 0.0 (+ (`self.RectLightY`) 0.1)) false false)
  (`SceneComponent.K2_AddWorldRotation` (`self.DirectionalLight`) (`KismetMathLibrary.MakeRotator` 0.0 (+ (`self.DirLightY`) 0.1)) false false))

(fn `UserConstructionScript`)