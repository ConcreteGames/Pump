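; Trigger actor that transitions the level's exponential height fog to its configured target look on collider overlap or through a ManualFogModifier event.
; INIT takes the first ExponentialHeightFog actor found and snapshots its current density, extinction, inscattering colors, albedo and emissive.
; A timeline, stretched to TransitionDuration, then blends each property from that snapshot to its target.
; The overlap has no actor filter, and nothing restores the original fog.
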(event `self.Collider.OnComponentBeginOverlap`
  (params (OverlappedComponent :type "PrimitiveComponent Object Reference") (OtherActor :type "Actor Object Reference") (OtherComp :type "PrimitiveComponent Object Reference") (OtherBodyIndex :type Integer) (bFromSweep :type Boolean) (SweepResult :type "HitResult Structure (by ref)"))
  (bind _pexponensialheightfogcomponent (`self.pExponensialHeightFogComponent`))
  (bind _pexponensialheightfogcomponent_2 (`self.pExponensialHeightFogComponent`))
  (bind __ (`/Game/Pump/Core/BP_FunctionLibrary.GetTimelinePercentage` (`self.FogTransition`)))
  (`self.INIT` :!label _label)
  (`TimelineComponent.SetTimelineLength` (`self.FogTransition`) (`self.TransitionDuration`))
  (`Timeline|FogTransition` :!via `PlayFromStart`
    (:`Update`
      (`ExponentialHeightFogComponent.SetFogDensity` _pexponensialheightfogcomponent (+ (`self.InitialFogDensity`) (* (- (`self.DesiredFogDensity`) (`self.InitialFogDensity`)) __)))
      (`ExponentialHeightFogComponent.SetVolumetricFogExtinctionScale` _pexponensialheightfogcomponent (+ (`self.InitialFogExtinction`) (* (- (`self.DesiredFogExtinction`) (`self.InitialFogExtinction`)) __)))
      (`ExponentialHeightFogComponent.SetFogInscatteringColor` _pexponensialheightfogcomponent (`KismetMathLibrary.LinearColorLerp` (`self.Initial_FogInscatteringColor`) (`self.FogInscatteringColor`) __))
      (`ExponentialHeightFogComponent.SetDirectionalInscatteringColor` _pexponensialheightfogcomponent_2 (`KismetMathLibrary.LinearColorLerp` (`self.Initial_DirectionalInscatteringColor`) (`self.DirectionalInscatteringColor`) __))
      (`ExponentialHeightFogComponent.SetVolumetricFogAlbedo` _pexponensialheightfogcomponent_2 (`KismetMathLibrary.Conv_LinearColorToColor` (`KismetMathLibrary.LinearColorLerp` (`KismetMathLibrary.Conv_ColorToLinearColor` (`self.Initial_Albedo`)) (`KismetMathLibrary.Conv_ColorToLinearColor` (`self.Albedo`)) __)))
      (`ExponentialHeightFogComponent.SetVolumetricFogEmissive` _pexponensialheightfogcomponent_2 (`KismetMathLibrary.LinearColorLerp` (`self.Initial_Emissive`) (`self.Emissive`) __)))))

(event `ManualFogModifier`
  (`/Game/Pump/Core/BP_FunctionLibrary.LogErer` "qfzqzfqz")
  (goto _label))

(fn `INIT`
  (bind _outactors (`GameplayStatics.GetAllActorsOfClass` "/Script/Engine.ExponentialHeightFog"))
  (bind _output (`|GetArrayItem` _outactors))
  (`/Game/Pump/Core/BP_FunctionLibrary.LogErer` (`KismetSystemLibrary.GetDisplayName` _output))
  (bind _component (`ExponentialHeightFog.Component` _output))
  (set `self.pExponensialHeightFogComponent` _component)
  (set `self.InitialFogDensity` (`ExponentialHeightFogComponent.FogDensity` _component))
  (set `self.InitialFogExtinction` (`ExponentialHeightFogComponent.VolumetricFogExtinctionScale` _component))
  (set `self.Initial_FogInscatteringColor` (`ExponentialHeightFogComponent.FogInscatteringColor` _component))
  (set `self.Initial_DirectionalInscatteringColor` (`ExponentialHeightFogComponent.DirectionalInscatteringColor` _component))
  (set `self.Initial_Albedo` (`ExponentialHeightFogComponent.VolumetricFogAlbedo` _component))
  (set `self.Initial_Emissive` (`ExponentialHeightFogComponent.VolumetricFogEmissive` _component)))

(fn `UserConstructionScript`)