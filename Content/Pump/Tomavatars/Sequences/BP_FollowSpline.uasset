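; BP_FollowSpline is a cine camera actor that follows the moving pulse of a BP_RedLineSpline from above.
; On BeginPlay it caches the first red line spline in the level and tells BP_LevelManager to change the fog.
; Each tick it moves to a fixed height above PulseLocation and aligns the camera to the nearest spline rotation, with pitch tilted downward.
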(event `self.ReceiveBeginPlay`
  (bind _outactors (`GameplayStatics.GetAllActorsOfClass` "/Game/Pump/LD/RedLine/BP_RedLineSpline.BP_RedLineSpline_C"))
  (set `self.NewVar_0` (`|GetArrayItem` _outactors))
  (bind _outactors_2 (`GameplayStatics.GetAllActorsOfClass` "/Game/Pump/Core/BP_LevelManager.BP_LevelManager_C"))
  (`/Game/Pump/Core/BP_LevelManager.ChangeFog` (`|GetArrayItem` _outactors_2) 2))

(event `self.ReceiveTick`
  (params (DeltaSeconds :type "Float (single-precision)"))
  (bind _newvar_0 (`self.NewVar_0`))
  (bind (_pulselocation_x _pulselocation_y _pulselocation_z) (`KismetMathLibrary.BreakVector` (`/Game/Pump/LD/RedLine/BP_RedLineSpline.PulseLocation` _newvar_0)))
  (bind _spline (`/Game/Pump/LD/RedLine/BP_RedLineSpline.Spline` _newvar_0))
  (`self.K2_SetActorLocation` (`KismetMathLibrary.MakeVector` (+ _pulselocation_x 0.0) _pulselocation_y (+ _pulselocation_z 1000.0)))
  (bind _distance (`/Game/Pump/Core/BP_FunctionLibrary.Find Distance Along Spline Closest to World Location` _spline (`/Game/Pump/LD/RedLine/BP_RedLineSpline.PulseLocation` _newvar_0)))
  (bind (_returnvalue_roll _returnvalue_pitch _returnvalue_yaw) (`KismetMathLibrary.BreakRotator` (`SplineComponent.GetRotationAtDistanceAlongSpline` _spline _distance "World")))
  (`SceneComponent.K2_SetWorldRotation` (`self.CineCamera`) (`KismetMathLibrary.MakeRotator` _returnvalue_roll (- _returnvalue_pitch 20.0) _returnvalue_yaw) false false))

(fn `UserConstructionScript`)