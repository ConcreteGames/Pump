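; Manager that highlights the next gravity platform the player should reach by driving its emissive material.
; On a first-step trigger, it fades out the current platform, then stores and pulses the supplied next one through curve-sampled timelines on material parameters.
; It ignores bonus platforms, detected as unexpected landings with no next platform, and handles first and last platforms.
; It also caches all platforms, which GetNextPF searches for the current one.
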(event `InventoryAllPF`
  (bind _outactors (`GameplayStatics.GetAllActorsOfClass` "/Game/Pump/LD/GravityPlateform/Plane/BP_GravityPlateform_Plane.BP_GravityPlateform_Plane_C"))
  (set `self.AllPF` _outactors))

(event `FirstStepTrigger`
  (params (NextPF :type "/Game/Pump/LD/GravityPlateform/Plane/BP_GravityPlateform_Plane Object Reference") (PF_FirstLanded :type "/Game/Pump/LD/GravityPlateform/Plane/BP_GravityPlateform_Plane Object Reference"))
  (bind _t_osc (`self.T_osc`))
  (bind _timeline_0 (`self.Timeline_0`))
  (bind _midlod0 (`/Game/Pump/LD/GravityPlateform/Plane/BP_GravityPlateform_Plane.MIDLOD0` (`self.CurrentPF`)))
  ;[1 1 1] test si c'est une PF bonus, si c'est le cas on ne fait rien
  (if (not (and (!= PF_FirstLanded (`self.CurrentPF`)) (not (`KismetSystemLibrary.IsValid` NextPF))))
    ;[1 1 1] secu pour la première du jeu
    (`/Engine/EditorBlueprintResources/StandardMacros.IsValid` (`self.CurrentPF`)
      (:`Is Valid`
        (`|ExecutionSequence`
          (:`then_0`
            ;[1 1 1] fade out la précédente
            (set `self.CurrentPFMat` (`/Game/Pump/LD/GravityPlateform/Plane/BP_GravityPlateform_Plane.MIDLOD0` (`self.CurrentPF`)))
            (`TimelineComponent.SetTimelineLength` _timeline_0 0.2)
            (`Timeline|Timeline_0` :!via `PlayFromStart`
              (:`Update`
                (`MaterialInstanceDynamic.SetScalarParameterValue` (`self.CurrentPFMat`) "NextPlateformFactor" (- 1.0 (`CurveFloat.GetFloatValue` (`self.CRV_NextPFEmissiveOsc`) (`/Game/Pump/Core/BP_FunctionLibrary.GetTimelinePercentage` _timeline_0)))))))
          (:`then_1`
            ;[1 1 1] sécu pour la dernière du niveau
            (`/Engine/EditorBlueprintResources/StandardMacros.IsValid` NextPF :!label _label
              (:`Is Valid`
                (set `self.CurrentPF` NextPF)
                (`MaterialInstanceDynamic.SetScalarParameterValue` _midlod0 "MaxNextPlatformEmissive" 1.0)
                (`MaterialInstanceDynamic.SetScalarParameterValue` _midlod0 "MinNextPlatformEmissive" 0.5)
                (`TimelineComponent.SetTimelineLength` _t_osc 1.5)
                (`Timeline|T_osc` :!via `PlayFromStart`
                  (:`Update`
                    (`MaterialInstanceDynamic.SetScalarParameterValue` _midlod0 "NextPlateformFactor" (`CurveFloat.GetFloatValue` (`self.CRV_NextPFEmissiveOsc`) (`/Game/Pump/Core/BP_FunctionLibrary.GetTimelinePercentage` _t_osc))))))))))
      (:`Is Not Valid`
        (goto _label)))))

(fn `UserConstructionScript`)