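; Player controller that routes gameplay and menu input, and hosts developer debug hotkeys.
; AnyKey events match keys against three concatenated binding arrays from the save, using modulo to resolve actions for the character or menu.
; The main menu near-freezes time dilation and supports rebinding, filtered by gamepad or non-gamepad key.
; Holding C through a timeline unlocks DevMode; debug keys cover time, profiling, resolution, level visibility, saves and saturation tests.
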(event `Key|Divide`
  (params (Key :type "Key Structure")))

(event `Key|Multiply`
  (params (Key :type "Key Structure")))

(event `TEST`
  (bind _output_get (set `self.TODELETE_SatuXYZ` (* 1.0 10000000000.0 10000000.0) :!label _label))
  (set `self.TODELETE_WantTooBreakSaturation` 4))

(event `Key|Enter`
  (params (Key :type "Key Structure"))
  (:`Pressed`
    (`/Game/Pump/Core/Character/BP_ActorMacroLibrary.TestDevMode`
      (:`true`
        (goto _label)))))

(event `Key|X`
  (params (Key :type "Key Structure"))
  ;[1 1 1] DEBUG time dilation
  (:`Pressed`
    (`/Game/Pump/Core/Character/BP_ActorMacroLibrary.TestDevMode`
      (:`true`
        (`GameplayStatics.SetGlobalTimeDilation` 0.1)))))

(event `Key|Add`
  (params (Key :type "Key Structure"))
  (bind _colorsaturation_x (`KismetMathLibrary.BreakVector4` (break `PostProcessSettings` (`PostProcessComponent.Settings` (`/Game/Pump/Core/Character/BP_GravityCharacter_Pump.PostProcess` (`/Game/Pump/Core/BP_FunctionLibrary.GetCharMatter`))))))
  (:`Pressed`
    (`/Game/Pump/Core/Character/BP_ActorMacroLibrary.TestDevMode`
      (:`true`
        (`|ExecutionSequence`
          (:`then_0`
            (set `self.TODELETE_SatuXYZ` _colorsaturation_x))
          (:`then_1`
            (`/Game/Pump/Core/Character/BP_ActorMacroLibrary.GateTickWithDelaySeconds` 0.001 :!label _label_2
              (:`Tick`
                (set `self.TODELETE_SatuXYZ` (* (`self.TODELETE_SatuXYZ`) 1.1))
                (`self.TEST_ApplySatu` :!label _label_3)
                (`self.TEST_LogCurrentSatu`))))))))
  (:`Released`
    (`/Game/Pump/Core/Character/BP_ActorMacroLibrary.TestDevMode`
      (:`true`
        (goto _label_2 :!via `Close`)))))

(event `Key|C`
  (params (Key :type "Key Structure"))
  ;[1 1 1] DEBUG time dilation
  (:`Pressed`
    (`|ExecutionSequence`
      (:`then_0`
        (`Timeline|T_SecretConcreteMode` :!via `PlayFromStart` :!label _label_4
          (:`Finished`
            (set `/Game/Pump/Core/BP_GameInstance.DevMode` true (`/Game/Pump/Core/BP_FunctionLibrary.GetGI`))
            (`GameplayStatics.PlaySound2D` "/Game/Movies/ConcreteIntro_audio.ConcreteIntro_audio" 1.0 1.0 0.0 null null))))
      (:`then_1`
        (`/Game/Pump/Core/Character/BP_ActorMacroLibrary.TestDevMode`
          (:`true`
            (`GameplayStatics.SetGlobalTimeDilation` 1.0))))))
  (:`Released`
    (goto _label_4 :!via `Stop`)))

(event `Key|V`
  (params (Key :type "Key Structure"))
  ;[1 1 1] DEBUG time dilation
  (:`Pressed`
    (`/Game/Pump/Core/Character/BP_ActorMacroLibrary.TestDevMode`
      (:`true`
        (`GameplayStatics.SetGlobalTimeDilation` 1.2)))))

(event `Key|Subtract`
  (params (Key :type "Key Structure"))
  (:`Pressed`
    (`/Game/Pump/Core/Character/BP_ActorMacroLibrary.TestDevMode`
      (:`true`
        (`|ExecutionSequence`
          (:`then_0`
            (set `self.TODELETE_SatuXYZ` (* (`self.TODELETE_SatuXYZ`) -1.0)))))))
  (:`Released`
    (`/Game/Pump/Core/Character/BP_ActorMacroLibrary.TestDevMode`
      (:`true`
        (`/Game/Pump/Core/Character/BP_ActorMacroLibrary.GateTickWithDelaySeconds` 0.001 :!via `Close`
          (:`Tick`
            (set `self.TODELETE_SatuXYZ` (* (`self.TODELETE_SatuXYZ`) 1.1))
            (goto _label_3)))))))

(event `Key|B`
  (params (Key :type "Key Structure"))
  ;[1 1 1] DEBUG time dilation
  (:`Pressed`
    (`/Game/Pump/Core/Character/BP_ActorMacroLibrary.TestDevMode`
      (:`true`
        (`GameplayStatics.SetGlobalTimeDilation` 5.0)))))

(event `Key|H`
  (params (Key :type "Key Structure"))
  ;[1 1 1] Screenshot command
  (:`Pressed`
    (`/Game/Pump/Core/Character/BP_ActorMacroLibrary.TestDevMode`
      (:`true`
        (`/Game/Pump/Core/BP_FunctionLibrary.ExecuteConsolCommandWithLog` "HighResShot 1920x1080")))))

(event `Key|Decimal`
  (params (Key :type "Key Structure")))

(event `Key|F`
  (params (Key :type "Key Structure"))
  ;[1 1 1] stats commands
  (:`Pressed`
    (`/Game/Pump/Core/Character/BP_ActorMacroLibrary.TestDevMode`
      (:`true`
        (`/Game/Pump/Core/BP_FunctionLibrary.ExecuteConsolCommandWithLog` "Stat FPS")))))

(event `Key|NumPadOne`
  (params (Key :type "Key Structure"))
  (:`Pressed`
    (`/Game/Pump/Core/Character/BP_ActorMacroLibrary.TestDevMode`
      (:`true`
        (`self.ShowHideALevel` "Chapter_1_Mineral")))))

(event `Key|G`
  (params (Key :type "Key Structure"))
  ;[1 1 1] stats commands
  (:`Pressed`
    (`/Game/Pump/Core/Character/BP_ActorMacroLibrary.TestDevMode`
      (:`true`
        (`/Game/Pump/Core/BP_FunctionLibrary.ExecuteConsolCommandWithLog` "Stat UnitGraph")))))

(event `Key|R`
  (params (Key :type "Key Structure"))
  ;[1 1 1] stats commands
  (:`Pressed`
    (`/Game/Pump/Core/Character/BP_ActorMacroLibrary.TestDevMode`
      (:`true`
        (`/Game/Pump/Core/BP_FunctionLibrary.ExecuteConsolCommandWithLog` "Stat Unit")))))

(event `Key|NumPadTwo`
  (params (Key :type "Key Structure"))
  (:`Pressed`
    (`/Game/Pump/Core/Character/BP_ActorMacroLibrary.TestDevMode`
      (:`true`
        (`self.ShowHideALevel` "Chapter_1_Mineral_Decor")))))

(event `Key|Y`
  (params (Key :type "Key Structure"))
  ;[1 1 1] stats commands
  (:`Pressed`
    (`/Game/Pump/Core/Character/BP_ActorMacroLibrary.TestDevMode`
      (:`true`
        (`/Game/Pump/Core/BP_FunctionLibrary.ExecuteConsolCommandWithLog` "stat SceneRendering")))))

(event `Key|NumPadThree`
  (params (Key :type "Key Structure"))
  (:`Pressed`
    (`/Game/Pump/Core/Character/BP_ActorMacroLibrary.TestDevMode`
      (:`true`
        (`self.ShowHideALevel` "Chapter_1_Mineral_PlanetStep")))))

(event `Key|U`
  (params (Key :type "Key Structure"))
  ;[1 1 1] stats commands
  (:`Pressed`
    (`/Game/Pump/Core/Character/BP_ActorMacroLibrary.TestDevMode`
      (:`true`
        (`/Game/Pump/Core/BP_FunctionLibrary.ExecuteConsolCommandWithLog` "stat Game")))))

(event `Key|NumPadFour`
  (params (Key :type "Key Structure"))
  (:`Pressed`
    (`/Game/Pump/Core/Character/BP_ActorMacroLibrary.TestDevMode`
      (:`true`
        (`self.ShowHideALevel` "Chapter_2_Vegetal")))))

(event `Key|I`
  (params (Key :type "Key Structure"))
  ;[1 1 1] stats commands
  (:`Pressed`
    (`/Game/Pump/Core/Character/BP_ActorMacroLibrary.TestDevMode`
      (:`true`
        (`/Game/Pump/Core/BP_FunctionLibrary.ExecuteConsolCommandWithLog` "ProfileGPU")))))

(event `Key|NumPadFive`
  (params (Key :type "Key Structure"))
  (:`Pressed`
    (`/Game/Pump/Core/Character/BP_ActorMacroLibrary.TestDevMode`
      (:`true`
        (`self.ShowHideALevel` "Chapter_2_Vegetal_Decor")))))

(event `Key|O`
  (params (Key :type "Key Structure"))
  ;[1 1 1] stats commands
  (:`Pressed`
    (`/Game/Pump/Core/Character/BP_ActorMacroLibrary.TestDevMode`
      (:`true`
        (`/Game/Pump/Core/BP_FunctionLibrary.ExecuteConsolCommandWithLog` "stat GPU")))))

(event `Key|P`
  (params (Key :type "Key Structure"))
  ;[1 1 1] stats commands
  (:`Pressed`
    (`/Game/Pump/Core/Character/BP_ActorMacroLibrary.TestDevMode`
      (:`true`
        (`/Game/Pump/Core/BP_FunctionLibrary.ExecuteConsolCommandWithLog` "stat streaming")))))

(event `Key|NumPadSix`
  (params (Key :type "Key Structure"))
  (:`Pressed`
    (`/Game/Pump/Core/Character/BP_ActorMacroLibrary.TestDevMode`
      (:`true`
        (`self.ShowHideALevel` "Chapter_2_Vegetal_PlanetStep")))))

(event `Key|NumPadSeven`
  (params (Key :type "Key Structure"))
  (:`Pressed`
    (`/Game/Pump/Core/Character/BP_ActorMacroLibrary.TestDevMode`
      (:`true`
        (`self.ShowHideALevel` "Chapter_3_Animal")))))

(event `Key|J`
  (params (Key :type "Key Structure"))
  ;[1 1 1] screen percentage commands
  (:`Pressed`
    (`/Game/Pump/Core/Character/BP_ActorMacroLibrary.TestDevMode`
      (:`true`
        (`/Game/Pump/Core/BP_FunctionLibrary.ExecuteConsolCommandWithLog` "r.ScreenPercentage 5")))))

(event `Key|K`
  (params (Key :type "Key Structure"))
  ;[1 1 1] screen percentage commands
  (:`Pressed`
    (`/Game/Pump/Core/Character/BP_ActorMacroLibrary.TestDevMode`
      (:`true`
        (`/Game/Pump/Core/BP_FunctionLibrary.ExecuteConsolCommandWithLog` "r.ScreenPercentage 25")))))

(event `Key|NumPadEight`
  (params (Key :type "Key Structure"))
  (:`Pressed`
    (`/Game/Pump/Core/Character/BP_ActorMacroLibrary.TestDevMode`
      (:`true`
        (`self.ShowHideALevel` "Chapter_3_Animal_Decor")))))

(event `Key|L`
  (params (Key :type "Key Structure"))
  ;[1 1 1] screen percentage commands
  (:`Pressed`
    (`/Game/Pump/Core/Character/BP_ActorMacroLibrary.TestDevMode`
      (:`true`
        (`/Game/Pump/Core/BP_FunctionLibrary.ExecuteConsolCommandWithLog` "r.ScreenPercentage 100")))))

(event `Key|NumPadNine`
  (params (Key :type "Key Structure"))
  (:`Pressed`
    (`/Game/Pump/Core/Character/BP_ActorMacroLibrary.TestDevMode`
      (:`true`
        (`self.ShowHideALevel` "Chapter_3_Animal_PlanetStep")))))

(event `Key|M`
  (params (Key :type "Key Structure"))
  ;[1 1 1] screen percentage commands
  (:`Pressed`
    (`/Game/Pump/Core/Character/BP_ActorMacroLibrary.TestDevMode`
      (:`true`
        (`/Game/Pump/Core/BP_FunctionLibrary.ExecuteConsolCommandWithLog` "r.ScreenPercentage 200")))))

(event `Key|Insert`
  (params (Key :type "Key Structure"))
  ;[1 1 1] profiling commands
  (:`Pressed`
    (`/Game/Pump/Core/Character/BP_ActorMacroLibrary.TestDevMode`
      (:`true`
        (`/Game/Pump/Core/BP_FunctionLibrary.ExecuteConsolCommandWithLog` "stat startfile")))))

(event `Key|End`
  (params (Key :type "Key Structure"))
  ;[1 1 1] profiling commands
  (:`Pressed`
    (`/Game/Pump/Core/Character/BP_ActorMacroLibrary.TestDevMode`
      (:`true`
        (`/Game/Pump/Core/BP_FunctionLibrary.ExecuteConsolCommandWithLog` "stat stopfile")))))

(event `Key|R`
  (params (Key :type "Key Structure"))
  ;[1 1 1] DEBUG delete save
  (:`Pressed`
    (`/Game/Pump/Core/Character/BP_ActorMacroLibrary.TestDevMode`
      (:`true`
        (`/Game/Pump/Core/BP_FunctionLibrary.LogErer` "--> Request delete save")
        (bind _returnvalue (`GameplayStatics.DoesSaveGameExist` (`/Game/Pump/Core/BP_GameInstance.SaveGameName` (`/Game/Pump/Core/BP_FunctionLibrary.GetGI`))))
        (if _returnvalue
          (`/Game/Pump/Core/BP_FunctionLibrary.LogErer` "Save founded, name : " (`/Game/Pump/Core/BP_GameInstance.SaveGameName` (`/Game/Pump/Core/BP_FunctionLibrary.GetGI`)))
          (bind _returnvalue_2 (`GameplayStatics.DeleteGameInSlot` (`/Game/Pump/Core/BP_GameInstance.SaveGameName` (`/Game/Pump/Core/BP_FunctionLibrary.GetGI`))))
          (`/Game/Pump/Core/BP_FunctionLibrary.LogErerBool` "Save deleted" _returnvalue_2))))))

(event `Key|T`
  (params (Key :type "Key Structure"))
  ;[1 1 1] DEBUG get or create save
  (:`Pressed`
    (`/Game/Pump/Core/Character/BP_ActorMacroLibrary.TestDevMode`
      (:`true`
        (`/Game/Pump/Core/BP_FunctionLibrary.LogErer` "--> Get or Create Save")
        (`/Game/Pump/Core/BP_GameInstance.GetOrCreateSave` (`/Game/Pump/Core/BP_FunctionLibrary.GetGI`))
        (`/Game/Pump/Core/BP_FunctionLibrary.LogErerBool` "Save OK" true)))))

(event `ShowMainMenu`
  (`/Engine/EditorBlueprintResources/StandardMacros.IsValid` (`self.pMainMenu`)
    (:`Is Valid`
      _)
    (:`Is Not Valid`
      ;[1 1 1] create menu
      (bind _returnvalue (`|CreateWidget` "/Game/ConcreteTemplateNew/Menu/UI_MainMenu.UI_MainMenu_C"))
      (set `self.pMainMenu` _returnvalue)))
  (if (not (`Widget.IsInViewport` (`self.pMainMenu`)))
    (`UserWidget.AddToViewport` (`self.pMainMenu`) 0)
    (`WidgetBlueprintLibrary.SetInputMode_GameAndUIEx` (`GameplayStatics.GetPlayerController` 0) (`/Game/ConcreteTemplateNew/Menu/UI_MainMenu.B_Continue` (`self.pMainMenu`))) ; Pas UI only car sinon ça nique le keybinding\n(et en plus je ne peux plus utiliser "R" et "T"\npour respectivement "delete" et "check" la save :P)
    (set `self.bShowMouseCursor` true)
    (`GameplayStatics.SetGlobalTimeDilation` 1e-06)
    (set `self.IsInMenu` true)))

(event `Key|AnyKey`
  (params (Key :type "Key Structure"))
  (bind _character (`/Game/Pump/Core/BP_FunctionLibrary.GetCharMatter`))
  (bind _psavegame (`/Game/Pump/Core/BP_FunctionLibrary.GetSave`))
  (bind _character_2 (`/Game/Pump/Core/BP_FunctionLibrary.GetCharMatter`))
  (bind _pmainmenu (`self.pMainMenu`))
  (bind _pmainmenu_2 (`self.pMainMenu`))
  (bind _key (`self.Key`))
  (:`Pressed`
    (set `self.IsKeyPressed` true)
    (set `self.Key` Key :!label _label_5)
    (if (`/Game/Pump/Core/BP_GameInstance.BlockControls` (`/Game/Pump/Core/BP_FunctionLibrary.GetGI`))
      _
      (elif (`self.IsInMenu`)
        (if (`self.IsKeyPressed`)
          ;[1 1 1] is in Key Binding mode
          (if (`self.IsInKeyBindingMode`)
            (if (or (== _key "Escape") (== _key "Gamepad_Special_Right"))
              (`/Game/ConcreteTemplateNew/Menu/UI_MainMenu.NewBinding` _pmainmenu "Tilt")
              (`/Game/ConcreteTemplateNew/Menu/UI_MainMenu.ExitKeyBinding` _pmainmenu)
              (else
                ;[1 1 1] is a valid key
                (if (== (`KismetInputLibrary.Key_IsGamepadKey` (`self.Key`)) (`self.BindedKeyIsGamepad`))
                  (`|ExecutionSequence`
                    (:`then_0`)
                    (:`then_1`
                      (`KismetArrayLibrary.Array_Set` (select `int` (`self.BindedKeyColumn`) :`0` (`/Game/ConcreteTemplateNew/BP_SaveGame.Setting_Keys_K1` _psavegame) :`1` (`/Game/ConcreteTemplateNew/BP_SaveGame.Setting_Keys_K2` _psavegame) :`2` (`/Game/ConcreteTemplateNew/BP_SaveGame.Setting_Keys_P` _psavegame)) (`self.BindedKeyRaw`) (`self.Key`))
                      (`/Game/Pump/Core/BP_FunctionLibrary.Save`)
                      (`/Game/ConcreteTemplateNew/Menu/UI_MainMenu.NewBinding` _pmainmenu_2 (`self.Key`))
                      (`/Game/ConcreteTemplateNew/Menu/UI_MainMenu.ExitKeyBinding` _pmainmenu_2))))))
            (else
              (bind _action (`self.TestPressedReleasedKey`)
                (:`Pressed`
                  (switch `/Game/ConcreteTemplateNew/E_Actions` _action
                    (:`NewEnumerator8`
                      _)
                    (:`NewEnumerator9`
                      _))
                  (`/Game/ConcreteTemplateNew/Menu/UI_MainMenu.Key_Back` (`self.pMainMenu`)))))))
        (else
          ;[1 1 1] Is using pad Test
          (`self.IsUsingPadTest` (`self.Key`)) ; Pour le character\npour les axis de rotation de la cam\nNE FONCTIONNE QUE SI LE MENU N'EST PAS FOCUS\n(ouais c'est un peu naze, du coup dans le menu ce n'est pas utilisable)
          (bind _action_2 (`self.TestPressedReleasedKey`)
            (:`Pressed`
              (switch `/Game/ConcreteTemplateNew/E_Actions` _action_2
                (:`NewEnumerator0`
                  (`/Game/Pump/Core/Character/BP_GravityCharacter_Pump.Action_Forward_Pressed` _character_2))
                (:`NewEnumerator1`
                  (`/Game/Pump/Core/Character/BP_GravityCharacter_Pump.Action_Backward_Pressed` _character_2))
                (:`NewEnumerator2`
                  (`/Game/Pump/Core/Character/BP_GravityCharacter_Pump.Action_StrafeLeft_Pressed` _character_2))
                (:`NewEnumerator3`
                  (`/Game/Pump/Core/Character/BP_GravityCharacter_Pump.Action_StrafeRight_Pressed` _character_2))
                (:`NewEnumerator4`
                  (`/Game/Pump/Core/Character/BP_GravityCharacter_Pump.Action_Jump` _character_2))
                (:`NewEnumerator5`
                  (`/Game/Pump/Core/Character/BP_GravityCharacter_Pump.Action_Pump_Pressed` _character_2))
                (:`NewEnumerator6`
                  (`/Game/Pump/Core/Character/BP_GravityCharacter_Pump.Action_Reverse_Pressed` _character_2))
                (:`NewEnumerator9`
                  (`self.ShowMainMenu`))))
            (:`Released`
              (switch `/Game/ConcreteTemplateNew/E_Actions` _action_2
                (:`NewEnumerator0`
                  (`/Game/Pump/Core/Character/BP_GravityCharacter_Pump.Action_Forward_Released` _character))
                (:`NewEnumerator1`
                  (`/Game/Pump/Core/Character/BP_GravityCharacter_Pump.Action_Backward_Released` _character))
                (:`NewEnumerator2`
                  (`/Game/Pump/Core/Character/BP_GravityCharacter_Pump.Action_StrafeLeft_Released` _character))
                (:`NewEnumerator3`
                  (`/Game/Pump/Core/Character/BP_GravityCharacter_Pump.Action_StrafeRight_Released` _character))
                (:`NewEnumerator5`
                  (`/Game/Pump/Core/Character/BP_GravityCharacter_Pump.Action_Pump_Released` _character))
                (:`NewEnumerator6`
                  (`/Game/Pump/Core/Character/BP_GravityCharacter_Pump.Action_Reverse_Released` _character)))))))))
  (:`Released`
    (set `self.IsKeyPressed` false)
    (goto _label_5)))

(fn `GetAllCurrentKeyBinding`
  (bind _psavegame (`/Game/Pump/Core/BP_FunctionLibrary.GetSave`))
  (bind _dynamic_allkeybinding (`self.Dynamic_AllKeyBinding`))
  (`KismetArrayLibrary.Array_Clear` _dynamic_allkeybinding)
  (`KismetArrayLibrary.Array_Append` _dynamic_allkeybinding (`/Game/ConcreteTemplateNew/BP_SaveGame.Setting_Keys_K1` _psavegame))
  (`KismetArrayLibrary.Array_Append` _dynamic_allkeybinding (`/Game/ConcreteTemplateNew/BP_SaveGame.Setting_Keys_K2` _psavegame))
  (`KismetArrayLibrary.Array_Append` _dynamic_allkeybinding (`/Game/ConcreteTemplateNew/BP_SaveGame.Setting_Keys_P` _psavegame)))

(fn `IsUsingPadTest`
  (params (Key :type "Key Structure (by ref)"))
  (set `self.IsUsingPad` (`KismetInputLibrary.Key_IsGamepadKey` Key)))

(fn `ShowHideALevel`
  (params (levelName :type Name))
  (bind _returnvalue (`KismetStringLibrary.Conv_NameToString` levelName))
  (bind _returnvalue_2 (not (`LevelStreaming.bShouldBeVisible` (`GameplayStatics.GetStreamingLevel` levelName))))
  (bind _outactors (`GameplayStatics.GetAllActorsOfClass` "/Game/Pump/Core/BP_LevelManager.BP_LevelManager_C"))
  (`/Game/Pump/Core/BP_LevelManager.ShowHideALevel` (`|GetArrayItem` _outactors) levelName _returnvalue_2)
  (if _returnvalue_2
    (`/Game/Pump/Core/BP_FunctionLibrary.LogErer` "Show" _returnvalue)
    (else
      (`/Game/Pump/Core/BP_FunctionLibrary.LogErer` "Hide" _returnvalue))))

(fn `TEST_ApplySatu`
  (set `PostProcessComponent.Settings` (make `PostProcessSettings` :`ColorSaturation` (`KismetMathLibrary.MakeVector4` (`self.TODELETE_SatuXYZ`))) (`/Game/Pump/Core/Character/BP_GravityCharacter_Pump.PostProcess` (`/Game/Pump/Core/BP_FunctionLibrary.GetCharMatter`))))

(fn `TEST_ApplySatu_Random`
  (set `PostProcessComponent.Settings` (make `PostProcessSettings` :`ColorSaturation` (`KismetMathLibrary.MakeVector4` (* 1.0 10000000876544.0 100000000376832.0))) (`/Game/Pump/Core/Character/BP_GravityCharacter_Pump.PostProcess` (`/Game/Pump/Core/BP_FunctionLibrary.GetCharMatter`))))

(fn `TEST_LogCurrentSatu`
  (bind (_colorsaturation_x _colorsaturation_y _colorsaturation_z _colorsaturation_w) (`KismetMathLibrary.BreakVector4` (break `PostProcessSettings` (`PostProcessComponent.Settings` (`/Game/Pump/Core/Character/BP_GravityCharacter_Pump.PostProcess` (`/Game/Pump/Core/BP_FunctionLibrary.GetCharMatter`))))))
  (`/Game/Pump/Core/BP_FunctionLibrary.LogErer` (`KismetStringLibrary.Concat_StrStr` (`KismetStringLibrary.Conv_DoubleToString` _colorsaturation_x) " - " (`KismetStringLibrary.Conv_DoubleToString` _colorsaturation_y)) (`KismetStringLibrary.Concat_StrStr` (`KismetStringLibrary.Conv_DoubleToString` _colorsaturation_z) " - " (`KismetStringLibrary.Conv_DoubleToString` _colorsaturation_w))))

(fn `UserConstructionScript`)