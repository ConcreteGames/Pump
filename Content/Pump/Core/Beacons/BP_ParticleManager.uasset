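; BP_ParticleManager is a manager actor that spawns Niagara effects on request through its SetParticleEvent.
; At BeginPlay it caches the player pawn cast to BP_GravityCharacter_Pump.
; SetParticleEvent stores the given system and transform, then spawns and activates it at either the player's current location and rotation or the supplied ones, chosen by a boolean.
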(event `self.ReceiveBeginPlay`
  (bind _asbp_gravity_character_pump (cast `/Game/Pump/Core/Character/BP_GravityCharacter_Pump` (`GameplayStatics.GetPlayerPawn` 0)))
  (set `self.PPlayerCharacter` _asbp_gravity_character_pump))

(event `/Game/Pump/Core/Beacons/BI_Events.SetParticleEvent`
  (params (VFXNiagaraSystem :type "NiagaraSystem Object Reference") (SpawnParticles :type Boolean) (IsCharacterLocation :type Boolean) (LocationIfNotCharacter :type "Vector Structure") (RotationIfNotCharacter :type "Rotator Structure"))
  (bind _ischaracterlocation (`self.IsCharacterLocation`))
  (bind _pplayercharacter (`self.PPlayerCharacter`))
  (set `self.VFX_ParticleSystem` VFXNiagaraSystem)
  (set `self.IsCharacterLocation` IsCharacterLocation)
  (bind _output_get (set `self.ParticleLocation` LocationIfNotCharacter))
  (bind _output_get_2 (set `self.ParticleRotation` RotationIfNotCharacter))
  (bind _returnvalue (`NiagaraFunctionLibrary.SpawnSystemAtLocation` (`self.VFX_ParticleSystem`) (select `bool` _ischaracterlocation :`false` _output_get :`true` (`self.K2_GetActorLocation` _pplayercharacter)) (select `bool` _ischaracterlocation :`false` _output_get_2 :`true` (`self.K2_GetActorRotation` _pplayercharacter))))
  (`ActorComponent.Activate` _returnvalue false))

(fn `UserConstructionScript`)