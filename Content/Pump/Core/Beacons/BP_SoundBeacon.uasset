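; BP_SoundBeacon is a level-placed trigger that changes the game's FMOD music or music effects when the player reaches it.
; On BeginPlay it caches the first Bp_SoundSystem, then the player pawn's first overlap fires the special event once and deactivates the Trigger.
; ESoundTriggers selects either TriggerMusicPart or an FXParameterChange with envelope settings on that system.
; An alternative timer-polled distance check exists, but its timer setup is never run.
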(event `self.ReceiveBeginPlay`
  ;[0 0.793 1] Init
  (bind _outactors (`GameplayStatics.GetAllActorsOfClass` "/Game/Pump/Core/SoundSystem/Bp_SoundSystem.Bp_SoundSystem_C"))
  (set `self.PSoundSystem` (`|GetArrayItem` _outactors)))

(event `TriggerSpecialEvent`
  ;[0.9505 1 0.000142] Trig Special Sound Event
  (switch `/Game/Pump/Core/SoundSystem/ESoundTriggers` (`self.ESoundTriggers`)
    (:`NewEnumerator0`
      (`self.FxChangeOutput`))
    (:`NewEnumerator1`
      (`self.TriggerMusicPart` (`self.PSoundSystem`) (`self.IsEventChange`) (`self.FmodEventToPlay`) (`self.MusicStepParameter`)))))

(event `self.Trigger.OnComponentBeginOverlap`
  (params (OverlappedComponent :type "PrimitiveComponent Object Reference") (OtherActor :type "Actor Object Reference") (OtherComp :type "PrimitiveComponent Object Reference") (OtherBodyIndex :type Integer) (bFromSweep :type Boolean) (SweepResult :type "HitResult Structure (by ref)"))
  ;[1 1 1] Trigger Overlap
  (if (== OtherActor (cast `/Game/Pump/Core/Character/BP_GravityCharacter_Pump` (`GameplayStatics.GetPlayerPawn` 0) :!pure true))
    (`/Engine/EditorBlueprintResources/StandardMacros.DoOnce` false
      (:`Completed`
        (`self.TriggerSpecialEvent`)
        (`ActorComponent.Deactivate` (`self.Trigger`))))))

(fn `FxChangeOutput`
  (bind _parameternames (`self.ParameterNames`))
  (`self.FXParameterChange` (`self.PSoundSystem`) (make `/Game/Pump/Core/SoundSystem/STR_MusicFx` _parameternames (`self.EnveloppeMinValue`) (`self.EnveloppeXValue`) (`self.MusicFxInitParameterValue`)) (`KismetArrayLibrary.Array_LastIndex` _parameternames) (`self.MusicFxEnveloppeLength`) (`self.ManualParameterInitValue`)))

(fn `GetPlayerVectorLength`
  (bind _asbp_gravity_character_pump (cast `/Game/Pump/Core/Character/BP_GravityCharacter_Pump` (`GameplayStatics.GetPlayerPawn` 0)))
  (bind _output_get (set `self.VectorLength` (`KismetMathLibrary.VSize` (- (`self.K2_GetActorLocation`) (`self.K2_GetActorLocation` _asbp_gravity_character_pump)))))
  (if (<= _output_get (`self.VectorLengthTriggerValue`))
    (`self.TriggerSpecialEvent`)
    (`KismetSystemLibrary.K2_ClearAndInvalidateTimerHandle` (`self.Timer`))))

(fn `UserConstructionScript`)