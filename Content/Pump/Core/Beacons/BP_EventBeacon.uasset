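; BP_EventBeacon is a trigger beacon that fires configured sound and particle events once, when the player's BP_GravityCharacter_Pump first overlaps it.
; BeginPlay caches the player, the first Bp_SoundSystem and the first BP_ParticleManager.
; The Operations list sets which branches run: sound triggers drive FX parameter, music and event calls on the sound system, while particles pass a Niagara system and placement to the manager.
; The shader branch is an empty stub.
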(event `self.ReceiveBeginPlay`
  ;[0 1 0.06728] Begin Play
  (`self.MakeActorsRefs`))

(event `self.Trigger.OnComponentBeginOverlap`
  (params (OverlappedComponent :type "PrimitiveComponent Object Reference") (OtherActor :type "Actor Object Reference") (OtherComp :type "PrimitiveComponent Object Reference") (OtherBodyIndex :type Integer) (bFromSweep :type Boolean) (SweepResult :type "HitResult Structure (by ref)"))
  ;[1 0.9745 0] Overlap Trigger Box
  (if (== OtherActor (`self.PCharacter`))
    (`/Engine/EditorBlueprintResources/StandardMacros.DoOnce` false
      (:`Completed`
        (`self.SetEventsToPlay`)
        (`self.SoundOperations`)
        (`self.ParticleOperations`)
        (`self.ShaderOperations`)))))

(fn `MakeActorsRefs`
  (bind _asbp_gravity_character_pump (cast `/Game/Pump/Core/Character/BP_GravityCharacter_Pump` (`GameplayStatics.GetPlayerPawn` 0)))
  (set `self.PCharacter` _asbp_gravity_character_pump)
  (bind _outactors (`GameplayStatics.GetAllActorsOfClass` "/Game/Pump/Core/SoundSystem/Bp_SoundSystem.Bp_SoundSystem_C"))
  (set `self.PSoundSystem` (`|GetArrayItem` _outactors))
  (bind _outactors_2 (`GameplayStatics.GetAllActorsOfClass` "/Game/Pump/Core/Beacons/BP_ParticleManager.BP_ParticleManager_C"))
  (set `self.PParticleManager` (`|GetArrayItem` _outactors_2)))

(fn `ParticleOperations`
  (if (`self.IsParticleEvent`)
    (`self.SetParticleEvent` (`self.PParticleManager`) (`self.VFXNiagaraSystem`) false (`self.ParticleIsCharacterLocation`) (`self.ParticleLocation`) (`self.ParticleRotation`))))

(fn `SetEventsToPlay`
  (bind _operations (`self.Operations`))
  (set `self.IsSoundEvent` (`KismetArrayLibrary.Array_Contains` _operations "NewEnumerator0"))
  (set `self.IsParticleEvent` (`KismetArrayLibrary.Array_Contains` _operations "NewEnumerator1"))
  (set `self.IsShaderEvent` (`KismetArrayLibrary.Array_Contains` _operations "NewEnumerator2")))

(fn `SFxChange`
  (bind _parameternames (`self.ParameterNames`))
  (`/Game/Pump/Core/SoundSystem/BI_Sound.FXParameterChange` (`self.PSoundSystem`) (make `/Game/Pump/Core/SoundSystem/STR_MusicFx` _parameternames (`self.EnveloppeMinValue`) (`self.EnveloppeXValue`) (`self.MusicFxInitParameterValue`)) (`KismetArrayLibrary.Array_LastIndex` _parameternames) (`self.MusicFxEnveloppeLength`) (`self.ManualParameterInitValue`)))

(fn `ShaderOperations`
  (if (`self.IsShaderEvent`)
    _))

(fn `SoundOperations`
  (bind _psoundsystem (`self.PSoundSystem`))
  (if (`self.IsSoundEvent`)
    (for _array_element (`self.ESoundTriggers`)
      (switch `/Game/Pump/Core/SoundSystem/ESoundTriggers` _array_element
        (:`NewEnumerator0`
          (`self.SFxChange`))
        (:`NewEnumerator1`
          (`/Game/Pump/Core/SoundSystem/BI_Sound.TriggerMusicPart` (`self.PSoundSystem`) (`self.IsEventChange`) (`self.FmodEventToPlay`) (`self.MusicStepParameter`)))
        (:`NewEnumerator2`
          (`/Game/Pump/Core/SoundSystem/Bp_SoundSystem.MusicPlayPauseStop` _psoundsystem "NewEnumerator0" 0.0 "None"))
        (:`NewEnumerator3`
          (`/Game/Pump/Core/SoundSystem/Bp_SoundSystem.TriggerEvent` _psoundsystem null))))))

(fn `UserConstructionScript`)