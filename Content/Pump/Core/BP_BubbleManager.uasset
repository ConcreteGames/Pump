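; BP_BubbleManager is an actor that registers the level's bubbles, reveals them by level and tracks how many have been entered.
; On BeginPlay it gathers all BP_BubbleMaster actors, sets their manager and starting state, hides them, then shows level 0.
; DisplayLevel reveals bubbles tagged "LevelIndex" plus the number, and DisplayNextLevel advances that index without hiding earlier ones.
; First-time entries update an entered ratio over all bubbles, and AddBubble registers additional ones.
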(event `HideAllBubbles`
  (for _array_element (`self.AllBubbles`)
    (`/Game/Pump/LD/Bubble/BP_BubbleMaster.SetVisiblity` _array_element false)))

(event `self.ReceiveBeginPlay`
  (`self.RegisterBubbles`)
  (`self.HideAllBubbles`)
  (`self.DisplayLevel` 0))

(event `OnABubbleIsEnteredForFirstTIme`
  (params (Bubble :type "/Game/Pump/LD/Bubble/BP_BubbleMaster Object Reference"))
  (`self.UpdateBubbleEnteredCount`))

(event `DisplayLevel`
  (params (LevelIndex :type Integer))
  (for _array_element (`self.AllBubbles`)
    (if (`KismetArrayLibrary.Array_Contains` (`Actor.Tags` _array_element) (`KismetStringLibrary.Conv_StringToName` (`KismetStringLibrary.Concat_StrStr` "LevelIndex" (`KismetStringLibrary.Conv_IntToString` LevelIndex))))
      (`/Game/Pump/LD/Bubble/BP_BubbleMaster.SetVisiblity` _array_element true))))

(event `AddBubble`
  (params (Bubble :type "/Game/Pump/LD/Bubble/BP_BubbleMaster Object Reference"))
  (`/Game/Pump/LD/Bubble/BP_BubbleMaster.SetBubbleManager` Bubble self)
  (`/Game/Pump/LD/Bubble/BP_BubbleMaster.SetBubbleManager` Bubble self)
  (`/Game/Pump/LD/Bubble/BP_BubbleMaster.SetDefaultState` Bubble (`self.BubbleColorAtStart`))
  (`KismetArrayLibrary.Array_AddUnique` (`self.AllBubbles`) Bubble))

(event `DisplayNextLevel`
  (bind _result (`/Engine/EditorBlueprintResources/StandardMacros.IncrementInt` (`self.CurrentLevelIndex`))
    (:`  `
      (`self.DisplayLevel` _result))))

(fn `UpdateBubbleEnteredCount`
  (bind _result (`/Engine/EditorBlueprintResources/StandardMacros.IncrementInt` (`self.BubbleEnteredCount`))
    (:`  `
      (set `self.BubbleEnteredRatio` (/ (`KismetMathLibrary.Conv_IntToDouble` _result) (`KismetMathLibrary.Conv_IntToDouble` (`KismetArrayLibrary.Array_Length` (`self.AllBubbles`))))))))

(fn `UserConstructionScript`)