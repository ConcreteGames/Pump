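; Blueprint function library of shared helpers for debugging, game framework access and simple spatial checks.
; Three log functions print long-lasting screen messages in randomized colors, with green or red tints for booleans and a marked error variant.
; Getters return the cast game instance, game mode and player controller, alongside a timeline progress ratio.
; Spatial checks test whether a component projects inside player zero's viewport or two components lie within a distance.
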(fn `GetGI`
  (returns (GI :type "/Game/Pump/Core/BP_GameInstance Object Reference"))
  (bind _asbp_game_instance (cast `/Game/Pump/Core/BP_GameInstance` (`GameplayStatics.GetGameInstance` null)))
  (return _asbp_game_instance))

(fn `GetGM`
  (returns (GM :type "/Game/Pump/Core/BP_Gamemode Object Reference"))
  (bind _asbp_gamemode (cast `/Game/Pump/Core/BP_Gamemode` (`GameplayStatics.GetGameMode` null)))
  (return _asbp_gamemode))

(fn `GetPCont`
  (params (PlayerIndex :type Integer))
  (returns (PCont :type "/Game/Pump/Core/BP_PlayerController Object Reference"))
  (bind _asbp_player_controller (cast `/Game/Pump/Core/BP_PlayerController` (`GameplayStatics.GetPlayerController` null PlayerIndex)))
  (return _asbp_player_controller))

(fn `GetTimelinePercentage`
  (params (Timeline :type "TimelineComponent Object Reference"))
  (returns (`%` :type "Float (double-precision)"))
  (return (/ (`TimelineComponent.GetPlaybackPosition` Timeline) (`TimelineComponent.GetTimelineLength` Timeline))))

(fn `IsCloserThan`
  (params (`1stSceneComponent` :type "SceneComponent Object Reference") (`2ndSceneComponent` :type "SceneComponent Object Reference") (Distance :type "Float (double-precision)"))
  (returns (IsCloser :type Boolean))
  (return (< (`KismetMathLibrary.VSize` (- (`SceneComponent.K2_GetComponentLocation` `1stSceneComponent`) (`SceneComponent.K2_GetComponentLocation` `2ndSceneComponent`))) Distance)))

(fn `IsOnScreen`
  (params (SceneComponent :type "SceneComponent Object Reference"))
  (returns (IsOnScreen :type Boolean))
  (bind (_returnvalue_x _returnvalue_y) (`KismetMathLibrary.BreakVector2D` (`WidgetLayoutLibrary.GetViewportSize` null)))
  (bind _screenlocation (`PlayerController.ProjectWorldLocationToScreen` (`GameplayStatics.GetPlayerController` null) (`SceneComponent.K2_GetComponentLocation` SceneComponent) false))
  (return (and (> (`KismetMathLibrary.BreakVector2D` _screenlocation) 0.0) (> (`.Y` (`KismetMathLibrary.BreakVector2D` _screenlocation)) 0.0) (< (`KismetMathLibrary.BreakVector2D` _screenlocation) _returnvalue_x) (< (`.Y` (`KismetMathLibrary.BreakVector2D` _screenlocation)) _returnvalue_y))))

(fn `LogErer`
  (params (String :type String))
  (`KismetSystemLibrary.PrintString` null String true true (make `LinearColor` (`KismetMathLibrary.RandomFloatInRange` 0.25 1.0) (`KismetMathLibrary.RandomFloatInRange` 0.25 1.0) (`KismetMathLibrary.RandomFloatInRange` 0.25 1.0) 1.0) 9999.0))

(fn `LogErerBool`
  (params (String :type String) (Bool :type Boolean))
  (bind _returnvalue (`KismetMathLibrary.RandomFloatInRange` 0.0 0.8))
  (bind _returnvalue_2 (`KismetMathLibrary.RandomFloatInRange` 0.0 0.5))
  (`KismetSystemLibrary.PrintString` null (`KismetStringLibrary.Concat_StrStr` String " = " (select `bool` Bool :`false` "FALSE" :`true` "true")) true true (select `bool` Bool :`false` (make `LinearColor` 1.0 _returnvalue _returnvalue 1.0) :`true` (make `LinearColor` _returnvalue_2 1.0 _returnvalue_2 1.0)) 9999.0))

(fn `LogErerror`
  (params (String :type String))
  (bind _returnvalue (`KismetMathLibrary.RandomFloatInRange` 0.5 1.0))
  (`KismetSystemLibrary.PrintString` null (`KismetStringLibrary.Concat_StrStr` "/!\\  ERROR: " String "  /!\\") true true (make `LinearColor` _returnvalue (`KismetMathLibrary.RandomFloatInRange` 0.0 0.5) _returnvalue 1.0) 9999.0))