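; BP_Optimisation is a debug tool that changes rendering quality console variables at runtime from NumPad keys 0 to 8.
; Each key drives a looping MultiGate whose index selects a preset value.
; That value is appended to the command name without a separating space, executed as a console command and logged.
; Several hard-coded scalability and quality commands are left unconnected and never run.
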(event `Key|NumPadZero`
  (params (Key :type "Key Structure"))
  (:`Pressed`
    (`/Game/Pump/Core/BP_FunctionLibrary.LogErer` "qsdqsd")
    (`|MultiGate` false true
      (:`Out 0`
        (bind _value (`LowEntryExtendedStandardLibrary.ExecToInteger` :!label _label))
        (bind _returnvalue (`KismetStringLibrary.Concat_StrStr` "r.ScreenPercentage " (select `int` _value :`0` "5" :`1` "50" :`2` "100")))
        (`KismetSystemLibrary.ExecuteConsoleCommand` _returnvalue null)
        (`/Game/Pump/Core/BP_FunctionLibrary.LogErer` "CC" (`KismetStringLibrary.Concat_StrStr` _returnvalue " on " "100")))
      (:`Out 1`
        (goto _label :!via `_1_`))
      (:`Out 2`
        (goto _label :!via `_2_`)))))

(event `Key|NumPadOne`
  (params (Key :type "Key Structure"))
  (:`Pressed`
    (`|MultiGate` false true
      (:`Out 0`
        (bind _value (`LowEntryExtendedStandardLibrary.ExecToInteger` :!label _label_2))
        (bind _returnvalue (`KismetStringLibrary.Concat_StrStr` "r.ViewDistanceScale " (select `int` _value :`0` "0.1" :`1` "0.5" :`2` "1")))
        (`KismetSystemLibrary.ExecuteConsoleCommand` _returnvalue null)
        (`/Game/Pump/Core/BP_FunctionLibrary.LogErer` "CC" (`KismetStringLibrary.Concat_StrStr` _returnvalue " on " "1")))
      (:`Out 1`
        (goto _label_2 :!via `_1_`))
      (:`Out 2`
        (goto _label_2 :!via `_2_`)))))

(event `Key|NumPadTwo`
  (params (Key :type "Key Structure"))
  (:`Pressed`
    (`|MultiGate` false true
      (:`Out 0`
        (bind _value (`LowEntryExtendedStandardLibrary.ExecToInteger` :!label _label_3))
        (bind _returnvalue (`KismetStringLibrary.Concat_StrStr` "r.PostProcessAAQuality " (select `int` _value :`0` "0" :`1` "1" :`2` "2" :`3` "3" :`4` "4" :`5` "5" :`6` "6")))
        (`KismetSystemLibrary.ExecuteConsoleCommand` _returnvalue null)
        (`/Game/Pump/Core/BP_FunctionLibrary.LogErer` "CC" (`KismetStringLibrary.Concat_StrStr` _returnvalue " on " "6")))
      (:`Out 1`
        (goto _label_3 :!via `_1_`))
      (:`Out 2`
        (goto _label_3 :!via `_2_`))
      (:`Out 3`
        (goto _label_3 :!via `_3_`))
      (:`Out 4`
        (goto _label_3 :!via `_4_`))
      (:`Out 5`
        (goto _label_3 :!via `_5_`))
      (:`Out 6`
        (goto _label_3 :!via `_6_`)))))

(event `Key|NumPadThree`
  (params (Key :type "Key Structure"))
  (:`Pressed`
    (`|MultiGate` false true
      (:`Out 0`
        (bind _value (`LowEntryExtendedStandardLibrary.ExecToInteger` :!label _label_4))
        (bind _returnvalue (`KismetStringLibrary.Concat_StrStr` "sg.PostProcessQuality " (select `int` _value :`0` "0" :`1` "1" :`2` "2" :`3` "3")))
        (`KismetSystemLibrary.ExecuteConsoleCommand` _returnvalue null)
        (`/Game/Pump/Core/BP_FunctionLibrary.LogErer` "CC" (`KismetStringLibrary.Concat_StrStr` _returnvalue " on " "3")))
      (:`Out 1`
        (goto _label_4 :!via `_1_`))
      (:`Out 2`
        (goto _label_4 :!via `_2_`))
      (:`Out 3`
        (goto _label_4 :!via `_3_`)))))

(event `Key|NumPadFour`
  (params (Key :type "Key Structure"))
  (:`Pressed`
    (`|MultiGate` false true
      (:`Out 0`
        (bind _value (`LowEntryExtendedStandardLibrary.ExecToInteger` :!label _label_5))
        (bind _returnvalue (`KismetStringLibrary.Concat_StrStr` "sg.ShadowQuality " (select `int` _value :`0` "0" :`1` "1" :`2` "2" :`3` "3")))
        (`KismetSystemLibrary.ExecuteConsoleCommand` _returnvalue null)
        (`/Game/Pump/Core/BP_FunctionLibrary.LogErer` "CC" (`KismetStringLibrary.Concat_StrStr` _returnvalue " on " "3")))
      (:`Out 1`
        (goto _label_5 :!via `_1_`))
      (:`Out 2`
        (goto _label_5 :!via `_2_`))
      (:`Out 3`
        (goto _label_5 :!via `_3_`)))))

(event `Key|NumPadFive`
  (params (Key :type "Key Structure"))
  (:`Pressed`
    (`|MultiGate` false true
      (:`Out 0`
        (bind _value (`LowEntryExtendedStandardLibrary.ExecToInteger` :!label _label_6))
        (bind _returnvalue (`KismetStringLibrary.Concat_StrStr` "sg.TextureQuality " (select `int` _value :`0` "0" :`1` "1" :`2` "2" :`3` "3")))
        (`KismetSystemLibrary.ExecuteConsoleCommand` _returnvalue null)
        (`/Game/Pump/Core/BP_FunctionLibrary.LogErer` "CC" (`KismetStringLibrary.Concat_StrStr` _returnvalue " on " "3")))
      (:`Out 1`
        (goto _label_6 :!via `_1_`))
      (:`Out 2`
        (goto _label_6 :!via `_2_`))
      (:`Out 3`
        (goto _label_6 :!via `_3_`)))))

(event `Key|NumPadSix`
  (params (Key :type "Key Structure"))
  (:`Pressed`
    (`|MultiGate` false true
      (:`Out 0`
        (bind _value (`LowEntryExtendedStandardLibrary.ExecToInteger` :!label _label_7))
        (bind _returnvalue (`KismetStringLibrary.Concat_StrStr` "sg.EffectsQuality " (select `int` _value :`0` "0" :`1` "1" :`2` "2" :`3` "3")))
        (`KismetSystemLibrary.ExecuteConsoleCommand` _returnvalue null)
        (`/Game/Pump/Core/BP_FunctionLibrary.LogErer` "CC" (`KismetStringLibrary.Concat_StrStr` _returnvalue " on " "3")))
      (:`Out 1`
        (goto _label_7 :!via `_1_`))
      (:`Out 2`
        (goto _label_7 :!via `_2_`))
      (:`Out 3`
        (goto _label_7 :!via `_3_`)))))

(event `Key|NumPadSeven`
  (params (Key :type "Key Structure"))
  (:`Pressed`
    (`|MultiGate` false true
      (:`Out 0`
        (bind _value (`LowEntryExtendedStandardLibrary.ExecToInteger` :!label _label_8))
        (bind _returnvalue (`KismetStringLibrary.Concat_StrStr` "r.DetailMode " (select `int` _value :`0` "0" :`1` "1" :`2` "2")))
        (`KismetSystemLibrary.ExecuteConsoleCommand` _returnvalue null)
        (`/Game/Pump/Core/BP_FunctionLibrary.LogErer` "CC" (`KismetStringLibrary.Concat_StrStr` _returnvalue " on " "2")))
      (:`Out 1`
        (goto _label_8 :!via `_1_`))
      (:`Out 2`
        (goto _label_8 :!via `_2_`)))))

(event `Key|NumPadEight`
  (params (Key :type "Key Structure"))
  (:`Pressed`
    (`|MultiGate` false true
      (:`Out 0`
        (bind _value (`LowEntryExtendedStandardLibrary.ExecToInteger` :!label _label_9))
        (bind _returnvalue (`KismetStringLibrary.Concat_StrStr` "FoliageQuality " (select `int` _value :`0` "0" :`1` "1" :`2` "2" :`3` "3")))
        (`KismetSystemLibrary.ExecuteConsoleCommand` _returnvalue null)
        (`/Game/Pump/Core/BP_FunctionLibrary.LogErer` "CC" (`KismetStringLibrary.Concat_StrStr` _returnvalue " on " "3")))
      (:`Out 1`
        (goto _label_9 :!via `_1_`))
      (:`Out 2`
        (goto _label_9 :!via `_2_`))
      (:`Out 3`
        (goto _label_9 :!via `_3_`)))))

(fn `UserConstructionScript`)