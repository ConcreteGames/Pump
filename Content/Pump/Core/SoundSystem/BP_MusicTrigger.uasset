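; Music trigger actor that drives the sound system's music from the player's progress along a spline.
; On BeginPlay it caches the gravity character pawn, the first Bp_SoundSystem in the level and the spline length, then starts a looping timer.
; Several times a second, the timer maps the player's closest distance along the spline to a normalized, clamped parameter and passes it to TriggerSplineMusic, with no overlap logic.
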(event `self.ReceiveBeginPlay`
  (bind _asbp_gravity_character_pump (cast `/Game/Pump/Core/Character/BP_GravityCharacter_Pump` (`GameplayStatics.GetPlayerPawn` 0)))
  (set `self.PlayerPawn` _asbp_gravity_character_pump)
  (bind _outactors (`GameplayStatics.GetAllActorsOfClass` "/Game/Pump/Core/SoundSystem/Bp_SoundSystem.Bp_SoundSystem_C"))
  (set `self.PSoundSystem` (`|GetArrayItem` _outactors))
  (set `self.SplineLength` (`SplineComponent.GetSplineLength` (`self.Spline`)))
  (bind _returnvalue (`KismetSystemLibrary.K2_SetTimer` null "MakeSplineMusicParameter" 0.2 true))
  (set `self.Timer` _returnvalue))

(fn `MakeSplineMusicParameter`
  (bind _distance (`/Game/Pump/Core/BP_FunctionLibrary.Find Distance Along Spline Closest to World Location` (`self.Spline`) (`self.K2_GetActorLocation` (`self.PlayerPawn`))))
  (bind _output_get (set `self.SplineParameter` (`KismetMathLibrary.MapRangeClamped` _distance 0.0 (`self.SplineLength`) 0.0 1.0)))
  (`self.TriggerSplineMusic` (`self.PSoundSystem`) _output_get))

(fn `UserConstructionScript`)