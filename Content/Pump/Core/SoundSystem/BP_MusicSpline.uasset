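; Spline actor that drives music through Bp_SoundSystem according to the player's position along its path.
; On a half-second looping timer, it maps the gravity character's closest point on the spline to a normalized parameter for TriggerSplineMusic.
; A work-in-progress check compares that point's local Y and Z to a limit to switch the music's play/pause state.
; The construction script aligns and scales an Arrow from the spline's endpoints.
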(event `self.ReceiveBeginPlay`
  (bind _asbp_gravity_character_pump (cast `/Game/Pump/Core/Character/BP_GravityCharacter_Pump` (`GameplayStatics.GetPlayerPawn` 0)))
  (set `self.PlayerPawn` _asbp_gravity_character_pump)
  (bind _outactors (`GameplayStatics.GetAllActorsOfClass` "/Game/Pump/Core/SoundSystem/Bp_SoundSystem.Bp_SoundSystem_C"))
  (set `self.PSoundSystem` (`|GetArrayItem` _outactors))
  (set `self.SplineLength` (`SplineComponent.GetSplineLength` (`self.Spline`)))
  (bind _returnvalue (`KismetSystemLibrary.K2_SetTimer` null "MakeSplineMusicParameter" 0.5 true))
  (set `self.Timer` _returnvalue)
  (`SplineComponent.SetDrawDebug` (`self.Spline`) true))

(fn `FindDistanceAlongSplineClosestToWorldLocation`
  (params (Spline :type "SplineComponent Object Reference") (Location :type "Vector Structure"))
  (returns (`Return Value Y` :type "Float (double-precision)") (`Return Value Z` :type "Float (double-precision)"))
  (bind (_returnvalue_x _returnvalue_y _returnvalue_z) (`KismetMathLibrary.BreakVector` (`SplineComponent.FindLocationClosestToWorldLocation` Spline Location "Local")))
  (return _returnvalue_y _returnvalue_z))

(fn `MakeSplineMusicParameter`
  (bind _psoundsystem (`self.PSoundSystem`))
  (bind _maxdistanceyztospline (`self.MaxDistanceYZToSpline`))
  (bind _returnvalue (* _maxdistanceyztospline -1.0))
  (bind (_return_value_y _return_value_z) (`self.FindDistanceAlongSplineClosestToWorldLocation` (`self.Spline`) (`self.K2_GetActorLocation` (`self.PlayerPawn`))))
  (bind _distance (`/Game/Pump/Core/BP_FunctionLibrary.Find Distance Along Spline Closest to World Location` (`self.Spline`) (`self.K2_GetActorLocation` (`self.PlayerPawn`))))
  (bind _output_get (set `self.SplineParameter` (`KismetMathLibrary.MapRangeClamped` _distance 0.0 (`self.SplineLength`) 0.0 1.0)))
  (`self.TriggerSplineMusic` (`self.PSoundSystem`) _output_get (0.0 0.0 0.0))
  ;[1 0.6608 0.2826] WIP : Y and Z Distance to Spline Behavior (Actually Pause Music)
  (if (or (>= _return_value_y _maxdistanceyztospline) (<= _return_value_y _returnvalue) (>= _return_value_z _maxdistanceyztospline) (<= _return_value_z _returnvalue)) :!pinned true
    (`/Game/Pump/Core/SoundSystem/Bp_SoundSystem.MusicPlayPauseStop` _psoundsystem "NewEnumerator1" 0.0 "None")
    (else
      (`/Game/Pump/Core/SoundSystem/Bp_SoundSystem.MusicPlayPauseStop` _psoundsystem "NewEnumerator4" 0.0 "None"))))

(fn `UserConstructionScript`
  (bind _spline (`self.Spline`))
  (bind _arrow (`self.Arrow`))
  (bind _returnvalue (`SplineComponent.GetLocationAtSplinePoint` _spline 0 "Local"))
  (bind _returnvalue_2 (`SplineComponent.GetLocationAtSplinePoint` _spline (`SplineComponent.GetNumberOfSplinePoints` _spline) "Local"))
  (`SceneComponent.SetWorldScale3D` _arrow (`KismetMathLibrary.MakeVector` (`KismetMathLibrary.VSize` (- _returnvalue _returnvalue_2)) 1.0 1.0))
  (`SceneComponent.K2_SetWorldRotation` _arrow (`KismetMathLibrary.FindLookAtRotation` _returnvalue _returnvalue_2) false false))