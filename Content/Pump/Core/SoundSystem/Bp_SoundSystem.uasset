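; Sound system Blueprint that runs an FMOD tempo reference track and tests whether player clicks land on the beat.
; Each FMOD beat restarts a timeline that samples curves into beat, half-beat and quarter-beat windows.
; The character's beat-witness callback logs whichever windows are open.
; Procedural drum, bass and synth events with random triggers and pitches exist, but their marker-name dispatch is disconnected.
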(event `self.ReceiveBeginPlay`
  (`self.InitTempoTemoin`)
  (add `/Game/Pump/Core/Character/BP_Character.BeatWitness` (cast `/Game/Pump/Core/Character/BP_Character` (`GameplayStatics.GetPlayerCharacter` 0) :!pure true) (delegate `BeatClick`)))

(event `BeatClick`
  (`self.ClickInBeatPopotte`))

(event `self.A_M_Temoin.OnTimelineBeat`
  (params (Bar :type Integer) (Beat :type Integer) (Position :type Integer) (Tempo :type "Float (single-precision)") (TimeSignatureUpper :type Integer) (TimeSignatureLower :type Integer))
  (bind __ (`/Game/Pump/Core/BP_FunctionLibrary.GetTimelinePercentage` (`self.BeatDecomposer`)))
  ;[0 1 0.137] Beat
  (`Timeline|BeatDecomposer` :!via `PlayFromStart`
    (:`Update`
      (set `self.Beat` (`CurveFloat.GetFloatValue` (`self.BeatCurve`) __))
      (set `self.HalfBeat` (`CurveFloat.GetFloatValue` (`self.HalfBeatCurve`) __))
      (set `self.QuaterBeat` (`CurveFloat.GetFloatValue` (`self.QuaterBeatCurve`) __)))))

(event `ClickInBeatPopotte`
  (`self.TestBeat`)
  (`self.TestHalfBeat`)
  (`self.TestQuaterBeat`))

(event `self.A_M_Temoin.OnTimelineMarker`
  (params (Name :type String) (Position :type Integer)))

(event `Whole`
  ;[1 1 1] Whole
)

(event `Half`
  ;[1 1 1] Half
  (if (`KismetMathLibrary.RandomBoolWithWeight` 0.8)
    (bind _returnvalue (`FMODBlueprintStatics.PlayEvent2D` "/Game/FMOD/Events/Music/SoundEvents/Bass/A_M_LV1_Bass01.A_M_LV1_Bass01"))
    (`FMODBlueprintStatics.EventInstanceSetParameter` _returnvalue "Pitch Major" (`KismetMathLibrary.Conv_IntToDouble` (select `int` (`KismetMathLibrary.RandomIntegerInRange` 0 2) :`0` 0 :`1` 3 :`2` 4)))))

(event `Quarter`
  ;[1 1 1] Quarter
  (`|MultiGate` false true
    (:`Out 0`
      _)
    (:`Out 1`
      (`FMODBlueprintStatics.PlayEvent2D` "/Game/FMOD/Events/Music/SoundEvents/Beat/A_M_SE_Beat_Clap01.A_M_SE_Beat_Clap01" :!label _label))
    (:`Out 2`
      _)
    (:`Out 3`
      (goto _label)))
  (`FMODBlueprintStatics.PlayEvent2D` "/Game/FMOD/Events/Music/SoundEvents/Beat/A_M_SE_Beat_Kick01.A_M_SE_Beat_Kick01"))

(event `Eighth`
  ;[1 1 1] Eighth
  (if (`KismetMathLibrary.RandomBoolWithWeight` 0.7)
    (bind _returnvalue (`FMODBlueprintStatics.PlayEvent2D` "/Game/FMOD/Events/Music/SoundEvents/Bass/A_M_LV1_Synth01.A_M_LV1_Synth01"))
    (`FMODBlueprintStatics.EventInstanceSetParameter` _returnvalue "Pitch Major" (`KismetMathLibrary.Conv_IntToDouble` (select `int` (`KismetMathLibrary.RandomIntegerInRange` 0 5) :`0` -7 :`1` -3 :`2` 0 :`3` 2 :`4` 3 :`5` 4)))))

(event `Sixteenth`
  ;[1 1 1] Sixteenth
  (`|ExecutionSequence`
    (:`then_0`
      (if (`KismetMathLibrary.RandomBoolWithWeight` 0.5)
        (`FMODBlueprintStatics.PlayEvent2D` "/Game/FMOD/Events/Music/SoundEvents/Beat/A_M_SE_Beat_HH01.A_M_SE_Beat_HH01")))
    (:`then_1`
      (if (`KismetMathLibrary.RandomBoolWithWeight` 0.05)
        (`FMODBlueprintStatics.PlayEvent2D` "/Game/FMOD/Events/Music/SoundEvents/Beat/A_M_SE_Beat_Clap01.A_M_SE_Beat_Clap01")))))

(fn `InitTempoTemoin`
  (`FMODAudioComponent.Play` (`self.A_M_Temoin`)))

(fn `MakeScale`)

(fn `TestBeat`
  (if (!= (`self.Beat`) 0.0)
    (`/Game/Pump/Core/BP_FunctionLibrary.LogErer` "Beat")))

(fn `TestHalfBeat`
  (if (!= (`self.HalfBeat`) 0.0)
    (`/Game/Pump/Core/BP_FunctionLibrary.LogErer` "Half")))

(fn `TestQuaterBeat`
  (if (!= (`self.QuaterBeat`) 0.0)
    (`/Game/Pump/Core/BP_FunctionLibrary.LogErer` "Quater")))

(fn `UserConstructionScript`)