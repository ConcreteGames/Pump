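; Level manager that runs chapter progression and save-based loading by toggling visibility of each chapter's streamed gameplay, decor and planet levels.
; Chapter changes use a white-screen fade, held until FPS stabilizes or a frame-count fallback fires, and update the sound manager.
; Save loading teleports the player and polls streaming levels before fading out.
; It also registers bubbles and gravity platforms, switches planet lights and toggles platform movement by player distance.
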(event `ForceLevel`
  (set `self.CurrentLevelIndex` (`self.CurrentLevelIndex`)))

(event `self.ReceiveBeginPlay`
  ;[0 1 0.1559] BEGIN PLAY
  ;[1 0 0.904] TEST!!!! c'était après le delais
  ; mais j'en ai besoin au début
  ; Du coup je le mets là pour test
  (`self.ResisterSoundManager`)
  (`KismetSystemLibrary.Delay` 1.0)
  (`self.RegisterBubbles`)
  (`self.RegisterGravityPlateform`)
  (`self.InitRockSpawner`)
  (`self.SetStartFogDensity`)
  (`KismetSystemLibrary.K2_SetTimerDelegate` (delegate `TogglePlateformsMovement`) 0.5 true)
  (`self.ToogleMovementByDistance` :!label _label))

(event `TogglePlateformsMovement`
  (goto _label))

(event `HideAllPlateforms`
  (for _array_element (`self.AllGravityPlatforms`)
    (`/Game/Pump/LD/GravityPlateform/BP_GravityPlateform.SetVisiblity` _array_element false)
    (cast `/Game/Pump/LD/GravityPlateform/Sphere/BP_GravityPlateform_Sphere_Step` _array_element)))

(event `HideAllBubbles`
  (for _array_element (`self.AllBubbles`)
    (`/Game/Pump/LD/Bubble/BP_BubbleMaster.SetVisiblity` _array_element false)))

(event `OnABubbleIsEnteredForFirstTIme`
  (params (Bubble :type "/Game/Pump/LD/Bubble/BP_BubbleMaster Object Reference"))
  (`self.UpdateBubbleEnteredCount`))

(event `DisplayNewLevel`
  (`KismetSystemLibrary.Delay` 1.0)
  (`self.GetOrCreateWhiteScreenLoading`)
  (`/Game/Pump/Core/BP_FunctionLibrary.AddWidgetToViewportIfNotHere` (`self.pUI_WhiteScreenLoading`))
  (`/Game/Pump/UI/UI_WhiteScreenLoading.FadeIn` (`self.pUI_WhiteScreenLoading`))
  (`KismetSystemLibrary.Delay` 0.25)
  (`self.DisableCurrentDirectionalLight`)
  (set `self.CurrentLevelIndex` (+ (`self.CurrentLevelIndex`) 1))
  (`self.DisplayCurrentLevel`)
  (`self.Loading`))

(event `DisplayCurrentLevel`
  (`self.EditCurrentLDAndDecorVisibility` true true true true true true (`self.CurrentLevelIndex`))
  (`/Game/Pump/Core/SoundSystem/Bp_SoundSystem.ChangeChapter` (`self.PSoundManager`) (`self.CurrentLevelIndex`)))

(event `Loading`
  (bind _fpsarray (`self.FPSArray`))
  (bind _fpsarray_secushittypc (`self.FPSArray_SecuShittyPC`))
  (bind _returnvalue (/ 1.0 (`GameplayStatics.GetWorldDeltaSeconds`)))
  (`KismetArrayLibrary.Array_Clear` (`self.FPSArray`))
  (`KismetArrayLibrary.Array_Clear` (`self.FPSArray_SecuShittyPC`))
  (`Timeline|T_WaitLoading` :!via `PlayFromStart`
    (:`Update`
      (`|ExecutionSequence`
        (:`then_0`
          ;[1 1 1] Après 10 frames à bon FPS on met fin au Loading
          (if (> _returnvalue 20.0)
            (`KismetArrayLibrary.Array_Add` _fpsarray)
            (if (>= (`KismetArrayLibrary.Array_Length` _fpsarray) 100)
              (`TimelineComponent.Stop` (`self.T_WaitLoading`) :!label _label_2)
              (`self.LoadingDone`))
            (else
              (`KismetArrayLibrary.Array_Clear` _fpsarray))))
        (:`then_1`
          ;[1 1 1] ShittyComputer security Loading Done quand même
          (`KismetArrayLibrary.Array_Add` _fpsarray_secushittypc _returnvalue)
          (if (>= (`KismetArrayLibrary.Array_Length` _fpsarray_secushittypc) 100)
            (goto _label_2)))))))

(event `LoadingDone`
  (`self.RegisterBubbles`)
  (`self.RegisterGravityPlateform`)
  (`self.GetOrCreateWhiteScreenLoading`)
  (`/Game/Pump/Core/BP_FunctionLibrary.AddWidgetToViewportIfNotHere` (`self.pUI_WhiteScreenLoading`))
  (`/Game/Pump/UI/UI_WhiteScreenLoading.FadeOut` (`self.pUI_WhiteScreenLoading`)))

(event `AddBubble`
  (params (Bubble :type "/Game/Pump/LD/Bubble/BP_BubbleMaster Object Reference"))
  (`/Game/Pump/LD/Bubble/BP_BubbleMaster.SetBubbleManager` Bubble self)
  (`/Game/Pump/LD/Bubble/BP_BubbleMaster.SetBubbleManager` Bubble self)
  (`/Game/Pump/LD/Bubble/BP_BubbleMaster.SetDefaultState` Bubble (`self.BubbleColorAtStart`))
  (`KismetArrayLibrary.Array_AddUnique` (`self.AllBubbles`) Bubble))

(event `UpdatePlatformsParticlesDirection`
  ;[1 0 0] DEBRANCHE CAR ERROR
)

(event `InitRockSpawner`
  (bind _outactors (`GameplayStatics.GetAllActorsOfClass` "/Game/Pump/LD/FlyingRocksSpawner/BP_FlyingRockSpawner.BP_FlyingRockSpawner_C"))
  (`/Game/Pump/LD/FlyingRocksSpawner/BP_FlyingRockSpawner.Init` (`|GetArrayItem` _outactors) self))

(event `UpdateStepLightsState`
  (for _array_element (`self.PlanetSteps`)
    (`self.SetLightActivation` (`/Game/Pump/LD/GravityPlateform/Sphere/BP_GravityPlateform_Sphere_Step.DirectionalLight` _array_element)))
  (`self.SetLightActivation` (`/Game/Pump/LD/GravityPlateform/Sphere/BP_GravityPlateform_Sphere_Step.DirectionalLight` (`self.CurrentPlanetStep`)) true))

(event `PlanetLandingDone`
  (`self.EditCurrentLDAndDecorVisibility` true false true false false false (`self.CurrentLevelIndex`)))

(event `LoadALevel`
  (params (ForceALevel :type Boolean) (ForcedLevel :type "/Game/Pump/Core/E_Chapters Enum" :default "NewEnumerator0"))
  (bind _local_leveltoload (`self.LOCAL_LevelToLoad`))
  (set `self.LOCAL_LevelToLoad` (select `bool` ForceALevel :`false` (`/Game/ConcreteTemplateNew/BP_SaveGame.CurrentLevel` (`/Game/Pump/Core/BP_FunctionLibrary.GetSave`)) :`true` ForcedLevel))
  (`self.ShowLastSavedLevel`)
  (`self.SetPlayersLocAndRot`)
  (`self.GetOrCreateWhiteScreenLoading`)
  (if (and (`LevelStreaming.IsLevelLoaded` (`GameplayStatics.GetStreamingLevel` (select `/Game/Pump/Core/E_Chapters` _local_leveltoload :`NewEnumerator0` "Chapter_1_Mineral" :`NewEnumerator1` "Chapter_1_Mineral" :`NewEnumerator2` "Chapter_2_Vegetal" :`NewEnumerator3` "Chapter_2_Vegetal" :`NewEnumerator4` "Chapter_3_Animal" :`NewEnumerator5` "Chapter_3_Animal" :`NewEnumerator7` "Chapter_4_Ending" :`NewEnumerator8` "Chapter_4_Ending" :!type "Name"))) (`LevelStreaming.IsLevelLoaded` (`GameplayStatics.GetStreamingLevel` (select `/Game/Pump/Core/E_Chapters` _local_leveltoload :`NewEnumerator0` "Chapter_1_Mineral_Decor" :`NewEnumerator1` "Chapter_1_Mineral_Decor" :`NewEnumerator2` "Chapter_2_Vegetal_Decor" :`NewEnumerator3` "Chapter_2_Vegetal_Decor" :`NewEnumerator4` "Chapter_3_Animal_Decor" :`NewEnumerator5` "Chapter_3_Animal_Decor" :`NewEnumerator7` "Chapter_4_Ending" :`NewEnumerator8` "Chapter_4_Ending" :!type "Name"))) (`LevelStreaming.IsLevelLoaded` (`GameplayStatics.GetStreamingLevel` (select `/Game/Pump/Core/E_Chapters` _local_leveltoload :`NewEnumerator0` "Chapter_1_Mineral_PlanetStep" :`NewEnumerator1` "Chapter_1_Mineral_PlanetStep" :`NewEnumerator2` "Chapter_2_Vegetal_PlanetStep" :`NewEnumerator3` "Chapter_2_Vegetal_PlanetStep" :`NewEnumerator4` "Chapter_3_Animal_PlanetStep" :`NewEnumerator5` "Chapter_3_Animal_PlanetStep" :`NewEnumerator7` "Chapter_4_Ending" :`NewEnumerator8` "Chapter_4_Ending" :!type "Name")))) :!pinned true :!label _label_3
    (`LowEntryExtendedStandardLibrary.DelayFrames` 60) ; petite sécu
    (`GameplayStatics.SetGlobalTimeDilation` 1.0)
    (`/Game/Pump/UI/UI_WhiteScreenLoading.FadeOut` (`self.pUI_WhiteScreenLoading`))
    (else
      (`LowEntryExtendedStandardLibrary.DelayFrames` 5)
      (goto _label_3))))

(event `End_ShowPlanet3`
  ;[1 1 1] if play End directly from the Menu: show planet step 3
  (if (not (`LevelStreaming.IsLevelVisible` (`GameplayStatics.GetStreamingLevel` "Chapter_3_Animal_PlanetStep")))
    (`self.ShowHideALevel` "Chapter_3_Animal_PlanetStep" true)
    (`KismetSystemLibrary.Delay` 0.1)
    ;[1 1 1] Show planet step 3 max scale
    (bind _outactors (`GameplayStatics.GetAllActorsOfClass` "/Game/Pump/LD/GravityPlateform/Sphere/Steps/BP_GravityPlateform_Sphere_Step_3.BP_GravityPlateform_Sphere_Step_3_C"))
    (bind _output (`|GetArrayItem` _outactors))
    (`/Engine/EditorBlueprintResources/StandardMacros.IsValid` _output
      (:`Is Valid`
        (`/Game/Pump/LD/GravityPlateform/Sphere/BP_GravityPlateform_Sphere_Step.GrowthEnded` _output true))
      (:`Is Not Valid`
        (`/Game/Pump/Core/BP_FunctionLibrary.LogErerror` "LA PLANET 3 n'est pas là à l'ending. Je ne peux pas lancer \"Start Planet Growth\"")))))

(fn `DisableCurrentDirectionalLight`
  (bind _outactors (`GameplayStatics.GetAllActorsOfClass` "/Game/Pump/LD/GravityPlateform/Sphere/BP_GravityPlateform_Sphere_Step.BP_GravityPlateform_Sphere_Step_C"))
  (for _array_element _outactors
    (if (`self.ActorHasTag` _array_element (`KismetStringLibrary.Conv_StringToName` (`KismetStringLibrary.Concat_StrStr` "LevelIndex" (`KismetStringLibrary.Conv_IntToString` (`self.CurrentLevelIndex`)))))
      (`self.SetLightActivation` (`/Game/Pump/LD/GravityPlateform/Sphere/BP_GravityPlateform_Sphere_Step.DirectionalLight` _array_element)))))

(fn `EditCurrentLDAndDecorVisibility`
  (params (LDEditVisibility :type Boolean) (LDNewVisibility :type Boolean) (DecorEditVisibility :type Boolean) (DecorNewVisibility :type Boolean) (PlanetEditVisibility :type Boolean) (PlanetNewVisibility :type Boolean) (LevelIndex :type Integer))
  (`|ExecutionSequence`
    (:`then_0`
      (if LDEditVisibility
        (`self.ShowHideALevel` (select `int` LevelIndex :`0` "Chapter_1_Mineral" :`1` "Chapter_2_Vegetal" :`2` "Chapter_3_Animal" :`3` "Chapter_4_Ending" :!type "Name") LDNewVisibility)
        (if (== LevelIndex 3)
          (`self.End_ShowPlanet3`))))
    (:`then_1`
      (if DecorEditVisibility
        (if (not (>= LevelIndex 3))
          (`self.ShowHideALevel` (select `int` LevelIndex :`0` "Chapter_1_Mineral_Decor" :`1` "Chapter_2_Vegetal_Decor" :`2` "Chapter_3_Animal_Decor" :!type "Name") DecorNewVisibility))))
    (:`then_2`
      (if PlanetEditVisibility
        (if (not (>= LevelIndex 3))
          (`self.ShowHideALevel` (select `int` LevelIndex :`0` "Chapter_1_Mineral_PlanetStep" :`1` "Chapter_2_Vegetal_PlanetStep" :`2` "Chapter_3_Animal_PlanetStep" :!type "Name") PlanetNewVisibility))))))

(fn `GetOrCreateWhiteScreenLoading`
  (returns (pUI_WhiteScreenLoading :type "/Game/Pump/UI/UI_WhiteScreenLoading Object Reference"))
  (`/Engine/EditorBlueprintResources/StandardMacros.IsValid` (`self.pUI_WhiteScreenLoading`)
    (:`Is Valid`
      _)
    (:`Is Not Valid`
      (bind _foundwidgets (`WidgetBlueprintLibrary.GetAllWidgetsOfClass` "/Game/Pump/UI/UI_WhiteScreenLoading.UI_WhiteScreenLoading_C"))
      (bind _output (`|GetArrayItem` _foundwidgets))
      (`/Engine/EditorBlueprintResources/StandardMacros.IsValid` _output
        (:`Is Valid`
          (set `self.pUI_WhiteScreenLoading` _output))
        (:`Is Not Valid`
          (bind _returnvalue (`|CreateWidget` "/Game/Pump/UI/UI_WhiteScreenLoading.UI_WhiteScreenLoading_C"))
          (set `self.pUI_WhiteScreenLoading` _returnvalue)))))
  (return (`self.pUI_WhiteScreenLoading`)))

(fn `ResisterSoundManager`
  (bind _outactors (`GameplayStatics.GetAllActorsOfClass` "/Game/Pump/Core/SoundSystem/Bp_SoundSystem.Bp_SoundSystem_C"))
  (set `self.PSoundManager` (`|GetArrayItem` _outactors)))

(fn `SetLightActivation`
  (params (TargetLight :type "LightComponentBase Object Reference") (State :type Boolean))
  (`LightComponentBase.SetCastShadows` TargetLight State)
  (`LightComponentBase.SetCastVolumetricShadow` TargetLight State)
  (`SceneComponent.SetVisibility` TargetLight State false)
  (if State
    (`ActorComponent.Activate` TargetLight true)
    (else
      (`ActorComponent.Deactivate` TargetLight))))

(fn `SetPlayersLocAndRot`
  (bind _local_leveltoload (`self.LOCAL_LevelToLoad`))
  (`self.K2_SetActorLocationAndRotation` (`/Game/Pump/Core/BP_FunctionLibrary.GetCharMatter`) (select `/Game/Pump/Core/E_Chapters` _local_leveltoload :`NewEnumerator0` (0.0 0.0 2000.0) :`NewEnumerator1` (107503.226563 6702.431152 54952.265625) :`NewEnumerator2` (113940.476563 -8175.588867 63645.882813) :`NewEnumerator3` (275817.90625 79093.4375 151080.1875) :`NewEnumerator4` (332551.8125 -172476.25 124966.015625) :`NewEnumerator5` (622891.5625 219507.359375 703583.1875) :`NewEnumerator7` (668596.875 227880.484375 788426.375) :!type "Vector Structure") (select `/Game/Pump/Core/E_Chapters` _local_leveltoload :`NewEnumerator0` (struct :`Pitch` -25.0 :`Yaw` -180.0) :`NewEnumerator1` (struct :`Pitch` 48.0 :`Yaw` -55.0) :`NewEnumerator2` (struct :`Yaw` -70.0) :`NewEnumerator3` (struct :`Pitch` -3.0 :`Yaw` -74.0 :`Roll` -147.0) :`NewEnumerator4` (struct :`Pitch` 3.0 :`Yaw` -90.0) :`NewEnumerator5` (struct :`Pitch` 78.0 :`Yaw` 20.0 :`Roll` 9.0) :!type "Rotator Structure") false true))

(fn `SetStartFogDensity`
  (bind _outactors (`GameplayStatics.GetAllActorsOfClass` "/Script/Engine.ExponentialHeightFog"))
  (`ExponentialHeightFogComponent.SetFogDensity` (`ExponentialHeightFog.Component` (`|GetArrayItem` _outactors)) 0.2))

(fn `ShowHideALevel`
  (params (levelName :type Name) (bShouldBeVisible :type Boolean))
  (set `LevelStreaming.bShouldBeVisible` bShouldBeVisible (`GameplayStatics.GetStreamingLevel` levelName)))

(fn `ShowLastSavedLevel`
  (set `self.CurrentLevelIndex` (select `/Game/Pump/Core/E_Chapters` (`self.LOCAL_LevelToLoad`) :`NewEnumerator2` 1 :`NewEnumerator3` 1 :`NewEnumerator4` 2 :`NewEnumerator5` 2 :`NewEnumerator7` 3))
  (`self.DisplayCurrentLevel`))

(fn `ToogleMovementByDistance`
  (bind _outactors (`GameplayStatics.GetAllActorsOfClass` "/Game/Pump/LD/GravityPlateform/Plane/BP_GravityPlateform_Plane_OneSided.BP_GravityPlateform_Plane_OneSided_C"))
  (for _array_element _outactors
    (if (< (`KismetMathLibrary.VSize` (- (`self.K2_GetActorLocation` _array_element) (`self.K2_GetActorLocation` (`/Game/Pump/Core/BP_FunctionLibrary.GetCharMatter`)))) (`self.PlateformsMovementActivationDistance`))
      (`/Game/Pump/LD/GravityPlateform/Plane/BP_GravityPlateform_Plane_OneSided.PlayMovement` _array_element)
      (else
        (`/Game/Pump/LD/GravityPlateform/Plane/BP_GravityPlateform_Plane_OneSided.StopMovement` _array_element)))))

(fn `UpdateBubbleEnteredCount`
  (bind _result (`/Engine/EditorBlueprintResources/StandardMacros.IncrementInt` (`self.BubbleEnteredCount`))
    (:`  `
      (set `self.BubbleEnteredRatio` (/ (`KismetMathLibrary.Conv_IntToDouble` _result) (`KismetMathLibrary.Conv_IntToDouble` (`KismetArrayLibrary.Array_Length` (`self.AllBubbles`))))))))

(fn `UserConstructionScript`)