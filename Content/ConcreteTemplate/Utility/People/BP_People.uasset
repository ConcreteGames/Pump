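; BP_People is a utility actor that displays people through a particle system, configured entirely in the Construction Script.
; UseThinPeople either keeps the component's existing template or, when false, swaps it to PS_PeopleLarge.
; Each variant gets a random material from its own set on slot 0, so the look can change whenever the script reruns.
; The Event Graph holds no active logic.
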(fn `UserConstructionScript`
  (if (`self.bUseThinPeople`)
    (`PrimitiveComponent.SetMaterial` (`self.ParticleSystem`) 0 (select `int` (`KismetMathLibrary.RandomIntegerInRange` 0 2) :`0` "/Game/ConcreteTemplate/Utility/People/MI_People_1.MI_People_1" :`1` "/Game/ConcreteTemplate/Utility/People/MI_People_2.MI_People_2" :`2` "/Game/ConcreteTemplate/Utility/People/MI_People_3.MI_People_3" :!type "MaterialInterface Object Reference"))
    (else
      (`ParticleSystemComponent.SetTemplate` (`self.ParticleSystem`) "/Game/ConcreteTemplate/Utility/People/PS_PeopleLarge.PS_PeopleLarge")
      (`PrimitiveComponent.SetMaterial` (`self.ParticleSystem`) 0 (select `int` (`KismetMathLibrary.RandomIntegerInRange` 0 1) :`0` "/Game/ConcreteTemplate/Utility/People/M_PeopleLarge_1.M_PeopleLarge_1" :`1` "/Game/ConcreteTemplate/Utility/People/MI_PeopleLarge_2.MI_PeopleLarge_2" :!type "MaterialInterface Object Reference")))))